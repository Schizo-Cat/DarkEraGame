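; Player controller for the black hole space game, owning the general UI, menu toggles, time speed and game states.
; BeginPlay finds manager actors, binds HUD buttons and debug CVars, and loads saves through the game instance.
; ChangeGameState applies data table rows to music, color, building, saving and resource drain.
; Tick watches black hole mass, triggering the death state when critical and an explosion and main menu return once it is gone.
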(event Custom|SetTimeSpeed
  (params (Time%20Speed :type Float%20%28single-precision%29))
  (bind _spaceship (Variables|References|GetSpaceShip))
  (bind _spaceship_2 (Variables|References|GetSpaceShip))
  (bind _generalui (Variables|References|GetGeneralUI))
  (bind _wbp_gamehud (Variables|/Game/UI/HUD/WBP_GeneralUI.WBP_GeneralUI_C|GetWBP_GameHUD _generalui))
  (bind _p_flamethrower (Variables|/Game/Core/Blueprints/BP_Ship.BP_Ship_C|GetP_Flamethrower _spaceship_2))
  (if (Variables|SpeedControl|GetCanChangeTime)
    (bind _output_get (Variables|Default|SettimeSpeed Time%20Speed))
    (if (> _output_get 0.0)
      (Variables|SpeedControl|SetSavedSpeed _output_get))
    (Utilities|IsValid _spaceship
      (:Is%20Valid
        (Variables|/Script/Engine.ParticleSystemComponent|SetCustomTimeDilation (Variables|/Game/Core/Blueprints/BP_Ship.BP_Ship_C|GetP_Flamethrower _spaceship) _output_get)
        (if (Variables|Default|GetIsTimeFrozen)
          (Variables|/Script/Engine.ParticleSystemComponent|SetCustomTimeDilation _p_flamethrower 0.0)
          (Default|SetButtonSelected _wbp_gamehud (Variables|/Game/UI/HUD/WBP_GameHUD.WBP_GameHUD_C|GetPauseButton _wbp_gamehud))
          (else
            (bind _output_get_2 (Variables|Default|SettimeSpeed (Variables|SpeedControl|GetSavedSpeed)))
            (Variables|/Script/Engine.ParticleSystemComponent|SetCustomTimeDilation _p_flamethrower _output_get_2)
            (if (== _output_get_2 (Variables|SpeedControl|GetSpeedOne))
              (Default|SetButtonSelected _wbp_gamehud (Variables|/Game/UI/HUD/WBP_GameHUD.WBP_GameHUD_C|GetSpeedOneButton _wbp_gamehud))
              (elif (== _output_get_2 (Variables|SpeedControl|GetSpeedTwo))
                (Default|SetButtonSelected _wbp_gamehud (Variables|/Game/UI/HUD/WBP_GameHUD.WBP_GameHUD_C|GetSpeedTwoButton _wbp_gamehud))
                (elif (== _output_get_2 (Variables|SpeedControl|GetSpeedThree))
                  (Default|SetButtonSelected _wbp_gamehud (Variables|/Game/UI/HUD/WBP_GameHUD.WBP_GameHUD_C|GetSpeedThreeButton _wbp_gamehud)))))))))))

(event Custom|LerpColor
  (bind _returnvalue (Rendering|Material|GetVectorParameterValue "/Game/Materials/MPC_Collection.MPC_Collection" "color" :!class /Script/Engine.KismetMaterialLibrary))
  (Rendering|Material|SetVectorParameterValue "/Game/Materials/MPC_Collection.MPC_Collection" "color" (* _returnvalue 2.0) :!class /Script/Engine.KismetMaterialLibrary))

(event Custom|SetBlackHoleName
  (params (BlackHoleName :type Text))
  (bind _output_get (Variables|Default|SetBlackHoleName BlackHoleName))
  (Rendering|Components|TextRender|SetText (Variables|/Game/UI/HUD/WBP_GameHUD.WBP_GameHUD_C|GetNameText (Variables|/Game/UI/HUD/WBP_GeneralUI.WBP_GeneralUI_C|GetWBP_GameHUD (Variables|References|GetGeneralUI))) _output_get))

(event Custom|ChangeGameState
  (params (GameStatus :type E_GameStatus%20Enum :default "NewEnumerator0"))
  (bind _basesurrounding (Variables|References|GetBaseSurrounding))
  ;[1 1 1] GameState
  (bind _outrownames (DataTable|GetDataTableRowNames (Variables|Default|GetStatesDataTable)))
  (bind _array_element (Utilities|Array|ForEachLoopwithBreak _outrownames :!label _label)
    (:LoopBody
      (bind _returnvalue (Utilities|GetDataTableRow (Variables|Default|GetStatesDataTable) _array_element)
        (:then
          (if (Utilities|Enum|Equal(Enum) GameStatus (.GameStateEnum (Utilities|Struct|BreakS_GameStatus _returnvalue)))
            (Variables|Default|SetCurrentGameState _returnvalue)
            (goto _label Break)))))
    (:Completed
      (Utilities|IsValid (Variables|Default|GetGlitchScreen)
        (:Is%20Valid
          (Widget|RemovefromParent (Variables|Default|GetGlitchScreen)))
        (:Is%20Not%20Valid
          _))
      (Utilities|FlowControl|Sequence
        (:then_0
          (if (== (.GameMusic (Utilities|Struct|BreakS_GameStatus (Variables|Default|GetCurrentGameState))) 0)
            _
            (else
              (Utilities|CompareMusic (.GameMusic (Utilities|Struct|BreakS_GameStatus (Variables|Default|GetCurrentGameState))))))
          (Variables|/Game/Core/Blueprints/TimeManager.TimeManager_C|SetIsTimeGoing (Variables|References|GetTimeManager) (not (.PauseResourceWastage (Utilities|Struct|BreakS_GameStatus (Variables|Default|GetCurrentGameState)))))
          (Variables|/Game/Core/Blueprints/BP_MainBlackHole.BP_MainBlackHole_C|SetIsMassLosing (Variables|References|GetBlackHole) (not (.PauseResourceWastage (Utilities|Struct|BreakS_GameStatus (Variables|Default|GetCurrentGameState)))))
          (Variables|/Game/Researches/BP_ResearchManager.BP_ResearchManager_C|SetIsResearchGoing (Variables|References|GetResearchManager) (not (.PauseResourceWastage (Utilities|Struct|BreakS_GameStatus (Variables|Default|GetCurrentGameState)))))
          (Default|TurnVisibility _basesurrounding (not (.DisableBuilding (Utilities|Struct|BreakS_GameStatus (Variables|Default|GetCurrentGameState)))))
          (Variables|/Game/Core/Blueprints/BP_BaseSurrounding.BP_BaseSurrounding_C|SetSlotsAvailable _basesurrounding (not (.DisableBuilding (Utilities|Struct|BreakS_GameStatus (Variables|Default|GetCurrentGameState)))))
          (CallFunction|EnableSaving (not (.DisableSavingGame (Utilities|Struct|BreakS_GameStatus (Variables|Default|GetCurrentGameState)))))
          (if (.IsAdditionalState (Utilities|Struct|BreakS_GameStatus (Variables|Default|GetCurrentGameState)))
            _
            (else
              _))
          (bind _output_get (Variables|Default|SetAppendColor (Math|Conversions|ToLinearColor(Color) (.GameColor (Utilities|Struct|BreakS_GameStatus (Variables|Default|GetCurrentGameState))))))
          (Default|SetGameColor (Variables|References|GetBaseSurrounding) _output_get))
        (:then_1
          (switch Utilities|FlowControl|Switch|SwitchonE_GameStatus (.GameStateEnum (Utilities|Struct|BreakS_GameStatus (Variables|Default|GetCurrentGameState)))
            (:NewEnumerator3
              (bind _returnvalue_2 (UserInterface|CreateWidget "/Game/UI/CriticalUI/WBP_GlitchingEffects.WBP_GlitchingEffects_C"))
              (bind _output_get_2 (Variables|Default|SetGlitchScreen _returnvalue_2))
              (UserInterface|Viewport|AddtoViewport _output_get_2 -15))))))))

(event Input|EnhancedActionEvents|EnhancedInputActionIA_Use
  (params (ActionValue :type Boolean) (ElapsedSeconds :type Float%20%28double-precision%29) (TriggeredSeconds :type Float%20%28double-precision%29) (InputAction :type Input%20Action%20Object%20Reference :default "/Game/Input/MenuControls/IA_Use.IA_Use"))
  ;[1 1 1] Black Hole Mass UI
  (:Started
    (Default|ClickSelected (Variables|References|GetBaseSurrounding))))

(event EventTick
  (params (DeltaSeconds :type Float%20%28single-precision%29))
  (bind _blackhole (Variables|References|GetBlackHole))
  (bind _currentmass (Variables|/Game/Core/Blueprints/BP_MainBlackHole.BP_MainBlackHole_C|GetCurrentMass _blackhole))
  (bind _returnvalue (Math|Float|Round _currentmass))
  ;[1 1 1] Black Hole Mass UI
  (if (Utilities|Enum|Equal(Enum) (Variables|Default|GetCurrentLevelName) "GameUniverse")
    (Variables|Default|SetDelta%20Seconds (* DeltaSeconds (Variables|Default|GettimeSpeed)))
    (Utilities|IsValid _blackhole
      (:Is%20Valid
        (Rendering|Components|TextRender|SetText (Variables|/Game/UI/HUD/WBP_GameHUD.WBP_GameHUD_C|GetMassText (Variables|/Game/UI/HUD/WBP_GeneralUI.WBP_GeneralUI_C|GetWBP_GameHUD (Variables|References|GetGeneralUI))) (Utilities|Text|ToText(Integer) _returnvalue))
        (bind _output_get (Variables|States|SetIsMassCritical (<= _returnvalue 100)))
        (if _output_get
          (Utilities|FlowControl|DoOnce false :!label _label
            (:Completed
              (CallFunction|ChangeGameState "NewEnumerator3")
              (goto _label_2 Reset)))
          (else
            (Utilities|FlowControl|DoOnce true :!label _label_2
              (:Completed
                (CallFunction|ChangeGameState "NewEnumerator5")
                (goto _label Reset))))))
      (:Is%20Not%20Valid
        (Utilities|FlowControl|DoOnce false
          (:Completed
            (bind _returnvalue_2 (Utilities|Time|SetTimerbyEvent (delegate Custom|LerpColor) 0.03 true))
            (Variables|Default|SetlerpTimer _returnvalue_2)
            (Utilities|Time|ClearandInvalidateTimerbyHandle (Variables|/Game/Core/Blueprints/TimeManager.TimeManager_C|GetTimerSetTime (Variables|References|GetTimeManager)))
            (Widget|RemovefromParent (Variables|References|GetGeneralUI))
            (Audio|Components|Audio|SetSound (Variables|Default|GetAudioPlayer) "/Game/Core/Audio/SFX/Black_hole_explosion.Black_hole_explosion")
            (Utilities|FlowControl|Delay 1.8)
            (Utilities|Time|ClearandInvalidateTimerbyHandle (Variables|Default|GetlerpTimer))
            (Utilities|FlowControl|Delay 2.0)
            (Game|OpenLevel(byObjectReference) "/Game/Maps/MainMenu.MainMenu")))))))

(event Custom|PauseTime
  ;[1 1 1] Time
)

(event Custom|ToggleResearchMenu
  ;[1 1 1] ResearchToggle
  (if (Variables|States|GetCanResearch)
    (Utilities|ToggleWidget (Variables|/Game/UI/HUD/WBP_GeneralUI.WBP_GeneralUI_C|GetResearchWindow (Variables|References|GetGeneralUI)) true true)))

(event Custom|ToggleSettings
  (bind _generalui (Variables|References|GetGeneralUI))
  (bind _wbp_settings (Variables|/Game/UI/HUD/WBP_GeneralUI.WBP_GeneralUI_C|GetWBP_Settings _generalui))
  ;[1 1 1] SettingsToggle
  (Default|SetMenuColor _wbp_settings)
  (Utilities|ToggleWidget _wbp_settings false false))

(event Custom|ToggleStatisticsWindow
  ;[1 1 1] ToggleStaticsWindow
  (Utilities|ToggleWidget (Variables|/Game/UI/HUD/WBP_GeneralUI.WBP_GeneralUI_C|GetWBP_MassStatistics (Variables|References|GetGeneralUI)) false false))

(event Custom|LoadSaveData
  ;[1 1 1] Load Saved Game
  (bind _returnvalue (SaveGame|LoadGamefromSlot "Save"))
  (bind _asbp_save_object (Utilities|Casting|CastToBP_SaveObject _returnvalue))
  (Variables|Default|SetSave%20Object _asbp_save_object)
  (Utilities|FlowControl|Sequence
    (:then_0
      (Variables|/Game/Core/Blueprints/BP_MainBlackHole.BP_MainBlackHole_C|SetCurrentMass (Variables|References|GetBlackHole) (Variables|/Game/SaveGame/BP_SaveObject.BP_SaveObject_C|GetMass (Variables|Default|GetSave%20Object))))
    (:then_1
      (for _array_element (Variables|/Game/SaveGame/BP_SaveObject.BP_SaveObject_C|GetJournalEnries (Variables|Default|GetSave%20Object))
        (Default|UpdateEntry (Variables|References|GetJournal) _array_element (.IsDiscovered (Utilities|Struct|BreakJournalEntry _array_element)) (.IsNewOne (Utilities|Struct|BreakJournalEntry _array_element)))))
    (:then_2
      (for _array_element_2 (Variables|/Game/SaveGame/BP_SaveObject.BP_SaveObject_C|GetResearches (Variables|Default|GetSave%20Object))
        (Default|AddResearchedResearch (Variables|References|GetResearchManager))
        (Rendering|Components|TextRender|SetText (Variables|/Game/UI/HUD/WBP_GameHUD.WBP_GameHUD_C|GetNameText (Variables|/Game/UI/HUD/WBP_GeneralUI.WBP_GeneralUI_C|GetWBP_GameHUD (Variables|References|GetGeneralUI))) (Utilities|Text|ToText(String) (Variables|/Game/SaveGame/BP_SaveObject.BP_SaveObject_C|GetName (Variables|Default|GetSave%20Object))))))))

(event Custom|ToggleBuildMenu
  (bind _generalui (Variables|References|GetGeneralUI))
  (bind _wbp_buildmenu (Variables|/Game/UI/HUD/WBP_GeneralUI.WBP_GeneralUI_C|GetWBP_BuildMenu _generalui))
  ;[1 1 1] ToggleBuildMenu
  (Utilities|ToggleWidget _wbp_buildmenu false false
    (:WidgetEnabled
      (Default|InitializeBuildings _wbp_buildmenu)
      (CallFunction|ChangeGameState "NewEnumerator6")
      (Variables|States|SetCanClick false))
    (:WIdgetDisabled
      (CallFunction|ChangeGameState "NewEnumerator5")
      (Variables|States|SetCanClick true))))

(event Custom|SetUpExtraction
  (params (NewValue :type Boolean))
  ;[1 1 1] States
  (Variables|States|SetCanExtract NewValue))

(event Custom|SetResearchStatus
  (params (NewValue :type Boolean))
  ;[1 1 1] States
  (Variables|States|SetCanResearch NewValue)
  (Widget|SetIsEnabled (Variables|/Game/UI/HUD/WBP_GameHUD.WBP_GameHUD_C|GetResearchButton (Variables|/Game/UI/HUD/WBP_GeneralUI.WBP_GeneralUI_C|GetWBP_GameHUD (Variables|References|GetGeneralUI))) true))

(event Custom|SetIsCloseToBaseStatus
  (params (NewValue :type Boolean))
  (bind _returnvalue (not NewValue))
  ;[1 1 1] States
  (Variables|States|SetIsCloseToBase NewValue)
  (Default|TurnCollision (Variables|References|GetBaseSurrounding) _returnvalue)
  (Default|TurnVisibility (Variables|References|GetBaseSurrounding) _returnvalue))

(event Custom|ToggleManagment
  ;[1 1 1] ShipManagment Toggle
  (Utilities|ToggleWidget (Variables|/Game/UI/HUD/WBP_GeneralUI.WBP_GeneralUI_C|GetWBP_ShipManagment (Variables|References|GetGeneralUI)) true true))

(event Custom|ToggleContact
  (bind _generalui (Variables|References|GetGeneralUI))
  (bind _wbp_gamehud (Variables|/Game/UI/HUD/WBP_GeneralUI.WBP_GeneralUI_C|GetWBP_GameHUD _generalui))
  (bind _communicationnotification (Variables|/Game/UI/HUD/WBP_GameHUD.WBP_GameHUD_C|GetCommunicationNotification _wbp_gamehud))
  ;[1 1 1] CommunicateWindowToggle
  (Utilities|ToggleWidget (Variables|/Game/UI/HUD/WBP_GeneralUI.WBP_GeneralUI_C|GetWBP_dialogueWindow _generalui) true true
    (:WidgetEnabled
      (if (Widget|IsVisible _communicationnotification)
        (Widget|SetVisibility _communicationnotification "Hidden")
        (Class|UserWidget|StopAnimation _wbp_gamehud (Variables|/Game/UI/HUD/WBP_GameHUD.WBP_GameHUD_C|GetCommunicationNotificatio _wbp_gamehud))))))

(event Custom|ToggleJournal
  (bind _generalui (Variables|References|GetGeneralUI))
  (bind _wbp_journalwidget (Variables|/Game/UI/HUD/WBP_GeneralUI.WBP_GeneralUI_C|GetWBP_JournalWidget _generalui))
  ;[1 1 1] JournalToggle
  (Utilities|ToggleWidget _wbp_journalwidget false false
    (:WidgetEnabled
      _)
    (:WIdgetDisabled
      _))
  (Default|CheckJournalOpen _wbp_journalwidget)
  (UserInterface|Animation|PlayAnimation _wbp_journalwidget (Variables|/Game/Journal/WBP_JournalWidget.WBP_JournalWidget_C|GetOpenJournal _wbp_journalwidget) 0.0 1 "Forward" 1.0 false))

(event Custom|Speed1
  ;[1 1 1] Time
  (CallFunction|SetTimeSpeed (Variables|SpeedControl|GetSpeedOne))
  (Variables|Default|SetIsTimeFrozen false))

(event Custom|Speed2
  ;[1 1 1] Time
  (CallFunction|SetTimeSpeed (Variables|SpeedControl|GetSpeedTwo))
  (Variables|Default|SetIsTimeFrozen false))

(event Custom|Speed3
  ;[1 1 1] Time
  (CallFunction|SetTimeSpeed (Variables|SpeedControl|GetSpeedThree))
  (Variables|Default|SetIsTimeFrozen false))

(event Custom|MapToggle
  ;[1 1 1] MapToggle
  (Utilities|ToggleWidget (Variables|/Game/UI/HUD/WBP_GeneralUI.WBP_GeneralUI_C|GetWBP_Map (Variables|References|GetGeneralUI)) true true))

(event Custom|ToggleEscMenu
  (bind _generalui (Variables|References|GetGeneralUI))
  (bind _wbp_menuhud (Variables|/Game/UI/HUD/WBP_GeneralUI.WBP_GeneralUI_C|GetWBP_MenuHUD _generalui))
  (bind _widgetswitcher (Variables|/Game/UI/HUD/WBP_GeneralUI.WBP_GeneralUI_C|GetWidgetSwitcher _generalui))
  ;[1 1 1] Open Menu Hud
  (if (== (Class|WidgetSwitcher|GetActiveWidgetIndex _widgetswitcher) 0)
    (Utilities|ToggleWidget _wbp_menuhud false false
      (:WidgetEnabled
        (Default|SetColorMenu _wbp_menuhud)))
    (else
      (Class|WidgetSwitcher|SetActiveWidgetIndex _widgetswitcher)
      (Input|AddMappingContext (PlayerController|LocalPlayerSubsystems|GetEnhancedInputLocalPlayerSubsystem self) "/Game/Input/Movement/IMC_Spectating.IMC_Spectating" 0 "(bIgnoreAllPressedKeysUntilRelease=True,bForceImmediately=False,bNotifyUserSettings=False)")
      (Variables|States|SetCanClick true))))

(event Custom|Command
  (params (CVarName :type String))
  (bind _tasksystem (Variables|References|GetTaskSystem))
  ;[1 1 1] CVARS
  (switch string CVarName
    (:deStartSingularity
      (bind _returnvalue (Utilities|GetDataTableRow "/Game/Core/DataTables/TaskList.TaskList" "E_6Objects")
        (:then
          (Default|AddTask _tasksystem _returnvalue)
          (Default|CompleteTask _tasksystem _returnvalue)
          (Default|ClearTasks _tasksystem))))
    (:deUnlockAllBuildings
      (bind _outrownames (DataTable|GetDataTableRowNames "/Game/Core/DataTables/DT_Buildings.DT_Buildings"))
      (for _array_element _outrownames
        (bind _returnvalue_2 (Utilities|GetDataTableRow "/Game/Core/DataTables/DT_Buildings.DT_Buildings" _array_element)
          (:then
            (Utilities|Array|Add (Variables|Default|GetAvailableBuildings) _returnvalue_2)))))))

(event Input|EnhancedActionEvents|EnhancedInputActionIA_Journal
  (params (ActionValue :type Boolean) (ElapsedSeconds :type Float%20%28double-precision%29) (TriggeredSeconds :type Float%20%28double-precision%29) (InputAction :type Input%20Action%20Object%20Reference :default "/Game/Input/MenuControls/IA_Journal.IA_Journal"))
  (bind _generalui (Variables|References|GetGeneralUI))
  (bind _wbp_journalwidget (Variables|/Game/UI/HUD/WBP_GeneralUI.WBP_GeneralUI_C|GetWBP_JournalWidget _generalui))
  ;[1 1 1] JournalToggle
  (:Started
    (Utilities|ToggleWidget _wbp_journalwidget false false
      (:WidgetEnabled
        _)
      (:WIdgetDisabled
        _))
    (Default|CheckJournalOpen _wbp_journalwidget)
    (UserInterface|Animation|PlayAnimation _wbp_journalwidget (Variables|/Game/Journal/WBP_JournalWidget.WBP_JournalWidget_C|GetOpenJournal _wbp_journalwidget) 0.0 1 "Forward" 1.0 false)))

(event Input|EnhancedActionEvents|EnhancedInputActionIA_Research
  (params (ActionValue :type Boolean) (ElapsedSeconds :type Float%20%28double-precision%29) (TriggeredSeconds :type Float%20%28double-precision%29) (InputAction :type Input%20Action%20Object%20Reference :default "/Game/Input/MenuControls/IA_Research.IA_Research"))
  ;[1 1 1] ResearchToggle
  (:Started
    (if (Variables|States|GetCanResearch)
      (Utilities|ToggleWidget (Variables|/Game/UI/HUD/WBP_GeneralUI.WBP_GeneralUI_C|GetResearchWindow (Variables|References|GetGeneralUI)) true true))))

(event Input|EnhancedActionEvents|EnhancedInputActionIA_Contact
  (params (ActionValue :type Boolean) (ElapsedSeconds :type Float%20%28double-precision%29) (TriggeredSeconds :type Float%20%28double-precision%29) (InputAction :type Input%20Action%20Object%20Reference :default "/Game/Input/MenuControls/IA_Contact.IA_Contact"))
  (bind _generalui (Variables|References|GetGeneralUI))
  (bind _wbp_gamehud (Variables|/Game/UI/HUD/WBP_GeneralUI.WBP_GeneralUI_C|GetWBP_GameHUD _generalui))
  (bind _communicationnotification (Variables|/Game/UI/HUD/WBP_GameHUD.WBP_GameHUD_C|GetCommunicationNotification _wbp_gamehud))
  ;[1 1 1] CommunicateWindowToggle
  (:Started
    (Utilities|ToggleWidget (Variables|/Game/UI/HUD/WBP_GeneralUI.WBP_GeneralUI_C|GetWBP_dialogueWindow _generalui) true true
      (:WidgetEnabled
        (if (Widget|IsVisible _communicationnotification)
          (Widget|SetVisibility _communicationnotification "Hidden")
          (Class|UserWidget|StopAnimation _wbp_gamehud (Variables|/Game/UI/HUD/WBP_GameHUD.WBP_GameHUD_C|GetCommunicationNotificatio _wbp_gamehud)))))))

(event Input|EnhancedActionEvents|EnhancedInputActionIA_Pause
  (params (ActionValue :type Boolean) (ElapsedSeconds :type Float%20%28double-precision%29) (TriggeredSeconds :type Float%20%28double-precision%29) (InputAction :type Input%20Action%20Object%20Reference :default "/Game/Input/MenuControls/IA_Pause.IA_Pause"))
  ;[1 1 1] Time
)

(event Input|EnhancedActionEvents|EnhancedInputActionIA_Speed1
  (params (ActionValue :type Boolean) (ElapsedSeconds :type Float%20%28double-precision%29) (TriggeredSeconds :type Float%20%28double-precision%29) (InputAction :type Input%20Action%20Object%20Reference :default "/Game/Input/MenuControls/IA_Speed1.IA_Speed1"))
  ;[1 1 1] Time
  (:Started
    (CallFunction|SetTimeSpeed (Variables|SpeedControl|GetSpeedOne))
    (Variables|Default|SetIsTimeFrozen false)))

(event Input|EnhancedActionEvents|EnhancedInputActionIA_Speed2
  (params (ActionValue :type Boolean) (ElapsedSeconds :type Float%20%28double-precision%29) (TriggeredSeconds :type Float%20%28double-precision%29) (InputAction :type Input%20Action%20Object%20Reference :default "/Game/Input/MenuControls/IA_Speed2.IA_Speed2"))
  ;[1 1 1] Time
  (:Started
    (CallFunction|SetTimeSpeed (Variables|SpeedControl|GetSpeedTwo))
    (Variables|Default|SetIsTimeFrozen false)))

(event Input|EnhancedActionEvents|EnhancedInputActionIA_Speed3
  (params (ActionValue :type Boolean) (ElapsedSeconds :type Float%20%28double-precision%29) (TriggeredSeconds :type Float%20%28double-precision%29) (InputAction :type Input%20Action%20Object%20Reference :default "/Game/Input/MenuControls/IA_Speed3.IA_Speed3"))
  ;[1 1 1] Time
  (:Started
    (CallFunction|SetTimeSpeed (Variables|SpeedControl|GetSpeedThree))
    (Variables|Default|SetIsTimeFrozen false)))

(event Input|EnhancedActionEvents|EnhancedInputActionIA_Map
  (params (ActionValue :type Boolean) (ElapsedSeconds :type Float%20%28double-precision%29) (TriggeredSeconds :type Float%20%28double-precision%29) (InputAction :type Input%20Action%20Object%20Reference :default "/Game/Input/MenuControls/IA_Map.IA_Map"))
  ;[1 1 1] MapToggle
  (:Started
    (Utilities|ToggleWidget (Variables|/Game/UI/HUD/WBP_GeneralUI.WBP_GeneralUI_C|GetWBP_Map (Variables|References|GetGeneralUI)) true true)))

(event Input|EnhancedActionEvents|EnhancedInputActionIA_Exit
  (params (ActionValue :type Boolean) (ElapsedSeconds :type Float%20%28double-precision%29) (TriggeredSeconds :type Float%20%28double-precision%29) (InputAction :type Input%20Action%20Object%20Reference :default "/Game/Input/MenuControls/IA_Exit.IA_Exit"))
  (bind _generalui (Variables|References|GetGeneralUI))
  (bind _wbp_menuhud (Variables|/Game/UI/HUD/WBP_GeneralUI.WBP_GeneralUI_C|GetWBP_MenuHUD _generalui))
  (bind _widgetswitcher (Variables|/Game/UI/HUD/WBP_GeneralUI.WBP_GeneralUI_C|GetWidgetSwitcher _generalui))
  ;[1 1 1] Open Menu Hud
  (:Started
    (if (== (Class|WidgetSwitcher|GetActiveWidgetIndex _widgetswitcher) 0)
      (Utilities|ToggleWidget _wbp_menuhud false false
        (:WidgetEnabled
          (Default|SetColorMenu _wbp_menuhud)))
      (else
        (Class|WidgetSwitcher|SetActiveWidgetIndex _widgetswitcher)
        (Input|AddMappingContext (PlayerController|LocalPlayerSubsystems|GetEnhancedInputLocalPlayerSubsystem self) "/Game/Input/Movement/IMC_Spectating.IMC_Spectating" 0 "(bIgnoreAllPressedKeysUntilRelease=True,bForceImmediately=False,bNotifyUserSettings=False)")
        (Variables|States|SetCanClick true)))))

(event EventBeginPlay
  (Utilities|FlowControl|Sequence
    (:then_0
      ;[1 1 1] References & Objects initializations
      (Utilities|FlowControl|Sequence
        (:then_0
          (bind _returnvalue (Actor|GetActorOfClass "/Game/Core/Player/BP_SpectatorPawn.BP_SpectatorPawn_C"))
          (Variables|References|SetBP_spectator _returnvalue))
        (:then_1
          (bind _returnvalue_2 (Actor|GetActorOfClass "/Game/VO/BP_VOManager.BP_VOManager_C"))
          (Variables|Default|SetVOManager _returnvalue_2))
        (:then_2
          (bind _returnvalue_3 (Actor|GetActorOfClass "/Game/Tasks/BP_TasksSystem.BP_TasksSystem_C"))
          (Variables|References|SetTaskSystem _returnvalue_3))
        (:then_3
          (bind _returnvalue_4 (Actor|GetActorOfClass "/Game/Core/Blueprints/TimeManager.TimeManager_C"))
          (Variables|References|SetTimeManager _returnvalue_4))
        (:then_4
          (bind _returnvalue_5 (Actor|GetActorOfClass "/Game/Core/Blueprints/BP_BaseSurrounding.BP_BaseSurrounding_C"))
          (Variables|References|SetBaseSurrounding _returnvalue_5))
        (:then_5
          (bind _returnvalue_6 (Actor|GetActorOfClass "/Game/Core/Blueprints/BP_Ship.BP_Ship_C"))
          (Variables|References|SetSpaceShip _returnvalue_6))
        (:then_6
          (bind _returnvalue_7 (Actor|GetActorOfClass "/Game/Researches/BP_ResearchManager.BP_ResearchManager_C"))
          (Variables|References|SetResearchManager _returnvalue_7))
        (:then_7
          (bind _returnvalue_8 (Actor|GetActorOfClass "/Game/Core/Blueprints/BP_MainBlackHole.BP_MainBlackHole_C"))
          (Variables|References|SetBlackHole _returnvalue_8))
        (:then_8
          (bind _returnvalue_9 (Actor|GetActorOfClass "/Game/UI/FractionsMenu/Dialogues/BP_DialoguSystem.BP_DialoguSystem_C"))
          (Variables|Default|SetDialogueSystem _returnvalue_9))
        (:then_9
          (bind _returnvalue_10 (UserInterface|CreateWidget "/Game/UI/HUD/WBP_GeneralUI.WBP_GeneralUI_C"))
          (bind _output_get (Variables|References|SetGeneralUI _returnvalue_10))
          (UserInterface|Viewport|AddtoViewport _output_get 0))))
    (:then_1
      ;[1 1 1] Load Saved Game
      (bind _returnvalue_11 (Game|GetCurrentLevelName true))
      (bind _output_get_2 (Variables|Default|SetCurrentLevelName _returnvalue_11))
      (if (Utilities|Enum|Equal(Enum) _output_get_2 "GameUniverse")
        _
        (else
          _))
      (bind _asbp_space_game_instance (Utilities|Casting|CastToBP_SpaceGameInstance (Game|GetGameInstance)))
      (EventDispatchers|BindEventtoOnSaveLoaded _asbp_space_game_instance (delegate Custom|LoadSaveData))
      (Default|FinishLevelLoaded _asbp_space_game_instance))
    (:then_2
      ;[1 1 1] Controls Binding
      (Variables|Default|SetbShowMouseCursor true)
      (Utilities|FlowControl|Sequence
        (:then_1
          (EventDispatchers|BindEventtoOnClicked (Variables|/Game/UI/HUD/WBP_GameHUD.WBP_GameHUD_C|GetJournalButton (Variables|/Game/UI/HUD/WBP_GeneralUI.WBP_GeneralUI_C|GetWBP_GameHUD (Variables|References|GetGeneralUI))) (delegate Custom|ToggleJournal))
          (EventDispatchers|BindEventtoOnClicked (Variables|/Game/UI/HUD/WBP_GameHUD.WBP_GameHUD_C|GetResearchButton (Variables|/Game/UI/HUD/WBP_GeneralUI.WBP_GeneralUI_C|GetWBP_GameHUD (Variables|References|GetGeneralUI))) (delegate Custom|ToggleResearchMenu))
          (EventDispatchers|BindEventtoOnClicked (Variables|/Game/UI/HUD/WBP_GameHUD.WBP_GameHUD_C|GetContactButton (Variables|/Game/UI/HUD/WBP_GeneralUI.WBP_GeneralUI_C|GetWBP_GameHUD (Variables|References|GetGeneralUI))) (delegate Custom|ToggleContact))
          (EventDispatchers|BindEventtoOnClicked (Variables|/Game/UI/HUD/WBP_GameHUD.WBP_GameHUD_C|GetMapButton (Variables|/Game/UI/HUD/WBP_GeneralUI.WBP_GeneralUI_C|GetWBP_GameHUD (Variables|References|GetGeneralUI))) (delegate Custom|MapToggle))
          (EventDispatchers|BindEventtoOnClicked (Variables|/Game/UI/HUD/WBP_GameHUD.WBP_GameHUD_C|GetBuildButton (Variables|/Game/UI/HUD/WBP_GeneralUI.WBP_GeneralUI_C|GetWBP_GameHUD (Variables|References|GetGeneralUI))) (delegate Custom|ToggleBuildMenu)))))
    (:then_3
      ;[1 1 1] States
      (EventDispatchers|BindEventtoExtractionStatusChange (delegate Custom|SetUpExtraction))
      (EventDispatchers|BindEventtoResearchStatusChange (delegate Custom|SetResearchStatus))
      (EventDispatchers|BindEventtoClosetoBaseStatusChange (delegate Custom|SetIsCloseToBaseStatus)))
    (:then_4
      ;[1 1 1] Time
      (EventDispatchers|BindEventtoOnClicked (Variables|/Game/UI/HUD/WBP_GameHUD.WBP_GameHUD_C|GetPauseButton (Variables|/Game/UI/HUD/WBP_GeneralUI.WBP_GeneralUI_C|GetWBP_GameHUD (Variables|References|GetGeneralUI))) (delegate Custom|PauseTime))
      (EventDispatchers|BindEventtoOnClicked (Variables|/Game/UI/HUD/WBP_GameHUD.WBP_GameHUD_C|GetSpeedOneButton (Variables|/Game/UI/HUD/WBP_GeneralUI.WBP_GeneralUI_C|GetWBP_GameHUD (Variables|References|GetGeneralUI))) (delegate Custom|Speed1))
      (EventDispatchers|BindEventtoOnClicked (Variables|/Game/UI/HUD/WBP_GameHUD.WBP_GameHUD_C|GetSpeedTwoButton (Variables|/Game/UI/HUD/WBP_GeneralUI.WBP_GeneralUI_C|GetWBP_GameHUD (Variables|References|GetGeneralUI))) (delegate Custom|Speed2))
      (EventDispatchers|BindEventtoOnClicked (Variables|/Game/UI/HUD/WBP_GameHUD.WBP_GameHUD_C|GetSpeedThreeButton (Variables|/Game/UI/HUD/WBP_GeneralUI.WBP_GeneralUI_C|GetWBP_GameHUD (Variables|References|GetGeneralUI))) (delegate Custom|Speed3)))
    (:then_5
      ;[1 1 1] CVARS
      (DataDrivenCVar|BindEventtoOnDataDrivenCVarDelegate (|DataDrivenCVarEngineSubsystem) (delegate Custom|Command)))))

(event Input|KeyboardEvents|F12
  (params (Key :type Key%20Structure :default "None"))
  ;[1 1 1] Maxwell
  (:Pressed
    (Default|ActivateMaxwell (Variables|References|GetBlackHole))))

(fn ConstructionScript)

(fn EnableSaving
  (params (bIsEnabled :type Boolean))
  (Widget|SetIsEnabled (Variables|/Game/UI/Menu/WBP_MenuHUD.WBP_MenuHUD_C|GetSaveGame (Variables|/Game/UI/HUD/WBP_GeneralUI.WBP_GeneralUI_C|GetWBP_MenuHUD (Variables|References|GetGeneralUI))) bIsEnabled))