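; Base building Blueprint for a space game that spins, lights itself from the black hole's state and can be highlighted.
; A looping timer yaws the Scene component in proportion to black hole mass and time speed, pausing while time is frozen.
; BaseSurrounding events update child lights: intensity follows current-to-initial mass ratio, color comes from a Material Parameter Collection.
; HighlightBuilding toggles a scalar material parameter across Scene's child static meshes.
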(event Custom|RotateBase
  (bind _scene (Variables|Default|GetScene))
  (bind _space_controller (Variables|Default|GetSpace%20Controller))
  (bind _blackhole (Variables|/Game/Core/Player/BP_SpacePlayerController.BP_SpacePlayerController_C|GetBlackHole _space_controller))
  (bind _relativerotation (Variables|/Script/Engine.SceneComponent|GetRelativeRotation _scene))
  (if (not (Variables|/Script/DarkEraProject.SpacePlayerController|GetIsTimeFrozen _space_controller))
    (Utilities|IsValid _blackhole
      (:Is%20Valid
        (Transformation|SetRelativeRotation _scene (Math|Rotator|MakeRotator (.roll _relativerotation) (.pitch _relativerotation) (+ (.yaw _relativerotation) (* 0.01 (/ (Variables|/Game/Core/Blueprints/BP_MainBlackHole.BP_MainBlackHole_C|GetCurrentMass _blackhole) 1e+01) (Variables|/Script/DarkEraProject.SpacePlayerController|GettimeSpeed _space_controller)))) false false)))))

(event Custom|SetLightColor
  ;[1 1 1] Lightning
  (bind _returnvalue (Rendering|Material|GetVectorParameterValue "/Game/Materials/MPC_Collection.MPC_Collection" "color" :!class /Script/Engine.KismetMaterialLibrary))
  (for _array_element (Components|GetChildrenComponents (Variables|Default|GetLights) false)
    (bind _aslight_component (Utilities|Casting|CastToLightComponent _array_element))
    (Rendering|Components|Light|SetLightColor _aslight_component _returnvalue true)))

(event Custom|HighlightBuilding
  (params (Enabled :type Boolean))
  (if Enabled
    (Variables|Default|SetHighlightValue 1.0)
    (else
      (Variables|Default|SetHighlightValue 0.0)))
  (for _array_element (Components|GetChildrenComponents (Variables|Default|GetScene) true)
    (bind _asstatic_mesh_component (Utilities|Casting|CastToStaticMeshComponent _array_element))
    (Rendering|Material|SetScalarParameterValueonMaterials _asstatic_mesh_component "HighlightEnabled" (Variables|Default|GetHighlightValue))))

(event Custom|SetLocalIntensity
  (bind _space_controller (Variables|Default|GetSpace%20Controller))
  (bind _blackhole (Variables|/Game/Core/Player/BP_SpacePlayerController.BP_SpacePlayerController_C|GetBlackHole _space_controller))
  ;[1 1 1] Lightning
  (Utilities|IsValid _blackhole
    (:Is%20Valid
      (for _array_element (Components|GetChildrenComponents (Variables|Default|GetLights) false)
        (bind _aslight_component (Utilities|Casting|CastToLightComponent _array_element))
        (Rendering|Components|Light|SetIntensity _aslight_component (* (/ (Variables|/Game/Core/Blueprints/BP_MainBlackHole.BP_MainBlackHole_C|GetCurrentMass _blackhole) (Variables|/Game/Core/Blueprints/BP_MainBlackHole.BP_MainBlackHole_C|GetInitialMass _blackhole)) 1e+01))))))

(event EventBeginPlay
  (bind _asbp_space_player_controller (Utilities|Casting|CastToBP_SpacePlayerController (Game|GetPlayerController 0)))
  (Variables|Default|SetSpace%20Controller _asbp_space_player_controller)
  (Utilities|Time|SetTimerbyEvent (delegate Custom|RotateBase) 0.01 true)
  ;[1 1 1] Lightning
  (EventDispatchers|BindEventtoSetGlobalLight (Variables|/Game/Core/Player/BP_SpacePlayerController.BP_SpacePlayerController_C|GetBaseSurrounding (Variables|Default|GetSpace%20Controller)) (delegate Custom|SetLocalIntensity))
  (CallFunction|SetLocalIntensity)
  (EventDispatchers|BindEventtoSetGlobalColor (Variables|/Game/Core/Player/BP_SpacePlayerController.BP_SpacePlayerController_C|GetBaseSurrounding (Variables|Default|GetSpace%20Controller)) (delegate Custom|SetLightColor))
  (CallFunction|SetLightColor))

(fn ConstructionScript)