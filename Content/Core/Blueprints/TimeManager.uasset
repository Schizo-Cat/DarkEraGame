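; TimeManager is a Blueprint that advances game time and counts decades for the HUD timeline.
; On BeginPlay it caches the space player controller, seeds CurrentTime from the current decade and starts a looping timer.
; Each tick adds speed-scaled time while time is running and not frozen by the controller.
; Decade progress fills the HUD bar against a hardcoded 100-unit span, then increments the decade and updates its labels.
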(event Custom|TimeSet
  (bind _currentdecade (Variables|Time|GetCurrentDecade))
  (bind _spacecontroller (Variables|Components|GetSpaceController))
  (bind _generalui (Variables|/Game/Core/Player/BP_SpacePlayerController.BP_SpacePlayerController_C|GetGeneralUI _spacecontroller))
  (bind _wbp_gamehud (Variables|/Game/UI/HUD/WBP_GeneralUI.WBP_GeneralUI_C|GetWBP_GameHUD _generalui))
  (bind _timeline (Variables|/Game/UI/HUD/WBP_GameHUD.WBP_GameHUD_C|GetTimeLine _wbp_gamehud))
  (if (Variables|Default|GetIsTimeGoing)
    (if (not (Variables|/Script/DarkEraProject.SpacePlayerController|GetIsTimeFrozen (Variables|Components|GetSpaceController)))
      (bind _output_get (Variables|Time|SetCurrentTime (+ (* 0.01 (Variables|Important|GetTimeSpeedMultiplier)) (Variables|Time|GetCurrentTime))))
      (Progress|SetPercent _timeline (/ (- _output_get (* (Variables|Important|GetDecadeLength) (Variables|Time|GetCurrentDecade))) 1e+02))
      (if (>= (/ (- _output_get (* (Variables|Important|GetDecadeLength) (Variables|Time|GetCurrentDecade))) 1e+02) 1.0)
        (Math|Integer|IncrementInt _currentdecade
          (:%20%20
            (Rendering|Components|TextRender|SetText (Variables|/Game/UI/HUD/WBP_GameHUD.WBP_GameHUD_C|GetCurrentDecadeText _wbp_gamehud) (Utilities|Text|ToText(Integer) _currentdecade))
            (Rendering|Components|TextRender|SetText (Variables|/Game/UI/HUD/WBP_GameHUD.WBP_GameHUD_C|GetNextDecadeText _wbp_gamehud) (Utilities|Text|ToText(Integer) (+ _currentdecade 1)))
            (Progress|SetPercent _timeline 0.0)))))))

(event EventBeginPlay
  (bind _asbp_space_player_controller (Utilities|Casting|CastToBP_SpacePlayerController (Game|GetPlayerController 0)))
  (Variables|Components|SetSpaceController _asbp_space_player_controller)
  (Variables|Time|SetCurrentTime (* (Variables|Important|GetDecadeLength) (Variables|Time|GetCurrentDecade)))
  (bind _returnvalue (Utilities|Time|SetTimerbyEvent (delegate Custom|TimeSet) 0.1 true))
  (Variables|Default|SetTimerSetTime _returnvalue))

(fn ConstructionScript)