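; Player ship/base that handles travel targets, resource extraction, combat mode and singularity travel.
; FlyToObject spawns a randomly placed target with quest pointer, attached to BP_Environment; a proximity timer opens the extraction minigame.
; Extraction feeds mass to the black hole, while EndFight swaps the enemy for an extractable body.
; Looping timers drive health-bar billboarding, mass-scaled base spin, turning and the singularity camera blend; module visibility is toggled by events.
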(event Custom|RotateBase
  (bind _spacecontroller (Variables|Default|GetSpaceController))
  (bind _blackhole (Variables|/Game/Core/Player/BP_SpacePlayerController.BP_SpacePlayerController_C|GetBlackHole _spacecontroller))
  ;[1 1 1] Rotate Base
  (if (not (Variables|/Script/DarkEraProject.SpacePlayerController|GetIsTimeFrozen _spacecontroller))
    (Utilities|IsValid _blackhole
      (:Is%20Valid
        (Transformation|AddLocalRotation (Variables|Default|GetWholeBaseRoot) (Math|Rotator|MakeRotator 0.0 0.0 (* 0.01 (/ (Variables|/Game/Core/Blueprints/BP_MainBlackHole.BP_MainBlackHole_C|GetCurrentMass _blackhole) 1e+01) (Variables|/Script/DarkEraProject.SpacePlayerController|GettimeSpeed _spacecontroller))) false false)
        (Transformation|SetActorRotation (Variables|/Game/Core/Player/BP_SpacePlayerController.BP_SpacePlayerController_C|GetBaseSurrounding (Variables|Default|GetSpaceController)) (Transformation|GetWorldRotation (Variables|Default|GetRotateBaseY)))))))

(event Custom|ZoomOut
  ;[1 1 1] ZoomTo singularity
)

(event Custom|RotateToSingularity
  (bind _spacecontroller (Variables|Default|GetSpaceController))
  (bind _bp_spectator (Variables|/Game/Core/Player/BP_SpacePlayerController.BP_SpacePlayerController_C|GetBP_spectator _spacecontroller))
  (bind _singularityoffset (Variables|/Game/Core/Player/BP_SpacePlayerController.BP_SpacePlayerController_C|GetSingularityOffset _spacecontroller))
  (bind _returnvalue (- "" _singularityoffset))
  (bind _x (Math|Vector|BreakVector _returnvalue))
  ;[1 1 1] SinglarityTravel
  (bind _output_get (Variables|Travelling|SetSingularityClose (+ (Variables|Travelling|GetSingularityClose) 0.01)))
  (Transformation|SetActorLocation _bp_spectator (Math|Vector|MakeVector (Math|Float|Lerp _x 0.0 _output_get) 0.0 0.0) false false)
  (Variables|/Script/Engine.SpringArmComponent|SetSocketOffset (Variables|/Game/Core/Player/BP_SpectatorPawn.BP_SpectatorPawn_C|GetSpringArm _bp_spectator) (Math|Vector|MakeVector (Math|Float|Lerp 0.0 _x (Variables|Travelling|GetSingularityClose)) 0.0 0.0))
  (if (>= (Variables|Travelling|GetSingularityClose) 1.0)
    _))

(event Custom|FlyObjectToBase
  (bind _targetflyobject (Variables|Travelling|GetTargetFlyObject))
  ;[1 1 1] Fly To object
  (Utilities|IsValid _targetflyobject
    (:Is%20Valid
      (Utilities|IsValid (Variables|Default|GetExtractMinigameWidget)
        (:Is%20Not%20Valid
          (if (<= (Transformation|GetDistanceTo self _targetflyobject) 3.5e+02)
            (if (Variables|/Game/Core/Player/BP_SpacePlayerController.BP_SpacePlayerController_C|GetCanExtract (Variables|Default|GetSpaceController))
              (Utilities|FlowControl|Sequence
                (:then_0
                  (Utilities|Time|InvalidateTimerHandle (Variables|Travelling|GetMoveToTimer))
                  (Widget|RemovefromParent (Variables|Default|GetQuestPointer))
                  (Variables|Default|SetQuestPointer 0))
                (:then_1
                  (bind _asbp_space_body_base (Utilities|Casting|CastToBP_SpaceBodyBase _targetflyobject))
                  (bind _returnvalue (UserInterface|CreateWidget "/Game/UI/Minigames/WBP_ExtractionMinigame.WBP_ExtractionMinigame_C" 0 (Variables|/Game/Core/Blueprints/ExtructableObjects/BP_SpaceBodyBase.BP_SpaceBodyBase_C|GetGravitationalDifficulty _asbp_space_body_base) (Variables|/Game/Core/Blueprints/ExtructableObjects/BP_SpaceBodyBase.BP_SpaceBodyBase_C|GetGravitationalSize _asbp_space_body_base)))
                  (bind _output_get (Variables|Default|SetExtractMinigameWidget _returnvalue))
                  (UserInterface|Viewport|AddtoViewport _output_get 0)
                  (Input|SetInputModeGameandUI (Variables|Default|GetSpaceController) 0 "DoNotLock" true false)
                  (Variables|/Game/Core/Player/BP_SpectatorPawn.BP_SpectatorPawn_C|SetEnabledMovement (Variables|/Game/Core/Player/BP_SpacePlayerController.BP_SpacePlayerController_C|GetBP_spectator (Variables|Default|GetSpaceController)) false)
                  (Utilities|Time|SetTimerbyEvent (delegate Custom|ShakeCamera) 1.0 true)
                  (CallFunction|RotateBasetoTarget (Math|Rotator|FindLookatRotation (Transformation|GetActorLocation) (Transformation|GetActorLocation (Variables|Travelling|GetTargetFlyObject))) 2.0))))))))))

(event Custom|ShakeCamera
  ;[1 1 1] Fly To object
  (Game|Feedback|ClientStartCameraShake (Variables|Default|GetSpaceController) "/Game/Core/BP_CameraShake_Dodge.BP_CameraShake_Dodge_C" 1.0 "CameraLocal" "0, 0, 0"))

(event Custom|RotateBaseToTarget
  (params (TargetRotation :type Rotator) (RotationTime :type Float%20%28double-precision%29))
  ;[1 1 1] RotationMethod
  (bind _returnvalue (Utilities|Time|SetTimerbyEvent (delegate Custom|RotateBack) 0.01 true))
  (Variables|Travelling|SetBaseRotationTimer _returnvalue))

(event Custom|TurnLaser
  (params (bNewVisibility :type Boolean))
  ;[1 1 1] TurnLaser
  (Rendering|SetVisibility (Variables|Default|GetCosmicLaser) bNewVisibility true))

(event Custom|TurnMatter
  (params (bNewVisibility :type Boolean))
  ;[1 1 1] TurnAntimatter
  (Rendering|SetVisibility (Variables|Default|GetAntimatterGuns) bNewVisibility true))

(event Custom|SetTarget
  ;[1 1 1] trigger fly
  (Variables|Travelling|SetTargetRotation (Math|Rotator|FindLookatRotation (Transformation|GetWorldLocation (Variables|Transformation|GetRootComponent)) (Transformation|GetActorLocation (Variables|Travelling|GetTargetFlyObject)))))

(event Custom|ExtractObject
  (bind _spacecontroller (Variables|Default|GetSpaceController))
  (bind _blackhole (Variables|/Game/Core/Player/BP_SpacePlayerController.BP_SpacePlayerController_C|GetBlackHole _spacecontroller))
  ;[1 1 1] ExtractObject
  (bind _asbp_space_body_base (Utilities|Casting|CastToBP_SpaceBodyBase (Variables|Travelling|GetTargetFlyObject)))
  (bind _output_get (Variables|Travelling|SetResourceObject _asbp_space_body_base))
  (Variables|/Game/Core/Blueprints/BP_MainBlackHole.BP_MainBlackHole_C|SetCurrentMass _blackhole (+ (Variables|/Game/Core/Blueprints/ExtructableObjects/BP_SpaceBodyBase.BP_SpaceBodyBase_C|GetMass _output_get) (Variables|/Game/Core/Blueprints/BP_MainBlackHole.BP_MainBlackHole_C|GetCurrentMass _blackhole)))
  ;;[0 0.979 1] Journal entry add(if any)
  (Utilities|IsValid (.DataTable (Utilities|Struct|BreakDataTableRowHandle (Variables|/Game/Core/Blueprints/ExtructableObjects/BP_SpaceBodyBase.BP_SpaceBodyBase_C|GetEntry _output_get)))
    (:Is%20Valid
      (bind _returnvalue (Utilities|GetDataTableRow (.DataTable (Utilities|Struct|BreakDataTableRowHandle (Variables|/Game/Core/Blueprints/ExtructableObjects/BP_SpaceBodyBase.BP_SpaceBodyBase_C|GetEntry _output_get))) (.RowName (Utilities|Struct|BreakDataTableRowHandle (Variables|/Game/Core/Blueprints/ExtructableObjects/BP_SpaceBodyBase.BP_SpaceBodyBase_C|GetEntry _output_get))))
        (:then
          (Default|AddEntry (Variables|/Game/UI/HUD/WBP_GeneralUI.WBP_GeneralUI_C|GetWBP_JournalWidget (Variables|/Game/Core/Player/BP_SpacePlayerController.BP_SpacePlayerController_C|GetGeneralUI (Variables|Default|GetSpaceController))) _returnvalue))
        (:RowNotFound
          _)))
    (:Is%20Not%20Valid
      _))
  (Utilities|IsValid (Variables|Travelling|GetResourceObject)
    (:Is%20Valid
      (Default|CallOnObjectCollected (Variables|Travelling|GetResourceObject))
      (Actor|DestroyActor (Variables|Travelling|GetResourceObject)))
    (:Is%20Not%20Valid
      _))
  (Variables|Travelling|SetTargetFlyObject 0)
  (CallFunction|RotateBasetoTarget "90.000000,0.000000,0.000000" 3.0))

(event Custom|TurnWarpDriver
  (params (bNewVisibility :type Boolean))
  ;[1 1 1] Drivers
  (Rendering|SetVisibility (Variables|Default|GetEngine) (not bNewVisibility) true)
  (Rendering|SetVisibility (Variables|Default|GetWarpDrive) bNewVisibility true))

(event Custom|TurnExtractor
  (params (bNewVisibility :type Boolean))
  ;[1 1 1] extractor
  (Rendering|SetVisibility (Variables|Default|GetExtractorComp) bNewVisibility true))

(event Custom|RotateBack
  (bind _spacecontroller (Variables|Default|GetSpaceController))
  (bind _timespeed (Variables|/Script/DarkEraProject.SpacePlayerController|GettimeSpeed _spacecontroller))
  ;[1 1 1] RotationMethod
  (if (not (Variables|/Script/DarkEraProject.SpacePlayerController|GetIsTimeFrozen (Variables|Default|GetSpaceController)))
    (Variables|Travelling|SetRotationProgress (+ (Variables|Travelling|GetRotationProgress) (* 0.01 _timespeed)))
    (Transformation|SetWorldRotation (Variables|/Script/Engine.Actor|GetRootComponent (Variables|/Game/Core/Player/BP_SpacePlayerController.BP_SpacePlayerController_C|GetBaseSurrounding (Variables|Default|GetSpaceController))) (Math|Interpolation|RInterpTo (Transformation|GetWorldRotation (Variables|Transformation|GetRootComponent)) (stale Custom|RotateBaseToTarget TargetRotation) 0.01 _timespeed) false false)
    (if (>= (Variables|Travelling|GetRotationProgress) (stale Custom|RotateBaseToTarget RotationTime))
      (Utilities|Time|ClearandInvalidateTimerbyHandle (Variables|Travelling|GetBaseRotationTimer))
      (Utilities|FlowControl|Sequence
        (:then_1
          (Transformation|SetWorldRotation (Variables|Transformation|GetRootComponent) (stale Custom|RotateBaseToTarget TargetRotation) false false)
          (Variables|/Game/Core/Player/BP_SpectatorPawn.BP_SpectatorPawn_C|SetEnabledMovement (Variables|/Game/Core/Player/BP_SpacePlayerController.BP_SpacePlayerController_C|GetBP_spectator (Variables|Default|GetSpaceController)) true))))))

(event Custom|FlyToObject
  (params (ObjectClass :type ResourcesType%20Enum :default "NewEnumerator0"))
  (bind _randommax (Variables|Travelling|GetRandomMax))
  (bind _randommin (Variables|Travelling|GetRandomMin))
  ;[1 1 1] trigger fly
  (Utilities|IsValid (Variables|Travelling|GetTargetFlyObject)
    (:Is%20Not%20Valid
      (bind _output_get (Variables|Travelling|SetObjectClass ObjectClass))
      (bind _returnvalue (Game|SpawnActorfromClass (Utilities|Select :Index _output_get :NewEnumerator0 "/Game/Core/Blueprints/ExtructableObjects/BP_NeutronStar.BP_NeutronStar_C" :NewEnumerator1 "/Game/Core/Blueprints/BP_SingularityProject.BP_SingularityProject_C" :NewEnumerator2 "/Game/Core/Blueprints/ExtructableObjects/BP_BlackHole.BP_BlackHole_C" :NewEnumerator3 "/Game/Core/Blueprints/ExtructableObjects/BP_QuestRuins.BP_QuestRuins_C" :NewEnumerator4 "/Game/Core/Blueprints/FractionObjects/BP_DestructionBase.BP_DestructionBase_C") (Math|Transform|MakeTransform (Math|Vector|MakeVector (Math|Conversions|ToFloat(Integer) (Math|Random|RandomIntegerinRange _randommin _randommax)) (Math|Conversions|ToFloat(Integer) (Math|Random|RandomIntegerinRange _randommin _randommax)) (Math|Conversions|ToFloat(Integer) (Math|Random|RandomIntegerinRange _randommin _randommax)))) "Undefined" "MultiplyWithRoot" 0 0))
      (Variables|Travelling|SetTargetFlyObject _returnvalue)
      (switch Utilities|FlowControl|Switch|SwitchonResourcesType (Variables|Travelling|GetObjectClass)
        (:NewEnumerator0
          (Variables|Travelling|SetDistance 1.5e+02 :!label _label)
          (CallFunction|SetTarget :!label _label_2)
          (bind _returnvalue_2 (UserInterface|CreateWidget "/Game/UI/HUD/WBP_QuestPointer.WBP_QuestPointer_C" 0 (Variables|Travelling|GetTargetFlyObject)))
          (Variables|Default|SetQuestPointer _returnvalue_2)
          (UserInterface|Viewport|AddtoViewport _returnvalue_2 0)
          (bind _returnvalue_3 (Actor|GetActorOfClass "/Game/Blueprints/BP_Environment.BP_Environment_C"))
          (Utilities|IsValid _returnvalue_3
            (:Is%20Valid
              (Transformation|AttachActorToActor (Variables|Travelling|GetTargetFlyObject) _returnvalue_3 "None" "KeepRelative" "KeepRelative" "KeepRelative" true)
              (bind _returnvalue_4 (Utilities|Time|SetTimerbyEvent (delegate Custom|FlyCheck) 0.1 true))
              (Variables|Travelling|SetMoveToTimer _returnvalue_4))))
        (:NewEnumerator1
          (CallFunction|TraveltoSingularity))
        (:NewEnumerator2
          (goto _label))
        (:NewEnumerator3
          (goto _label))
        (:NewEnumerator4
          (Variables|Travelling|SetDistance 3e+02)
          (goto _label_2))))))

(event Custom|TravelToSingularity
  (bind _spacecontroller (Variables|Default|GetSpaceController))
  (bind _spacecontroller_2 (Variables|Default|GetSpaceController))
  (bind _spacecontroller_3 (Variables|Default|GetSpaceController))
  (bind _generalui (Variables|/Game/Core/Player/BP_SpacePlayerController.BP_SpacePlayerController_C|GetGeneralUI _spacecontroller_2))
  (bind _wbp_singularitywindow (Variables|/Game/UI/HUD/WBP_GeneralUI.WBP_GeneralUI_C|GetWBP_SingularityWindow _generalui))
  ;[1 1 1] ZoomTo singularity
  (Transformation|SetActorLocation (Variables|Travelling|GetTargetFlyObject) "0, 0, 0" false false)
  (CallFunction|SetTarget)
  (Variables|/Script/UMG.WidgetSwitcher|SetActiveWidgetIndex (Variables|/Game/UI/HUD/WBP_GeneralUI.WBP_GeneralUI_C|GetHudmenus (Variables|/Game/Core/Player/BP_SpacePlayerController.BP_SpacePlayerController_C|GetGeneralUI _spacecontroller)) 1)
  (bind _returnvalue (Actor|GetActorOfClass "/Game/Core/Blueprints/BP_SingularityProject.BP_SingularityProject_C"))
  (Variables|/Game/UI/SingularityWindow/WBP_SingularityWindow.WBP_SingularityWindow_C|SetSingularityProject _wbp_singularitywindow _returnvalue)
  (Variables|/Game/Core/Player/BP_SpacePlayerController.BP_SpacePlayerController_C|SetIsSingularityMode _spacecontroller_2 true)
  (Default|ChangeGameState _spacecontroller_2 "NewEnumerator0")
  (Widget|SetVisibility (Variables|/Game/UI/Map/WBP_Map.WBP_Map_C|GetMassiveBlackHolesOverlay (Variables|/Game/UI/HUD/WBP_GeneralUI.WBP_GeneralUI_C|GetWBP_Map _generalui)) "Visible")
  (Utilities|IsValid (Variables|/Game/UI/SingularityWindow/WBP_SingularityWindow.WBP_SingularityWindow_C|GetSingularityProject _wbp_singularitywindow)
    (:Is%20Valid
      (Default|UpdateHoleVisuals (Variables|/Game/UI/SingularityWindow/WBP_SingularityWindow.WBP_SingularityWindow_C|GetSingularityProject _wbp_singularitywindow) (Variables|/Game/Core/Player/BP_SpacePlayerController.BP_SpacePlayerController_C|GetSingularityProgression _spacecontroller_2))
      (Transformation|SetActorLocation (Variables|/Game/Core/Player/BP_SpacePlayerController.BP_SpacePlayerController_C|GetBP_spectator _spacecontroller) (Transformation|GetActorLocation) false false)
      (Variables|/Script/Engine.SpringArmComponent|SetSocketOffset (Variables|/Game/Core/Player/BP_SpectatorPawn.BP_SpectatorPawn_C|GetSpringArm (Variables|/Game/Core/Player/BP_SpacePlayerController.BP_SpacePlayerController_C|GetBP_spectator _spacecontroller_3)) (Math|Vector|MakeVector 0.0 0.0 0.0))
      (Rendering|SetActorHiddenInGame (Variables|/Game/Core/Blueprints/BP_SingularityProject.BP_SingularityProject_C|GetSingularityHole (Variables|/Game/UI/SingularityWindow/WBP_SingularityWindow.WBP_SingularityWindow_C|GetSingularityProject _wbp_singularitywindow)) false)
      (Rendering|SetActorHiddenInGame (Variables|/Game/Core/Player/BP_SpacePlayerController.BP_SpacePlayerController_C|GetBaseSurrounding _spacecontroller_3) true)
      (Utilities|Time|SetTimerbyEvent (delegate Custom|RotateToSingularity) 0.01 true))))

(event Custom|FlyCheck
  ;[1 1 1] trigger fly
  (CallFunction|FlyObjecttoBase))

(event Custom|SetRotation
  (bind _healthbar (Variables|Default|GetHealthBar))
  (bind _damagetext (Variables|Default|GetDamageText))
  (bind _spacecontroller (Variables|Default|GetSpaceController))
  (bind _bp_spectator (Variables|/Game/Core/Player/BP_SpacePlayerController.BP_SpacePlayerController_C|GetBP_spectator _spacecontroller))
  (bind _camera (Variables|/Game/Core/Player/BP_SpectatorPawn.BP_SpectatorPawn_C|GetCamera _bp_spectator))
  (bind _returnvalue (Transformation|GetWorldLocation _camera))
  ;[1 1 1] FightStuffInitialization
  (Transformation|SetWorldRotation _healthbar (Math|Rotator|FindLookatRotation (Transformation|GetWorldLocation _healthbar) _returnvalue) false false)
  (Transformation|SetWorldRotation _damagetext (Math|Rotator|FindLookatRotation (Transformation|GetWorldLocation _damagetext) _returnvalue) false false))

(event EventBeginPlay
  (bind _health (Variables|Fighting|GetHealth))
  (Variables|Default|SetInitial%20Damage%20Text%20Z%20Position (.z (Variables|/Script/Engine.SceneComponent|GetRelativeLocation (Variables|Default|GetDamageText))))
  (Effects|Particles|Trails|EndTrails (Variables|Default|GetEnemyHitParticle))
  (Components|Activation|Deactivate (Variables|Default|GetP_Flamethrower))
  (bind _asbp_space_player_controller (Utilities|Casting|CastToBP_SpacePlayerController (Game|GetPlayerController 0)))
  (Variables|Default|SetSpaceController _asbp_space_player_controller)
  (Rendering|SetVisibility (Variables|Default|GetWarpDrive) false true)
  (CallFunction|TurnLaser false)
  ;[1 1 1] Rotate Base
  (Utilities|Time|SetTimerbyEvent (delegate Custom|RotateBase) 0.01 true)
  ;[1 1 1] FightStuffInitialization
  (bind _aswbp_health_bar (Utilities|Casting|CastToWBP_HealthBar (UserInterface|GetWidget (Variables|Default|GetHealthBar))))
  (bind _output_get (Variables|Fighting|SetAs%20WBP%20Health%20Bar _aswbp_health_bar))
  (Default|SetInitialHealth _output_get (Math|Conversions|ToFloat(Integer) _health))
  (Default|UpdateHealth _output_get (Math|Conversions|ToFloat(Integer) _health))
  (bind _outrownames (DataTable|GetDataTableRowNames "/Game/Core/DataTables/DT_FractionsList.DT_FractionsList"))
  (bind _array_element (Utilities|Array|ForEachLoopwithBreak _outrownames :!label _label)
    (:LoopBody
      (bind _returnvalue (Utilities|GetDataTableRow "/Game/Core/DataTables/DT_FractionsList.DT_FractionsList" _array_element)
        (:then
          (if (Utilities|Enum|Equal(Enum) (.fraction _returnvalue) "NewEnumerator0")
            (Variables|/Game/Core/Blueprints/FractionObjects/WBP_HealthBar.WBP_HealthBar_C|SetBarColor (Variables|Fighting|GetAs%20WBP%20Health%20Bar) (Math|Conversions|ToLinearColor(Color) (.color _returnvalue)))
            (goto _label Break)))))
    (:Completed
      (Utilities|Time|SetTimerbyEvent (delegate Custom|SetRotation) 0.01 true))))

(event Custom|EndFight
  (bind _spacecontroller (Variables|Default|GetSpaceController))
  (bind _spacecontroller_2 (Variables|Default|GetSpaceController))
  (bind _generalui (Variables|/Game/Core/Player/BP_SpacePlayerController.BP_SpacePlayerController_C|GetGeneralUI _spacecontroller))
  (bind _wbp_gamehud (Variables|/Game/UI/HUD/WBP_GeneralUI.WBP_GeneralUI_C|GetWBP_GameHUD _generalui))
  (bind _extractbutton (Variables|/Game/UI/HUD/WBP_GameHUD.WBP_GameHUD_C|GetExtractButton _wbp_gamehud))
  ;[1 1 1] EndFight
  (bind _returnvalue (Utilities|GetDataTableRow "/Game/Core/DataTables/TaskList.TaskList" "E_EnemySector")
    (:then
      (Default|CompleteTask (Variables|/Game/Core/Player/BP_SpacePlayerController.BP_SpacePlayerController_C|GetTaskSystem _spacecontroller_2) _returnvalue)
      (Rendering|SetVisibility (Variables|Default|GetEnemyHitParticle) false true)
      (Variables|/Game/Core/Player/BP_SpacePlayerController.BP_SpacePlayerController_C|SetIsFightMode _spacecontroller_2 false)
      (Default|ChangeGameState _spacecontroller_2 "NewEnumerator5")
      (Widget|SetVisibility (Variables|/Game/UI/HUD/WBP_GameHUD.WBP_GameHUD_C|GetAttackHorizontalBox (Variables|/Game/UI/HUD/WBP_GeneralUI.WBP_GeneralUI_C|GetWBP_GameHUD (Variables|/Game/Core/Player/BP_SpacePlayerController.BP_SpacePlayerController_C|GetGeneralUI _spacecontroller_2))) "Hidden")
      (Rendering|SetVisibility (Variables|Default|GetHealthBar) false false)
      (bind _asbp_fraction_object_base (Utilities|Casting|CastToBP_FractionObjectBase (Variables|Travelling|GetTargetFlyObject)))
      (bind _returnvalue_2 (Game|SpawnActorfromClass (Variables|/Script/Engine.ChildActorComponent|GetChildActorClass (Variables|/Game/Core/Blueprints/FractionObjects/BP_FractionObjectBase.BP_FractionObjectBase_C|GetBP_SpaceBodyBase _asbp_fraction_object_base)) (Transformation|GetWorldTransform (Variables|/Game/Core/Blueprints/FractionObjects/BP_FractionObjectBase.BP_FractionObjectBase_C|GetBP_SpaceBodyBase _asbp_fraction_object_base)) "Undefined" "MultiplyWithRoot" 0 0))
      (bind _asbp_space_body_base (Utilities|Casting|CastToBP_SpaceBodyBase _returnvalue_2))
      (Variables|/Game/Core/Blueprints/ExtructableObjects/BP_SpaceBodyBase.BP_SpaceBodyBase_C|SetMass _asbp_space_body_base 1e+02)
      (Actor|DestroyActor _asbp_fraction_object_base)
      (Variables|Travelling|SetTargetFlyObject _asbp_space_body_base)
      (Widget|SetVisibility _extractbutton "Visible")
      (Widget|SetIsEnabled _extractbutton true))))

(event Custom|StartFight
  (bind _battlestats (Variables|Fighting|GetBattleStats))
  (bind _spacecontroller (Variables|Default|GetSpaceController))
  (bind _generalui (Variables|/Game/Core/Player/BP_SpacePlayerController.BP_SpacePlayerController_C|GetGeneralUI _spacecontroller))
  (bind _wbp_gamehud (Variables|/Game/UI/HUD/WBP_GeneralUI.WBP_GeneralUI_C|GetWBP_GameHUD _generalui))
  ;[1 1 1] StartFight
  (bind _asbp_fraction_object_base (Utilities|Casting|CastToBP_FractionObjectBase (Variables|Travelling|GetTargetFlyObject)))
  (Variables|Fighting|SetEnemyShip _asbp_fraction_object_base)
  (Variables|/Game/Core/Player/BP_SpacePlayerController.BP_SpacePlayerController_C|SetIsFightMode _spacecontroller true)
  (Default|ChangeGameState _spacecontroller "NewEnumerator1")
  (Rendering|SetVisibility (Variables|Default|GetHealthBar) true false)
  (Widget|SetVisibility (Variables|/Game/UI/HUD/WBP_GameHUD.WBP_GameHUD_C|GetAttackHorizontalBox _wbp_gamehud) "Visible")
  (Rendering|SetVisibility (Variables|Default|GetEnemyHitParticle) true true)
  (Widget|SetIsEnabled (Variables|/Game/UI/HUD/WBP_GameHUD.WBP_GameHUD_C|GetBombAttack _wbp_gamehud) (> (.bombsquantity _battlestats) 0))
  (Widget|SetIsEnabled (Variables|/Game/UI/HUD/WBP_GameHUD.WBP_GameHUD_C|GetLaserAttack _wbp_gamehud) (.haslaser _battlestats))
  (Widget|SetIsEnabled (Variables|/Game/UI/HUD/WBP_GameHUD.WBP_GameHUD_C|GetShieldActivation _wbp_gamehud) (and (.canhaveshield _battlestats) (.hasshield _battlestats))))

(fn ConstructionScript)