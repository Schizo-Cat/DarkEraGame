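; Main black hole actor whose mass drains over time, acting as a depleting resource tied to the space player controller.
; A looping timer subtracts mass unless time is frozen, draining faster during research or travel, and scales the sphere by remaining mass.
; At zero mass it hides the HUD, disables scene post-processing and destroys itself.
; ActivateMaxwell swaps two spheres for a timer-spun Maxwell mesh.
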(event Custom|CountMass
  (bind _bp_space_player_controller (Variables|Default|GetBP%20Space%20Player%20Controller))
  (bind _bp_space_player_controller_2 (Variables|Default|GetBP%20Space%20Player%20Controller))
  (if (Variables|Default|GetIsMassLosing)
    (Utilities|IsValid _bp_space_player_controller
      (:Is%20Valid
        (if (not (Variables|/Game/Core/Player/BP_SpacePlayerController.BP_SpacePlayerController_C|GetIsTimeFrozen _bp_space_player_controller))
          (if (> (Variables|Default|GetCurrentMass) 0.0)
            (Utilities|FlowControl|Sequence
              (:then_0
                (if (Variables|/Game/Researches/BP_ResearchManager.BP_ResearchManager_C|GetIsResearching (Variables|/Game/Core/Player/BP_SpacePlayerController.BP_SpacePlayerController_C|GetResearchManager _bp_space_player_controller_2))
                  (Variables|Default|SetResearchDebaffValue 1.0)
                  (else
                    (Variables|Default|SetResearchDebaffValue 0.0))))
              (:then_1
                (if (Variables|/Game/Core/Player/BP_SpacePlayerController.BP_SpacePlayerController_C|GetIstravelling _bp_space_player_controller_2)
                  (Variables|Default|SetTravellingDebaffValue 1.0)
                  (else
                    (Variables|Default|SetTravellingDebaffValue 0.0))))
              (:then_2
                (bind _output_get (Variables|Default|SetCurrentMass (- (Variables|Default|GetCurrentMass) (* (+ (Variables|Default|GetMassLossRate) (Variables|Default|GetResearchDebaffValue) (Variables|Default|GetTravellingDebaffValue)) (Variables|/Game/Core/Player/BP_SpacePlayerController.BP_SpacePlayerController_C|GetDelta%20Seconds _bp_space_player_controller)))))
                (if (< (/ _output_get (Variables|Default|GetInitialMass)) 1.5)
                  (Transformation|SetRelativeScale3D (Variables|Default|GetSphere) (Math|Conversions|ToVector(Float) (/ _output_get (Variables|Default|GetInitialMass)))))))
            (else
              (Development|ExecuteConsoleCommand "ShowHUD false" 0)
              (Development|ExecuteConsoleCommand "PostProcessAffectsScene 0" 0)
              (Actor|DestroyActor))))))))

(event Custom|ActivateMaxwell
  (Rendering|SetVisibility (Variables|Default|GetSphere2) false false)
  (Rendering|SetVisibility (Variables|Default|Getmaxwell_Maxwell) true true)
  (Utilities|Time|SetTimerbyEvent (delegate Custom|RotateMaxwell) 0.005 true))

(event Custom|RotateMaxwell
  (bind _maxwell_maxwell (Variables|Default|Getmaxwell_Maxwell))
  (bind _relativerotation (Variables|/Script/Engine.SceneComponent|GetRelativeRotation _maxwell_maxwell))
  (Utilities|IsValid self
    (:Is%20Valid
      (Transformation|SetRelativeRotation _maxwell_maxwell (Math|Rotator|MakeRotator (.roll _relativerotation) (.pitch _relativerotation) (+ (.yaw _relativerotation) 1.0)) false false))))

(event EventBeginPlay
  (bind _asbp_space_player_controller (Utilities|Casting|CastToBP_SpacePlayerController (Game|GetPlayerController 0)))
  (Variables|Default|SetBP%20Space%20Player%20Controller _asbp_space_player_controller)
  (Utilities|Time|SetTimerbyEvent (delegate Custom|CountMass) 0.01 true)
  (Variables|Default|SetCurrentMass (Variables|Default|GetInitialMass))
  (Components|Sphere|SetSphereRadius (Variables|Default|GetSphere) 0.0 false))

(fn ConstructionScript)