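; Base actor for a faction-owned enemy object that faces the player's ship and fights it in turn-based exchanges.
; BeginPlay attaches it to the spectator's environment, colors its health bar from the faction data table, and starts timers for time-scaled roll and camera-facing widgets.
; Attack applies stat-scaled damage with critical chance, then either ends the fight or counterattacks after a delay.
; Both hits drive health bars, trail particles and timer-lerped floating damage text.
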(event Custom|Attack
  (params (Damage :type Integer) (AttackType :type EAttackType%20Enum :default "NewEnumerator0"))
  (bind _returnvalue (Math|Random|RandomIntegerinRange 10 30))
  (bind _spacecontroller (Variables|Default|GetSpaceController))
  (bind _enemybattlestats (Variables|Default|GetEnemyBattleStats))
  (bind _spacecontroller_2 (Variables|Default|GetSpaceController))
  (bind _spacecontroller_3 (Variables|Default|GetSpaceController))
  (bind _spacecontroller_4 (Variables|Default|GetSpaceController))
  (bind _damagetext (Variables|Default|GetDamageText))
  (bind _returnvalue_2 (* (.damagemultiplier _enemybattlestats) 20))
  (bind _spaceship (Variables|/Game/Core/Player/BP_SpacePlayerController.BP_SpacePlayerController_C|GetSpaceShip _spacecontroller_4))
  (bind _spaceship_2 (Variables|/Game/Core/Player/BP_SpacePlayerController.BP_SpacePlayerController_C|GetSpaceShip _spacecontroller))
  (bind _spaceship_3 (Variables|/Game/Core/Player/BP_SpacePlayerController.BP_SpacePlayerController_C|GetSpaceShip _spacecontroller_2))
  (bind _spaceship_4 (Variables|/Game/Core/Player/BP_SpacePlayerController.BP_SpacePlayerController_C|GetSpaceShip _spacecontroller_3))
  (bind _relativelocation (Variables|/Script/Engine.SceneComponent|GetRelativeLocation _damagetext))
  (bind _returnvalue_3 (+ _returnvalue_2 _returnvalue))
  (bind _battlestats (Variables|/Game/Core/Blueprints/BP_Ship.BP_Ship_C|GetBattleStats _spaceship_3))
  (bind _battlestats_2 (Variables|/Game/Core/Blueprints/BP_Ship.BP_Ship_C|GetBattleStats _spaceship))
  (bind _as_wbp_health_bar (Variables|/Game/Core/Blueprints/BP_Ship.BP_Ship_C|GetAs%20WBP%20Health%20Bar _spaceship))
  (bind _damagetext_2 (Variables|/Game/Core/Blueprints/BP_Ship.BP_Ship_C|GetDamageText _spaceship_2))
  (bind _enemyhitparticle (Variables|/Game/Core/Blueprints/BP_Ship.BP_Ship_C|GetEnemyHitParticle _spaceship_4))
  (bind _selfhitparticle (Variables|/Game/Core/Blueprints/BP_Ship.BP_Ship_C|GetSelfHitParticle _spaceship_2))
  (bind _returnvalue_4 (/ _returnvalue_3 (.resistance _battlestats_2)))
  (bind _relativelocation_2 (Variables|/Script/Engine.SceneComponent|GetRelativeLocation _damagetext_2))
  ;[1 1 1] AttackLogic
  (bind _aswbp_damage_text (Utilities|Casting|CastToWBP_DamageText (UserInterface|GetWidget (Variables|/Game/Core/Blueprints/BP_Ship.BP_Ship_C|GetDamageText (Variables|/Game/Core/Player/BP_SpacePlayerController.BP_SpacePlayerController_C|GetSpaceShip (Variables|Default|GetSpaceController)))))
    (:then
      (Rendering|Components|TextRender|SetText (Variables|/Game/Core/Blueprints/FractionObjects/WBP_DamageText.WBP_DamageText_C|GetDamageText _aswbp_damage_text) ""))
    (:CastFailed
      _))
  (Widget|SetIsEnabled (Variables|/Game/UI/HUD/WBP_GameHUD.WBP_GameHUD_C|GetAttackHorizontalBox (Variables|/Game/UI/HUD/WBP_GeneralUI.WBP_GeneralUI_C|GetWBP_GameHUD (Variables|/Game/Core/Player/BP_SpacePlayerController.BP_SpacePlayerController_C|GetGeneralUI (Variables|Default|GetSpaceController)))) false)
  (Variables|Default|SetAttack%20Type AttackType)
  (Variables|Default|SetDamageAmount (/ (* Damage (.damagemultiplier _battlestats)) (.resistance (Variables|Default|GetEnemyBattleStats))))
  (bind _aswbp_damage_text_2 (Utilities|Casting|CastToWBP_DamageText (UserInterface|GetWidget (Variables|Default|GetDamageText))))
  (if (< (Math|Random|RandomIntegerinRange 1 100) (.criticalchance _battlestats))
    (Variables|Default|SetDamageAmount (+ (Variables|Default|GetDamageAmount) 100 (Math|Random|RandomIntegerinRange 25 75)))
    (Class|CommonTextBlock|SetStyle (Variables|/Game/Core/Blueprints/FractionObjects/WBP_DamageText.WBP_DamageText_C|GetDamageText _aswbp_damage_text_2) "/Game/Core/Fonts/BP_TextStyleBigRed.BP_TextStyleBigRed_C")
    (else
      (Class|CommonTextBlock|SetStyle (Variables|/Game/Core/Blueprints/FractionObjects/WBP_DamageText.WBP_DamageText_C|GetDamageText _aswbp_damage_text_2) "/Game/Core/Fonts/BP_TextStyleBig.BP_TextStyleBig_C")))
  (Rendering|Components|TextRender|SetText (Variables|/Game/Core/Blueprints/FractionObjects/WBP_DamageText.WBP_DamageText_C|GetDamageText _aswbp_damage_text_2) (Utilities|Text|ToText(Integer) (- 0 (Variables|Default|GetDamageAmount))))
  (Transformation|SetRelativeLocation _damagetext (Math|Vector|MakeVector (.x _relativelocation) (.y _relativelocation) (Variables|Default|GetInitial%20Damage%20Text%20Z%20Position)) false false)
  (CallFunction|DamageTextHoverAnim (Variables|Default|GetDamageText))
  (bind _output_get (Variables|Default|SetHealth (- (Variables|Default|GetHealth) (Variables|Default|GetDamageAmount))))
  (Default|UpdateHealth (Variables|Default|GetAs%20WBP%20Health%20Bar) (Math|Conversions|ToFloat(Integer) _output_get))
  (if (<= _output_get 0)
    (Default|EndFight (Variables|/Game/Core/Player/BP_SpacePlayerController.BP_SpacePlayerController_C|GetSpaceShip (Variables|Default|GetSpaceController)))
    (else
      (Effects|Particles|Trails|BeginTrails _enemyhitparticle "None" "None" "ETrailWidthMode_FromCentre" 0.0)
      (Utilities|FlowControl|Delay 0.5)
      (Effects|Particles|Trails|EndTrails _enemyhitparticle)
      (Utilities|FlowControl|Delay 1.0)
      (Widget|SetIsEnabled (Variables|/Game/UI/HUD/WBP_GameHUD.WBP_GameHUD_C|GetAttackHorizontalBox (Variables|/Game/UI/HUD/WBP_GeneralUI.WBP_GeneralUI_C|GetWBP_GameHUD (Variables|/Game/Core/Player/BP_SpacePlayerController.BP_SpacePlayerController_C|GetGeneralUI (Variables|Default|GetSpaceController)))) true)
      (Variables|Default|SetAttack%20Type (.OutItem (Utilities|Array|Random (Utilities|Array|MakeArray "NewEnumerator1" "NewEnumerator0"))))
      (bind _output_get_2 (Variables|/Game/Core/Blueprints/BP_Ship.BP_Ship_C|SetHealth _spaceship (- (Variables|/Game/Core/Blueprints/BP_Ship.BP_Ship_C|GetHealth _spaceship) _returnvalue_4)))
      (Utilities|IsValid _as_wbp_health_bar
        (:Is%20Valid
          (Default|UpdateHealth _as_wbp_health_bar (Math|Conversions|ToFloat(Integer) _output_get_2))
          (bind _aswbp_damage_text_3 (Utilities|Casting|CastToWBP_DamageText (UserInterface|GetWidget _damagetext_2)))
          (Rendering|Components|TextRender|SetText (Variables|/Game/Core/Blueprints/FractionObjects/WBP_DamageText.WBP_DamageText_C|GetDamageText _aswbp_damage_text_3) (Utilities|Text|ToText(Integer) (- 0 _returnvalue_4)))
          (Transformation|SetRelativeLocation _damagetext_2 (Math|Vector|MakeVector (.x _relativelocation_2) (.y _relativelocation_2) (Variables|/Game/Core/Blueprints/BP_Ship.BP_Ship_C|GetInitial%20Damage%20Text%20Z%20Position _spaceship_2)) false false)
          (CallFunction|DamageTextHoverAnim _damagetext_2)
          (Effects|Particles|Trails|BeginTrails _selfhitparticle "None" "None" "ETrailWidthMode_FromCentre" 0.0)
          (Utilities|FlowControl|Delay 0.5)
          (Effects|Particles|Trails|EndTrails _selfhitparticle))))))

(event Custom|RotateBase
  (bind _spacecontroller (Variables|Default|GetSpaceController))
  (bind _staticmesh (Variables|Default|GetStaticMesh))
  (bind _relativerotation (Variables|/Script/Engine.SceneComponent|GetRelativeRotation _staticmesh))
  (if (not (Variables|/Game/Core/Player/BP_SpacePlayerController.BP_SpacePlayerController_C|GetIsTimeFrozen _spacecontroller))
    (Transformation|SetRelativeRotation _staticmesh (Math|Rotator|MakeRotator (+ (.roll _relativerotation) (* 1.0 (Variables|/Game/Core/Player/BP_SpacePlayerController.BP_SpacePlayerController_C|GettimeSpeed _spacecontroller))) (.pitch _relativerotation) (.yaw _relativerotation)) false false)))

(event Custom|DamageTextHoverAnim
  (params (DamageText :type Scene%20Component%20Object%20Reference))
  ;[1 1 1] TextHoverAnimation
  (Variables|Default|SetIsPlayerText (!= DamageText (Variables|Default|GetDamageText)))
  (Rendering|SetVisibility DamageText true false)
  (bind _returnvalue (Utilities|Time|SetTimerbyEvent (delegate Custom|LerpAnimation) 0.001 true)))

(event Custom|LerpAnimation
  (bind _initial_damage_text_z_position (Variables|Default|GetInitial%20Damage%20Text%20Z%20Position))
  (bind _isplayertext (Variables|Default|GetIsPlayerText))
  (bind _spacecontroller (Variables|Default|GetSpaceController))
  (bind _spaceship (Variables|/Game/Core/Player/BP_SpacePlayerController.BP_SpacePlayerController_C|GetSpaceShip _spacecontroller))
  (bind _initial_damage_text_z_position_2 (Variables|/Game/Core/Blueprints/BP_Ship.BP_Ship_C|GetInitial%20Damage%20Text%20Z%20Position _spaceship))
  (bind _returnvalue (select _isplayertext _initial_damage_text_z_position_2 _initial_damage_text_z_position))
  ;[1 1 1] TextHoverAnimation
  (bind _output_get (Variables|Default|SetAlphaOfAnimation (+ (Variables|Default|GetAlphaOfAnimation) 0.001)))
  (Transformation|SetRelativeLocation (stale Custom|DamageTextHoverAnim DamageText) (Math|Vector|MakeVector 0.0 0.0 (Math|Float|Lerp _returnvalue (+ _returnvalue 1e+02) (+ (Variables|Default|GetAlphaOfAnimation) 0.001))) false false)
  (if (> _output_get 1.0)
    (Variables|Default|SetAlphaOfAnimation 0.0)
    (Rendering|SetVisibility (stale Custom|DamageTextHoverAnim DamageText) false false)
    (Utilities|Time|ClearandInvalidateTimerbyHandle (stale Custom|DamageTextHoverAnim _returnvalue))))

(event Custom|SetRotation
  (bind _healthbar (Variables|Default|GetHealthBar))
  (Transformation|SetWorldRotation _healthbar (Math|Rotator|FindLookatRotation (Transformation|GetWorldLocation _healthbar) (Transformation|GetWorldLocation (Variables|/Game/Core/Player/BP_SpectatorPawn.BP_SpectatorPawn_C|GetCamera (Variables|/Game/Core/Player/BP_SpacePlayerController.BP_SpacePlayerController_C|GetBP_spectator (Variables|Default|GetSpaceController))))) false false))

(event EventTick
  (params (DeltaSeconds :type Float%20%28single-precision%29))
  (Transformation|SetRelativeRotation (Variables|Default|GetStaticMesh) (Math|Rotator|FindLookatRotation (Transformation|GetWorldLocation (Variables|Transformation|GetRootComponent)) (Transformation|GetActorLocation (Variables|/Game/Core/Player/BP_SpacePlayerController.BP_SpacePlayerController_C|GetSpaceShip (Variables|Default|GetSpaceController)))) false false))

(event EventBeginPlay
  (bind _health (Variables|Default|GetHealth))
  (Utilities|FlowControl|Delay 1.0)
  (Variables|Default|SetInitial%20Damage%20Text%20Z%20Position (.z (Variables|/Script/Engine.SceneComponent|GetRelativeLocation (Variables|Default|GetDamageText))))
  (bind _asbp_space_player_controller (Utilities|Casting|CastToBP_SpacePlayerController (Game|GetPlayerController 0)))
  (bind _output_get (Variables|Default|SetSpaceController _asbp_space_player_controller))
  (Rendering|SetVisibility (Variables|Default|GetDamageText) false false)
  (Transformation|AttachActorToActor (Variables|/Game/Core/Player/BP_SpectatorPawn.BP_SpectatorPawn_C|GetEnvironment (Variables|/Game/Core/Player/BP_SpacePlayerController.BP_SpacePlayerController_C|GetBP_spectator _output_get)) "None" "SnapToTarget" "KeepRelative" "KeepRelative" true)
  (Utilities|Time|SetTimerbyEvent (delegate Custom|SetRotation) 0.01 true)
  (Utilities|Time|SetTimerbyEvent (delegate Custom|RotateBase) 0.01 true)
  (bind _aswbp_health_bar (Utilities|Casting|CastToWBP_HealthBar (UserInterface|GetWidget (Variables|Default|GetHealthBar))))
  (bind _output_get_2 (Variables|Default|SetAs%20WBP%20Health%20Bar _aswbp_health_bar))
  (Default|SetInitialHealth _output_get_2 (Math|Conversions|ToFloat(Integer) _health))
  (Default|UpdateHealth _output_get_2 (Math|Conversions|ToFloat(Integer) _health))
  (bind _outrownames (DataTable|GetDataTableRowNames "/Game/Core/DataTables/DT_FractionsList.DT_FractionsList"))
  (bind _array_element (Utilities|Array|ForEachLoopwithBreak _outrownames :!label _label)
    (:LoopBody
      (bind _returnvalue (Utilities|GetDataTableRow "/Game/Core/DataTables/DT_FractionsList.DT_FractionsList" _array_element)
        (:then
          (if (Utilities|Enum|Equal(Enum) (.fraction _returnvalue) (Variables|Default|GetFraction))
            (Variables|/Game/Core/Blueprints/FractionObjects/WBP_HealthBar.WBP_HealthBar_C|SetBarColor (Variables|Default|GetAs%20WBP%20Health%20Bar) (Math|Conversions|ToLinearColor(Color) (.color _returnvalue)))
            (goto _label Break)))))))

(fn ConstructionScript)