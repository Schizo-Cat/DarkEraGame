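; Base-surroundings actor that handles slot-based building and ties the game's lighting to the black hole's remaining mass.
; Tick turns slot widgets toward the camera and traces under the cursor to highlight slots, menu entries and buildings for ClickSelected.
; Clicks open build menus or research; BuildBuilding spends black hole mass, replaces the slot and completes tasks.
; A looping timer scales lights and MPC "deathofuniverse" by mass ratio, while SetGameColor tints lights and UI.
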(event Custom|TurnVisibility
  (params (IsVisible :type Boolean)))

(event Custom|SetGameColor
  (params (Color :type Linear%20Color%20Structure))
  (Utilities|IsValid (Variables|/Game/Core/Player/BP_SpacePlayerController.BP_SpacePlayerController_C|GetBlackHole (Variables|Default|GetBP%20Space%20Player%20Controller))
    (:Is%20Valid
      (bind _output_get (Variables|Default|SetColor Color))
      (Rendering|Material|SetVectorParameterValue "/Game/Materials/MPC_Collection.MPC_Collection" "color" _output_get :!class /Script/Engine.KismetMaterialLibrary)
      (Rendering|Components|Light|SetLightColor (Variables|Default|GetPointLight) _output_get true)
      (Default|SetUIColor (Variables|/Game/UI/HUD/WBP_GeneralUI.WBP_GeneralUI_C|GetWBP_GameHUD (Variables|/Game/Core/Player/BP_SpacePlayerController.BP_SpacePlayerController_C|GetGeneralUI (Variables|Default|GetBP%20Space%20Player%20Controller))))
      (Default|CallSetGlobalColor)
      (for _array_element (Variables|Default|GetSlotsArray)
        (bind _aswbp_build_button (Utilities|Casting|CastToWBP_BuildButton (UserInterface|GetWidget _array_element)))
        (Appearance|SetColorandOpacity (Variables|/Game/Core/Buildings/WBP_BuildButton.WBP_BuildButton_C|GetImage_84 _aswbp_build_button) (Utilities|Struct|MakeLinearColor (.r (Variables|Default|GetColor)) (.g (Variables|Default|GetColor)) (.b (Variables|Default|GetColor)) 0.5) :!class /Script/UMG.Image)))))

(event Custom|SetSpaceIntensity
  (bind _bp_space_player_controller (Variables|Default|GetBP%20Space%20Player%20Controller))
  (bind _blackhole (Variables|/Game/Core/Player/BP_SpacePlayerController.BP_SpacePlayerController_C|GetBlackHole _bp_space_player_controller))
  (bind _currentmass (Variables|/Game/Core/Blueprints/BP_MainBlackHole.BP_MainBlackHole_C|GetCurrentMass _blackhole))
  (bind _initialmass (Variables|/Game/Core/Blueprints/BP_MainBlackHole.BP_MainBlackHole_C|GetInitialMass _blackhole))
  (bind _returnvalue (/ _currentmass _initialmass))
  (bind _returnvalue_2 (- _returnvalue 0.2))
  (Default|CallSetGlobalLight)
  (Utilities|IsValid _blackhole
    (:Is%20Valid
      (Rendering|Components|Light|SetIntensity (Variables|Default|GetPointLight) _returnvalue)
      (if (<= _returnvalue_2 0.0)
        (Rendering|Material|SetScalarParameterValue "/Game/Materials/MPC_Collection.MPC_Collection" "deathofuniverse" 0.0 :!class /Script/Engine.KismetMaterialLibrary)
        (else
          (Rendering|Material|SetScalarParameterValue "/Game/Materials/MPC_Collection.MPC_Collection" "deathofuniverse" _returnvalue_2 :!class /Script/Engine.KismetMaterialLibrary))))))

(event Custom|ClickSelected
  (bind _thisactor (Variables|Default|GetThisActor))
  (bind _thisactor_2 (Variables|Default|GetThisActor))
  (bind _thisactor_3 (Variables|Default|GetThisActor))
  (bind _componenttags (Variables|/Script/Engine.ActorComponent|GetComponentTags _thisactor))
  ;[1 1 1] ClickSelected
  (Utilities|IsValid _thisactor
    (:Is%20Valid
      (switch name (Utilities|Array|Get(acopy) _componenttags)
        (:Slot
          (if (Variables|Default|GetSlotsAvailable)
            (if (Utilities|Array|IsNotEmpty (Variables|/Game/Core/Player/BP_SpacePlayerController.BP_SpacePlayerController_C|GetAvailableBuildings (Variables|Default|GetBP%20Space%20Player%20Controller)))
              (Utilities|IsValid (Variables|Default|GetSelectedOpenMenu)
                (:Is%20Valid
                  (for _array_element (Variables|Default|GetSlotsArray)
                    (Rendering|SetVisibility _array_element true false)
                    (Collision|SetCollisionEnabled _array_element "QueryAndPhysics"))
                  (Actor|DestroyActor (Variables|Default|GetSelectedOpenMenu)))
                (:Is%20Not%20Valid
                  _))
              (Utilities|IsValid _thisactor_2
                (:Is%20Valid
                  (Variables|Default|SetClickedSlot _thisactor_2)
                  (Collision|SetCollisionEnabled _thisactor_3 "NoCollision")
                  (Rendering|SetVisibility _thisactor_3 false false)
                  (Transformation|SetWorldScale3D _thisactor_3 (Variables|Default|GetDefaultSlotScale))
                  (bind _returnvalue (Game|SpawnActorfromClass "/Game/Core/Buildings/BuildingClickable.BuildingClickable_C" (Transformation|GetWorldTransform _thisactor_3) "Undefined" "MultiplyWithRoot" 0 0))
                  (bind _output_get (Variables|Default|SetSelectedOpenMenu _returnvalue))
                  (Transformation|AttachComponentToComponent _returnvalue _thisactor_3 "None" "KeepWorld" "KeepWorld" "KeepRelative" true))))))
        (:BaseMenu
          (if (Variables|Default|GetSlotsAvailable)
            (bind _aswidget_component (Utilities|Casting|CastToWidgetComponent (Variables|Default|GetThisActor)))
            (bind _aswbp_build_slot (Utilities|Casting|CastToWBP_BuildSlot (UserInterface|GetWidget _aswidget_component)))
            (CallFunction|BuildBuilding (Variables|/Game/Core/Buildings/WBP_BuildSlot.WBP_BuildSlot_C|GetBuildStructure _aswbp_build_slot))
            (if (not (Utilities|Array|IsNotEmpty (Variables|/Game/Core/Player/BP_SpacePlayerController.BP_SpacePlayerController_C|GetAvailableBuildings (Variables|Default|GetBP%20Space%20Player%20Controller))))
              (Rendering|SetVisibility (Variables|Default|GetButtons) false true))))
        (:BuildingBase
          ;[1 1 1] PickBuilding
          (Default|HighlightBuilding (Variables|Default|GetSelectedBuilding) false)
          (switch name (Utilities|Array|Get(acopy) _componenttags 1)
            (:ResearchBase
              (Default|ToggleResearchMenu (Variables|Default|GetBP%20Space%20Player%20Controller)))))))))

(event Custom|TurnCollision
  (params (Enabled :type Boolean))
  ;[1 1 1] TurnCollision
  (for _array_element (Variables|Default|GetSlotsArray)
    (if Enabled
      (Collision|SetCollisionEnabled _array_element "QueryAndPhysics")
      (else
        (Collision|SetCollisionEnabled _array_element "NoCollision")))))

(event EventBeginPlay
  (bind _asbp_space_player_controller (Utilities|Casting|CastToBP_SpacePlayerController (Game|GetPlayerController 0)))
  (Variables|Default|SetBP%20Space%20Player%20Controller _asbp_space_player_controller)
  (Variables|Default|SetSlotsArray (Utilities|Array|MakeArray (Variables|Default|GetWidget6) (Variables|Default|GetWidget5) (Variables|Default|GetWidget4) (Variables|Default|GetWidget3) (Variables|Default|GetWidget2) (Variables|Default|GetWidget1) (Variables|Default|GetWidget7) (Variables|Default|GetWidget)))
  (Utilities|FlowControl|Delay 0.1)
  (CallFunction|SetGameColor (Variables|Default|GetColor))
  (bind _returnvalue (Utilities|Time|SetTimerbyEvent (delegate Custom|SetSpaceIntensity) 3.0 true))
  (Variables|Default|SetGameIntensityChangeTimer _returnvalue)
  (Utilities|Time|SetTimerbyEvent 0 0.1 true)
  (bind _returnvalue_2 (Utilities|GetDataTableRow "/Game/Core/DataTables/DT_Buildings.DT_Buildings" "ResearchBase")
    (:then
      (Utilities|Array|Add (Variables|/Game/Core/Player/BP_SpacePlayerController.BP_SpacePlayerController_C|GetAvailableBuildings (Variables|Default|GetBP%20Space%20Player%20Controller)) _returnvalue_2))))

(event EventTick
  (params (DeltaSeconds :type Float%20%28single-precision%29))
  (bind _bp_space_player_controller (Variables|Default|GetBP%20Space%20Player%20Controller))
  (bind _hitresult (Game|Player|GetHitResultUnderCursorbyChannel _bp_space_player_controller "TraceTypeQuery1" false))
  (bind (_bblockinghit _binitialoverlap _time _distance _location _impactpoint _normal _impactnormal _physmat _hitactor _hitcomponent) (Collision|BreakHitResult _hitresult))
  ;[1 1 1] PickBuilding
  (for _array_element (Variables|Default|GetSlotsArray)
    (Utilities|LookatCamera _array_element)
    (if (== (Class|WidgetSwitcher|GetActiveWidgetIndex (Variables|/Game/UI/HUD/WBP_GeneralUI.WBP_GeneralUI_C|GetWidgetSwitcher (Variables|/Game/Core/Player/BP_SpacePlayerController.BP_SpacePlayerController_C|GetGeneralUI _bp_space_player_controller))) 0)
      (if _bblockinghit
        (Variables|Default|SetLastActor (Variables|Default|GetThisActor))
        (Variables|Default|SetThisActor _hitcomponent)
        (Utilities|IsValid (Variables|Default|GetLastActor)
          (:Is%20Valid
            (Utilities|IsValid (Variables|Default|GetThisActor)
              (:Is%20Valid
                (if (!= (Variables|Default|GetLastActor) (Variables|Default|GetThisActor))
                  (switch name (Utilities|Array|Get(acopy) (Variables|/Script/Engine.ActorComponent|GetComponentTags (Variables|Default|GetLastActor))) :!label _label
                    (:Slot
                      (Transformation|SetWorldScale3D (Variables|Default|GetLastActor) (Variables|Default|GetDefaultSlotScale)))
                    (:BaseMenu
                      (Transformation|SetRelativeScale3D (Variables|Default|GetLastActor) "1.000000,1.000000,1.000000"))
                    (:BuildingBase
                      (bind _asbp_building_base (Utilities|Casting|CastToBP_BuildingBase (Variables|Default|GetSavedBuildingActor)))
                      (Default|HighlightBuilding _asbp_building_base false)
                      (Variables|Default|SetSelectedBuilding 0)))
                  (else
                    (Audio|PlaySound2D "/Game/Core/Audio/SFX/ResearchHover.ResearchHover" 0.0 1.0 0.0 0 0 :!label _label_2)
                    (switch name (Utilities|Array|Get(acopy) (Variables|/Script/Engine.ActorComponent|GetComponentTags (Variables|Default|GetThisActor)))
                      (:Slot
                        (Transformation|SetWorldScale3D (Variables|Default|GetThisActor) (Variables|Default|GetSelectedScale)))
                      (:BaseMenu
                        (Transformation|SetRelativeScale3D (Variables|Default|GetThisActor) "1.200000,1.200000,1.200000"))
                      (:BuildingBase
                        (bind _output_get (Variables|Default|SetSavedBuildingActor _hitactor))
                        (bind _asbp_building_base_2 (Utilities|Casting|CastToBP_BuildingBase _output_get))
                        (bind _output_get_2 (Variables|Default|SetSelectedBuilding _asbp_building_base_2))
                        (Default|HighlightBuilding _output_get_2 true))))))
              (:Is%20Not%20Valid
                (goto _label))))
          (:Is%20Not%20Valid
            (Utilities|IsValid (Variables|Default|GetThisActor)
              (:Is%20Valid
                (goto _label_2)))))))))

(fn ConstructionScript)

(fn BuildBuilding
  (params (Item :type Build%20Information%20Structure%20%28by%20ref%29))
  (bind (_buildingname _cost _tag _image _buildclass) (Utilities|Struct|BreakBuildInformation Item))
  (bind _bp_space_player_controller (Variables|Default|GetBP%20Space%20Player%20Controller))
  (bind _bp_space_player_controller_2 (Variables|Default|GetBP%20Space%20Player%20Controller))
  (bind _bp_space_player_controller_3 (Variables|Default|GetBP%20Space%20Player%20Controller))
  (bind _clickedslot (Variables|Default|GetClickedSlot))
  (bind _tasksystem (Variables|/Game/Core/Player/BP_SpacePlayerController.BP_SpacePlayerController_C|GetTaskSystem _bp_space_player_controller))
  (bind _availablebuildings (Variables|/Game/Core/Player/BP_SpacePlayerController.BP_SpacePlayerController_C|GetAvailableBuildings _bp_space_player_controller_3))
  (bind _blackhole (Variables|/Game/Core/Player/BP_SpacePlayerController.BP_SpacePlayerController_C|GetBlackHole _bp_space_player_controller_2))
  (if (> (- (Variables|/Game/Core/Blueprints/BP_MainBlackHole.BP_MainBlackHole_C|GetCurrentMass _blackhole) _cost) 1e+02)
    (Variables|/Game/Core/Blueprints/BP_MainBlackHole.BP_MainBlackHole_C|SetCurrentMass _blackhole (- (Variables|/Game/Core/Blueprints/BP_MainBlackHole.BP_MainBlackHole_C|GetCurrentMass _blackhole) _cost))
    (Utilities|FlowControl|Sequence
      (:then_0
        (bind _returnvalue (Game|SpawnActorfromClass _buildclass (Math|Transform|MakeTransform (.location (Transformation|GetActorTransform (Variables|Default|GetSelectedOpenMenu))) "0, 0, 0" "1.000000,1.000000,1.000000") "AlwaysSpawn" "MultiplyWithRoot" 0 0))
        (Variables|Default|SetSpawnedBuilding _returnvalue)
        (Utilities|IsValid (Variables|Default|GetSpawnedBuilding)
          (:Is%20Valid
            (Utilities|Array|Add (Variables|Default|GetCurrentBuildings) (Variables|Default|GetSpawnedBuilding))
            (Utilities|Array|RemoveItem _availablebuildings Item)
            (Actor|DestroyActor (Variables|Default|GetSelectedOpenMenu))
            (bind _aswidget_component (Utilities|Casting|CastToWidgetComponent _clickedslot))
            (Utilities|Array|RemoveItem (Variables|Default|GetSlotsArray) _aswidget_component)
            (Components|DestroyComponent _clickedslot)
            (Transformation|AttachComponentToComponent (Variables|Default|GetSpawnedBuilding) (Variables|Default|GetScene) "None" "KeepWorld" "SnapToTarget" "KeepWorld" false)
            (switch name (Utilities|Array|Get(acopy) (Variables|/Script/Engine.Actor|GetTags (Variables|Default|GetSpawnedBuilding)) 1)
              (:ResearchBase
                (bind _returnvalue_2 (Utilities|GetDataTableRow "/Game/Core/DataTables/TaskList.TaskList" "B_ResearchBase")
                  (:then
                    (Default|CompleteTask _tasksystem _returnvalue_2))))
              (:Colony
                (bind _returnvalue_3 (Utilities|GetDataTableRow "/Game/Core/DataTables/TaskList.TaskList" "B_Colony")
                  (:then
                    (Default|CompleteTask _tasksystem _returnvalue_3))))))))
      (:then_1
        (if (Utilities|Array|IsEmpty _availablebuildings)
          (Variables|Default|SetSlotsAvailable false)
          (CallFunction|TurnVisibility false)
          (Variables|Default|SetSelectedObject 0)
          (Utilities|IsValid (Variables|Default|GetSelectedOpenMenu)
            (:Is%20Valid
              (Actor|DestroyActor (Variables|Default|GetSelectedOpenMenu))
              (Variables|Default|SetSelectedOpenMenu 0))))))))