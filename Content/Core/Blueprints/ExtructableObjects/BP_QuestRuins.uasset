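; BP_QuestRuins is an extractable quest ruins object that plays story beats as it is approached and extracted.
; BeginPlay rolls a random mass and sets its lore entry.
; Getting closer hides the general UI, then async-loads and plays the relic-found Level Sequence cinematic.
; Extraction starts a Research faction dialogue through the SpaceController's dialogue system, using rows from the dialogue and faction data tables.
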(event EventBeginPlay
  (|CallParentFunction)
  (Variables|Default|SetMass (Math|Random|RandomFloatinRange 5.0 1e+01))
  (Variables|Default|SetEntry (Variables|Default|GetLoreEntrt)))

(event EventOnGotCloser
  (|CallParentFunction)
  (Widget|SetVisibility (Variables|/Game/Core/Player/BP_SpacePlayerController.BP_SpacePlayerController_C|GetGeneralUI (Variables|Default|GetSpaceController)) "Hidden")
  (bind _object (Utilities|AsyncLoadAsset "/Game/Cinematic/RelicFounsCinematic.RelicFounsCinematic")
    (:Completed
      (bind _aslevel_sequence (Utilities|Casting|CastToLevelSequence _object))
      (bind (_outactor _returnvalue) (Sequencer|Player|CreateLevelSequencePlayer _aslevel_sequence))
      (Sequencer|Player|Play (Variables|/Script/LevelSequence.LevelSequenceActor|GetSequencePlayer _outactor) :!class /Script/MovieScene.MovieSceneSequencePlayer))))

(fn ConstructionScript
  (|CallParentFunction))

(fn OnExtracted
  (|CallParentFunction)
  (bind _returnvalue (Utilities|GetDataTableRow "/Game/Core/DataTables/DT_Dialogues.DT_Dialogues" "SF_1Rel_Extracted")
    (:then
      (bind _returnvalue_2 (Utilities|GetDataTableRow "/Game/Core/DataTables/DT_FractionsList.DT_FractionsList" "ResearchFraction")
        (:then
          (Default|InitiateDialogue (Variables|/Game/Core/Player/BP_SpacePlayerController.BP_SpacePlayerController_C|GetDialogueSystem (Variables|Default|GetSpaceController)) _returnvalue _returnvalue_2))))))