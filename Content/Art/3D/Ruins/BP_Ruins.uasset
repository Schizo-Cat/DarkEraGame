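; BP_Ruins is a ruins prop whose sphere-type mesh pieces spin continuously in two counter-rotating pairs.
; On BeginPlay it caches the BP_SpacePlayerController and starts a fast looping timer that drives the rotation.
; Each tick yaws one pair forward and the other backward, scaled by the controller's TimeSpeed, with each pair following the yaw of one lead piece.
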(event Custom|RotateBase
  (bind _sfera_tipo_ruins_cube_001 (Variables|Default|Getsfera_tipo_ruins_Cube_001))
  (bind _sfera_tipo_ruins_cube_002 (Variables|Default|Getsfera_tipo_ruins_Cube_002))
  (Transformation|SetRelativeRotation _sfera_tipo_ruins_cube_002 (Math|Rotator|MakeRotator 0.0 0.0 (+ (.yaw (Variables|/Script/Engine.SceneComponent|GetRelativeRotation _sfera_tipo_ruins_cube_002)) (* 0.01 (Variables|/Script/DarkEraProject.SpacePlayerController|GettimeSpeed (stale EventBeginPlay _output_get))))) false false)
  (Transformation|SetRelativeRotation _sfera_tipo_ruins_cube_001 (Math|Rotator|MakeRotator 0.0 0.0 (- (.yaw (Variables|/Script/Engine.SceneComponent|GetRelativeRotation _sfera_tipo_ruins_cube_001)) (* 0.01 (Variables|/Script/DarkEraProject.SpacePlayerController|GettimeSpeed (stale EventBeginPlay _output_get))))) false false))

(event EventBeginPlay
  (bind _asbp_space_player_controller (Utilities|Casting|CastToBP_SpacePlayerController (Game|GetPlayerController 0)))
  (bind _output_get (Variables|Default|SetSpaceController _asbp_space_player_controller))
  (Utilities|Time|SetTimerbyEvent (delegate Custom|RotateBase) 0.01 true))

(fn ConstructionScript)