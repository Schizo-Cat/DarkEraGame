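; BP_SpaceBodyBase is a base space body actor that slowly drifts toward the player's spaceship.
; BeginPlay caches the BP_SpacePlayerController of player 0 to reach its SpaceShip.
; Each Tick lerps the body's location toward the ship by a small delta-time-scaled alpha, without sweeping.
; The move applies only while the new position stays at least a minimum distance from the ship.
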(event EventTick
  (params (DeltaSeconds :type Float%20%28single-precision%29))
  (bind _returnvalue (Transformation|GetActorLocation))
  (bind _returnvalue_2 (/ DeltaSeconds 1e+01))
  (bind _spacecontroller (Variables|Default|GetSpaceController))
  (bind _spaceship (Variables|/Game/BP_SpacePlayerController.BP_SpacePlayerController_C|GetSpaceShip _spacecontroller))
  (bind _returnvalue_3 (Transformation|GetActorLocation _spaceship))
  (bind _returnvalue_4 (Math|Vector|Lerp(Vector) _returnvalue _returnvalue_3 _returnvalue_2))
  (Utilities|IsValid _spaceship
    (:Is%20Valid
      (if (>= (Math|Vector|Distance(Vector) _returnvalue_4 _returnvalue_3) 3e+02)
        (Transformation|SetActorLocation _returnvalue_4 false false)))))

(event EventBeginPlay
  (bind _asbp_space_player_controller (Utilities|Casting|CastToBP_SpacePlayerController (Game|GetPlayerController 0)))
  (Variables|Default|SetSpaceController _asbp_space_player_controller))

(fn ConstructionScript)