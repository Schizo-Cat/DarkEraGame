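; Neutron star actor among the extractable space objects, with a randomized mass and its own neutron Entry assigned at BeginPlay.
; A fast looping timer spins the Scene component on roll, scaling each step by the space player controller's TimeSpeed.
; The construction script applies the configurable star material to the sphere and the light color to the point light.
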(event Custom|RotateBase
  (bind _scene (Variables|Default|GetScene))
  (Transformation|SetRelativeRotation _scene (Math|Rotator|MakeRotator (+ (.roll (Variables|/Script/Engine.SceneComponent|GetRelativeRotation _scene)) (* 5.0 (Variables|/Script/DarkEraProject.SpacePlayerController|GettimeSpeed (stale EventBeginPlay _output_get)))) 0.0 0.0) false false))

(event EventBeginPlay
  (|CallParentFunction)
  (Variables|Default|SetMass (Math|Random|RandomFloatinRange 2e+01 5e+01))
  (Variables|Default|SetEntry (Variables|Default|GetNeutronEntry))
  (bind _asbp_space_player_controller (Utilities|Casting|CastToBP_SpacePlayerController (Game|GetPlayerController 0)))
  (bind _output_get (Variables|Default|SetSpaceController _asbp_space_player_controller))
  (Utilities|Time|SetTimerbyEvent (delegate Custom|RotateBase) 0.01 true))

(fn ConstructionScript
  (|CallParentFunction)
  (Rendering|Material|SetMaterial (Variables|Default|GetSphere) 0 (Variables|Default|GetMaterialOfStar))
  (Rendering|Components|Light|SetLightColor (Variables|Default|GetPointLight) (Variables|Default|GetLightColor) true))