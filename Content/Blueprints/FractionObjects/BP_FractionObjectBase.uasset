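; Base actor for attackable faction objects in the space game, with health and an overhead health bar widget.
; On BeginPlay it turns its mesh toward the player's ship once and colors the bar from its faction's row in DT_FractionsList.
; A fast looping timer keeps the bar facing the spectator camera.
; Attack reduces health and updates the bar, then ends the ship's fight and destroys the actor at zero.
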(event Custom|Attack
  (params (Damage :type Integer))
  (bind _output_get (Variables|Default|SetHealth (- (Variables|Default|GetHealth) Damage)))
  (Default|UpdateHealth (Variables|Default|GetAs%20WBP%20Health%20Bar) (Math|Conversions|ToFloat(Integer) _output_get))
  (if (<= _output_get 0)
    (Default|EndFight (Variables|/Game/BP_SpacePlayerController.BP_SpacePlayerController_C|GetSpaceShip (Variables|Default|GetSpaceController)))
    (Actor|DestroyActor)))

(event Custom|SetRotation
  (bind _healthbar (Variables|Default|GetHealthBar))
  (Transformation|SetWorldRotation _healthbar (Math|Rotator|FindLookatRotation (Transformation|GetWorldLocation _healthbar) (Transformation|GetWorldLocation (Variables|/Game/BP_SpectatorPawn.BP_SpectatorPawn_C|GetCamera (Variables|/Game/BP_SpacePlayerController.BP_SpacePlayerController_C|GetBP_spectator (Variables|Default|GetSpaceController))))) false false))

(event EventBeginPlay
  (bind _staticmesh (Variables|Default|GetStaticMesh))
  (bind _health (Variables|Default|GetHealth))
  (bind _asbp_space_player_controller (Utilities|Casting|CastToBP_SpacePlayerController (Game|GetPlayerController 0)))
  (bind _output_get (Variables|Default|SetSpaceController _asbp_space_player_controller))
  (Transformation|SetRelativeRotation _staticmesh (Math|Rotator|FindLookatRotation (Transformation|GetWorldLocation _staticmesh) (Transformation|GetActorLocation (Variables|/Game/BP_SpacePlayerController.BP_SpacePlayerController_C|GetSpaceShip _output_get))) false false)
  (Utilities|Time|SetTimerbyEvent (delegate Custom|SetRotation) 0.01 true)
  (bind _aswbp_health_bar (Utilities|Casting|CastToWBP_HealthBar (UserInterface|GetWidget (Variables|Default|GetHealthBar))))
  (bind _output_get_2 (Variables|Default|SetAs%20WBP%20Health%20Bar _aswbp_health_bar))
  (Default|SetInitialHealth _output_get_2 (Math|Conversions|ToFloat(Integer) _health))
  (Default|UpdateHealth _output_get_2 (Math|Conversions|ToFloat(Integer) _health))
  (bind _outrownames (DataTable|GetDataTableRowNames "/Game/UI/FractionsMenu/DT_FractionsList.DT_FractionsList"))
  (bind _array_element (Utilities|Array|ForEachLoopwithBreak _outrownames :!label _label)
    (:LoopBody
      (bind _returnvalue (Utilities|GetDataTableRow "/Game/UI/FractionsMenu/DT_FractionsList.DT_FractionsList" _array_element)
        (:then
          (if (Utilities|Enum|Equal(Enum) (.fraction _returnvalue) (Variables|Default|GetFraction))
            (Variables|/Game/Blueprints/FractionObjects/WBP_HealthBar.WBP_HealthBar_C|SetBarColor (Variables|Default|GetAs%20WBP%20Health%20Bar) (Math|Conversions|ToLinearColor(Color) (.color _returnvalue)))
            (goto _label Break)))))))

(fn ConstructionScript)