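; BP_SpaceBodyBase is a base space body that slides toward the player's ship to play out space travel.
; Each Tick, unless time is frozen, it lerps toward the ship by delta time and TimeSpeed, writing its negated position to the MPC spaceOffset parameter.
; Within 300 units it stops and, once only, shuts off the ship's thruster effect, resets its rotation, clears Istravelling and sets the black hole's MassLossRate.
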(event EventTick
  (params (DeltaSeconds :type Float%20%28single-precision%29))
  (bind _returnvalue (Transformation|GetActorLocation))
  (bind _returnvalue_2 (/ DeltaSeconds 1e+01))
  (bind _spacecontroller (Variables|Default|GetSpaceController))
  (bind _spacecontroller_2 (Variables|Default|GetSpaceController))
  (bind _timespeed (Variables|/Script/DarkEraProject.SpacePlayerController|GettimeSpeed _spacecontroller_2))
  (bind _spaceship (Variables|/Game/BP_SpacePlayerController.BP_SpacePlayerController_C|GetSpaceShip _spacecontroller_2))
  (bind _spaceship_2 (Variables|/Game/BP_SpacePlayerController.BP_SpacePlayerController_C|GetSpaceShip _spacecontroller))
  (bind _returnvalue_3 (Transformation|GetActorLocation _spaceship))
  (bind _returnvalue_4 (* _returnvalue_2 _timespeed))
  (bind _returnvalue_5 (Math|Vector|Lerp(Vector) _returnvalue _returnvalue_3 _returnvalue_4))
  (if (not (Variables|/Script/DarkEraProject.SpacePlayerController|GetIsTimeFrozen _spacecontroller_2))
    (Utilities|IsValid _spaceship
      (:Is%20Valid
        (if (>= (Math|Vector|Distance(Vector) _returnvalue_5 _returnvalue_3) 3e+02)
          (Transformation|SetActorLocation _returnvalue_5 false false)
          (Rendering|Material|SetVectorParameterValue "/Game/Materials/MPC_Collection.MPC_Collection" "spaceOffset" (Math|Conversions|ToLinearColor(Vector) (- "" _returnvalue_5)) :!class /Script/Engine.KismetMaterialLibrary)
          (else
            (Utilities|FlowControl|DoOnce false
              (:Completed
                (Components|Activation|Deactivate (Variables|/Game/Blueprints/BP_Ship.BP_Ship_C|GetP_Flamethrower _spaceship_2))
                (Transformation|SetActorRotation _spaceship_2 "90.000000,0.000000,0.000000")
                (Variables|/Game/BP_SpacePlayerController.BP_SpacePlayerController_C|SetIstravelling _spacecontroller false)
                (Variables|/Script/DarkEraProject.BlackHole|SetMassLossRate (Variables|/Game/BP_SpacePlayerController.BP_SpacePlayerController_C|GetBlackHole _spacecontroller) 1.0)))))))))

(event EventBeginPlay
  (bind _asbp_space_player_controller (Utilities|Casting|CastToBP_SpacePlayerController (Game|GetPlayerController 0)))
  (Variables|Default|SetSpaceController _asbp_space_player_controller))

(fn ConstructionScript)