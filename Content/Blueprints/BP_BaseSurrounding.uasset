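; Surrounding environment of the base, providing camera-facing widget slots where buildings are placed, plus the space scene's lighting.
; A looping timer traces under the cursor to highlight slots, menu options and buildings by component tag.
; ClickSelected opens build menus, spawns research or meteor bases paid with black hole mass, or toggles the research menu.
; A slower timer scales lights and a material parameter collection by remaining mass, while SetGameColor tints lights and UI.
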(event Custom|TurnVisibility
  (params (IsVisible :type Boolean))
  (bind _selectedopenmenu (Variables|Default|GetSelectedOpenMenu))
  (if (Variables|Default|GetSlotsAvailable)
    (for _array_element (Variables|Default|GetSlotsArray)
      (Rendering|SetVisibility _array_element IsVisible false)
      (for _array_element_2 (Variables|Default|GetCurrentBuildings)
        (Utilities|IsValid _array_element_2
          (:Is%20Valid
            (Default|HighlightBuilding _array_element_2 false)
            (Utilities|IsValid _selectedopenmenu
              (:Is%20Valid
                (Actor|DestroyActor _selectedopenmenu)))))))))

(event Custom|SetGameColor
  (params (Color :type Linear%20Color%20Structure))
  (Utilities|IsValid (Variables|/Game/BP_SpacePlayerController.BP_SpacePlayerController_C|GetBlackHole (Variables|Default|GetBP%20Space%20Player%20Controller))
    (:Is%20Valid
      (bind _output_get (Variables|Default|SetColor Color))
      (Rendering|Material|SetVectorParameterValue "/Game/Materials/MPC_Collection.MPC_Collection" "color" _output_get :!class /Script/Engine.KismetMaterialLibrary)
      (Rendering|Components|Light|SetLightColor (Variables|Default|GetPointLight) _output_get true)
      (Default|SetUIColor (Variables|/Game/UI/HUD/WBP_GeneralUI.WBP_GeneralUI_C|GetWBP_GameHUD (Variables|/Game/BP_SpacePlayerController.BP_SpacePlayerController_C|GetGeneralUI (Variables|Default|GetBP%20Space%20Player%20Controller))))
      (Default|CallSetGlobalColor)
      (for _array_element (Variables|Default|GetSlotsArray)
        (bind _aswbp_build_button (Utilities|Casting|CastToWBP_BuildButton (UserInterface|GetWidget _array_element)))
        (Appearance|SetColorandOpacity (Variables|/Game/UI/Buildings/WBP_BuildButton.WBP_BuildButton_C|GetImage_84 _aswbp_build_button) (Utilities|Struct|MakeLinearColor (.r (Variables|Default|GetColor)) (.g (Variables|Default|GetColor)) (.b (Variables|Default|GetColor)) 0.5) :!class /Script/UMG.Image)))))

(event Custom|SetSpaceIntensity
  (bind _bp_space_player_controller (Variables|Default|GetBP%20Space%20Player%20Controller))
  (bind _blackhole (Variables|/Game/BP_SpacePlayerController.BP_SpacePlayerController_C|GetBlackHole _bp_space_player_controller))
  (bind _currentmass (Variables|/Script/DarkEraProject.BlackHole|GetCurrentMass _blackhole))
  (bind _initialmass (Variables|/Script/DarkEraProject.BlackHole|GetInitialMass _blackhole))
  (bind _returnvalue (/ _currentmass _initialmass))
  (bind _returnvalue_2 (- _returnvalue 0.2))
  (Default|CallSetGlobalLight)
  (Utilities|IsValid _blackhole
    (:Is%20Valid
      (Rendering|Components|Light|SetIntensity (Variables|Default|GetPointLight) _returnvalue)
      (if (<= _returnvalue_2 0.0)
        (Rendering|Material|SetScalarParameterValue "/Game/Materials/MPC_Collection.MPC_Collection" "deathofuniverse" 0.0 :!class /Script/Engine.KismetMaterialLibrary)
        (else
          (Rendering|Material|SetScalarParameterValue "/Game/Materials/MPC_Collection.MPC_Collection" "deathofuniverse" _returnvalue_2 :!class /Script/Engine.KismetMaterialLibrary))))))

(event Custom|SelectObject
  (bind _returnvalue (Game|GetPlayerController 0))
  (bind _hitresult (Game|Player|GetHitResultUnderCursorbyChannel _returnvalue "TraceTypeQuery1" false))
  (bind (_bblockinghit _binitialoverlap _time _distance _location _impactpoint _normal _impactnormal _physmat _hitactor _hitcomponent) (Collision|BreakHitResult _hitresult))
  ;[1 1 1] ClickSelect
  (if (Variables|/Game/BP_SpacePlayerController.BP_SpacePlayerController_C|GetCanClick (Variables|Default|GetBP%20Space%20Player%20Controller))
    (Utilities|IsValid _hitcomponent
      (:Is%20Valid
        (switch name (Utilities|Array|Get(acopy) (Variables|/Script/Engine.ActorComponent|GetComponentTags _hitcomponent))
          (:Slot
            (bind _output_get (Variables|Default|SetSelectedObject _hitcomponent))
            (Utilities|DeselectAllSlots
              (:Completed
                (Utilities|FlowControl|Sequence
                  (:then_0
                    (Utilities|FlowControl|DoOnce false :!label _label
                      (:Completed
                        (Audio|PlaySound2D "/Game/Sounds/SFX/ResearchHover.ResearchHover" 1.0 1.0 0.0 0 0))))
                  (:then_1
                    (Transformation|SetWorldScale3D _output_get (Variables|Default|GetSelectedScale))
                    (Utilities|IsValid (Variables|Default|GetSelectedBuilding) :!label _label_2
                      (:Is%20Valid
                        (Default|HighlightBuilding (Variables|Default|GetSelectedBuilding) false)
                        (Variables|Default|SetSelectedBuilding 0)
                        (goto _label Reset))))))))
          (:BaseMenu
            (bind _output_get_2 (Variables|Default|SetSelectedObject _hitcomponent))
            (Utilities|IsValid (Variables|Default|GetSelectedOpenMenu)
              (:Is%20Valid
                (for _array_element (Variables|/Game/UI/Buildings/BuildingClickable.BuildingClickable_C|GetMenusObjects (Variables|Default|GetSelectedOpenMenu))
                  (Transformation|SetRelativeScale3D _array_element "1.000000,1.000000,1.000000")
                  (Utilities|IsValid _output_get_2
                    (:Is%20Valid
                      (Transformation|SetRelativeScale3D _output_get_2 "1.200000,1.200000,1.200000")))))))
          (:BuildingBase
            (Variables|Default|SetSelectedObject _hitcomponent)
            (Utilities|IsValid _hitactor
              (:Is%20Valid
                (for _array_element_2 (Variables|Default|GetCurrentBuildings)
                  (Utilities|IsValid _array_element_2
                    (:Is%20Valid
                      (Default|HighlightBuilding _array_element_2 false))))
                (bind _asbp_building_base (Utilities|Casting|CastToBP_BuildingBase _hitactor))
                (bind _output_get_3 (Variables|Default|SetSelectedBuilding _asbp_building_base))
                (Default|HighlightBuilding _output_get_3 true)
                (if (not (Variables|/Game/BP_SpacePlayerController.BP_SpacePlayerController_C|GetIsMassCritical (Variables|Default|GetBP%20Space%20Player%20Controller)))
                  (Utilities|IsValid (Variables|Default|GetSelectedOpenMenu)
                    (:Is%20Valid
                      (Actor|DestroyActor (Variables|Default|GetSelectedOpenMenu))
                      (Variables|Default|SetSelectedOpenMenu 0))
                    (:Is%20Not%20Valid
                      _))
                  (for _array_element_3 (Variables|Default|GetSlotsArray)
                    (Rendering|SetVisibility _array_element_3 true false))
                  (CallFunction|TurnCollision true)
                  (Utilities|DeselectAllSlots)))))))
      (:Is%20Not%20Valid
        (Utilities|DeselectAllSlots
          (:Completed
            (Variables|Default|SetSelectedObject 0)
            (Utilities|FlowControl|Sequence
              (:then_0
                (goto _label Reset))
              (:then_1
                (goto _label_2)))))))))

(event Custom|ClickSelected
  (bind _bp_space_player_controller (Variables|Default|GetBP%20Space%20Player%20Controller))
  (bind _bp_space_player_controller_2 (Variables|Default|GetBP%20Space%20Player%20Controller))
  (bind _blackhole (Variables|/Game/BP_SpacePlayerController.BP_SpacePlayerController_C|GetBlackHole _bp_space_player_controller))
  (bind _tasksystem (Variables|/Game/BP_SpacePlayerController.BP_SpacePlayerController_C|GetTaskSystem _bp_space_player_controller_2))
  ;[1 1 1] ClickSelected
  (Utilities|IsValid (Variables|Default|GetSelectedObject)
    (:Is%20Valid
      (switch name (Utilities|Array|Get(acopy) (Variables|/Script/Engine.ActorComponent|GetComponentTags (Variables|Default|GetSelectedObject)))
        (:Slot
          (if (Variables|Default|GetSlotsAvailable)
            (if (Utilities|Array|IsNotEmpty (Variables|/Game/BP_SpacePlayerController.BP_SpacePlayerController_C|GetAvailableBuildings (Variables|Default|GetBP%20Space%20Player%20Controller)))
              (Utilities|IsValid (Variables|Default|GetSelectedOpenMenu)
                (:Is%20Valid
                  (for _array_element (Variables|Default|GetSlotsArray)
                    (Rendering|SetVisibility _array_element true false)
                    (Collision|SetCollisionEnabled _array_element "QueryAndPhysics"))
                  (Actor|DestroyActor (Variables|Default|GetSelectedOpenMenu)))
                (:Is%20Not%20Valid
                  _))
              (Utilities|IsValid (Variables|Default|GetSelectedObject)
                (:Is%20Valid
                  (Variables|Default|SetClickedSlot (Variables|Default|GetSelectedObject))
                  (Collision|SetCollisionEnabled (Variables|Default|GetSelectedObject) "NoCollision")
                  (Rendering|SetVisibility (Variables|Default|GetSelectedObject) false false)
                  (Transformation|SetWorldScale3D (Variables|Default|GetSelectedObject) (Variables|Default|GetDefaultSlotScale))
                  (bind _returnvalue (Game|SpawnActorfromClass "/Game/UI/Buildings/BuildingClickable.BuildingClickable_C" (Transformation|GetWorldTransform (Variables|Default|GetSelectedObject)) "Undefined" "MultiplyWithRoot" 0 0))
                  (bind _output_get (Variables|Default|SetSelectedOpenMenu _returnvalue))
                  (Transformation|AttachComponentToComponent _returnvalue (Variables|Default|GetSelectedObject) "None" "KeepWorld" "KeepWorld" "KeepRelative" true))))))
        (:BaseMenu
          (if (Variables|Default|GetSlotsAvailable)
            ;[1 1 1] BuildResearchBase
            (bind _aswidget_component (Utilities|Casting|CastToWidgetComponent (Variables|Default|GetSelectedObject)))
            (bind _aswbp_build_slot (Utilities|Casting|CastToWBP_BuildSlot (UserInterface|GetWidget _aswidget_component)))
            (if (> (- (Variables|/Script/DarkEraProject.BlackHole|GetCurrentMass _blackhole) (.Cost (Utilities|Struct|BreakBuildInformation (Variables|/Game/UI/Buildings/WBP_BuildSlot.WBP_BuildSlot_C|GetBuildStructure _aswbp_build_slot)))) 1e+02)
              (Variables|/Script/DarkEraProject.BlackHole|SetCurrentMass _blackhole (- (Variables|/Script/DarkEraProject.BlackHole|GetCurrentMass _blackhole) (.Cost (Utilities|Struct|BreakBuildInformation (Variables|/Game/UI/Buildings/WBP_BuildSlot.WBP_BuildSlot_C|GetBuildStructure _aswbp_build_slot)))))
              (switch string (.Tag (Utilities|Struct|BreakBuildInformation (Variables|/Game/UI/Buildings/WBP_BuildSlot.WBP_BuildSlot_C|GetBuildStructure _aswbp_build_slot)))
                (:ResearchBaseMenu
                  (bind _returnvalue_2 (Game|SpawnActorfromClass "/Game/UI/Buildings/BP_ResearchBase.BP_ResearchBase_C" (Math|Transform|MakeTransform (.location (Transformation|GetActorTransform (Variables|Default|GetSelectedOpenMenu))) "0, 0, 0" "1.000000,1.000000,1.000000") "AlwaysSpawn" "MultiplyWithRoot" 0 0))
                  (Variables|Default|SetSpawnedBuilding _returnvalue_2))
                (:MeteorBaseMenu
                  (bind _returnvalue_3 (Game|SpawnActorfromClass "/Game/UI/Buildings/BP_MeteorBase.BP_MeteorBase_C" (Math|Transform|MakeTransform (.location (Transformation|GetActorTransform (Variables|Default|GetSelectedOpenMenu))) "0, 0, 0" "1.000000,1.000000,1.000000") "AlwaysSpawn" "MultiplyWithRoot" 0 0))
                  (Variables|Default|SetSpawnedBuilding _returnvalue_3)))
              (Utilities|IsValid (Variables|Default|GetSpawnedBuilding)
                (:Is%20Valid
                  (Utilities|Array|Add (Variables|Default|GetCurrentBuildings) 0)
                  (Utilities|Array|RemoveItem (Variables|/Game/BP_SpacePlayerController.BP_SpacePlayerController_C|GetAvailableBuildings _bp_space_player_controller) (Variables|/Game/UI/Buildings/WBP_BuildSlot.WBP_BuildSlot_C|GetBuildStructure _aswbp_build_slot))
                  (Actor|DestroyActor (Variables|Default|GetSelectedOpenMenu))
                  (bind _aswidget_component_2 (Utilities|Casting|CastToWidgetComponent (Variables|Default|GetClickedSlot)))
                  (Utilities|Array|RemoveItem (Variables|Default|GetSlotsArray) _aswidget_component_2)
                  (Components|DestroyComponent (Variables|Default|GetClickedSlot))
                  (Transformation|AttachComponentToComponent (Variables|Default|GetSpawnedBuilding) (Variables|Default|GetScene) "None" "KeepWorld" "SnapToTarget" "KeepWorld" false)
                  (Utilities|FlowControl|DoOnce false
                    (:Completed
                      (Variables|/Game/BP_SpacePlayerController.BP_SpacePlayerController_C|SetCanResearch _bp_space_player_controller_2 true)
                      (Widget|SetIsEnabled (Variables|/Game/UI/HUD/WBP_GameHUD.WBP_GameHUD_C|GetResearchButton (Variables|/Game/UI/HUD/WBP_GeneralUI.WBP_GeneralUI_C|GetWBP_GameHUD (Variables|/Game/BP_SpacePlayerController.BP_SpacePlayerController_C|GetGeneralUI _bp_space_player_controller_2))) true)
                      (bind _returnvalue_4 (Utilities|GetDataTableRow "/Game/Tasks/TaskList.TaskList" "buildResearchBase")
                        (:then
                          (Default|CompleteTask _tasksystem _returnvalue_4)
                          (bind _returnvalue_5 (Utilities|GetDataTableRow "/Game/Tasks/TaskList.TaskList" "extractionResearch")
                            (:then
                              (Default|AddTask _tasksystem _returnvalue_5)
                              (bind _returnvalue_6 (Utilities|GetDataTableRow "/Game/Tasks/TaskList.TaskList" "flyRocketTo")
                                (:then
                                  (Default|AddTask _tasksystem _returnvalue_6))))))))))))))
        (:BuildingBase
          (switch name (Utilities|Array|Get(acopy) (Variables|/Script/Engine.ActorComponent|GetComponentTags (Variables|Default|GetSelectedObject)) 1)
            (:ResearchBase
              (Default|ToggleResearchMenu (Variables|Default|GetBP%20Space%20Player%20Controller))
              (Default|HighlightBuilding (Variables|Default|GetSelectedBuilding) false)
              (Variables|Default|SetSelectedBuilding 0)
              (Variables|Default|SetSelectedObject 0))))))))

(event Custom|TurnCollision
  (params (Enabled :type Boolean))
  ;[1 1 1] TurnCollision
  (for _array_element (Variables|Default|GetSlotsArray)
    (if Enabled
      (Collision|SetCollisionEnabled _array_element "QueryAndPhysics")
      (else
        (Collision|SetCollisionEnabled _array_element "NoCollision")))))

(event EventBeginPlay
  (bind _asbp_space_player_controller (Utilities|Casting|CastToBP_SpacePlayerController (Game|GetPlayerController 0)))
  (Variables|Default|SetBP%20Space%20Player%20Controller _asbp_space_player_controller)
  (Variables|Default|SetSlotsArray (Utilities|Array|MakeArray (Variables|Default|GetWidget6) (Variables|Default|GetWidget5) (Variables|Default|GetWidget4) (Variables|Default|GetWidget3) (Variables|Default|GetWidget2) (Variables|Default|GetWidget1) (Variables|Default|GetWidget7) (Variables|Default|GetWidget)))
  (Utilities|FlowControl|Delay 0.1)
  (CallFunction|SetGameColor (Variables|Default|GetColor))
  (bind _returnvalue (Utilities|Time|SetTimerbyEvent (delegate Custom|SetSpaceIntensity) 3.0 true))
  (Variables|Default|SetGameIntensityChangeTimer _returnvalue)
  (Utilities|Time|SetTimerbyEvent (delegate Custom|SelectObject) 0.1 true)
  (bind _outrownames (DataTable|GetDataTableRowNames "/Game/UI/Buildings/DT_Buildings.DT_Buildings"))
  (for _array_element _outrownames
    (bind _returnvalue_2 (Utilities|GetDataTableRow "/Game/UI/Buildings/DT_Buildings.DT_Buildings" _array_element)
      (:then
        (Utilities|Array|Add (Variables|/Game/BP_SpacePlayerController.BP_SpacePlayerController_C|GetAvailableBuildings (Variables|Default|GetBP%20Space%20Player%20Controller)) _returnvalue_2)))))

(event EventTick
  (params (DeltaSeconds :type Float%20%28single-precision%29))
  (for _array_element (Variables|Default|GetSlotsArray)
    (Utilities|LookatCamera _array_element)))

(fn ConstructionScript)