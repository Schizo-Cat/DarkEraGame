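; BP_Ship is the player's spaceship, which travels to a randomly spawned BP_BlackHole target and extracts its mass into the controller's black hole.
; A looping timer turns the ship toward the target, then fires the flamethrower and doubles black hole mass loss.
; Tick fakes flight by pulling the target toward the ship and updating a material-collection space offset, scaled by TimeSpeed.
; Arrival reveals the Extract button and resets mass loss.
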(event Custom|FlyToObject
  (bind _randommax (Variables|Default|GetRandomMax))
  (bind _randommin (Variables|Default|GetRandomMin))
  ;[1 1 1] trigger fly
  (Utilities|IsValid (Variables|Default|GetTargetFlyObject)
    (:Is%20Not%20Valid
      (bind _returnvalue (Game|SpawnActorfromClass "/Game/Blueprints/ExtructableObjects/BP_BlackHole.BP_BlackHole_C" (Math|Transform|MakeTransform (Math|Vector|MakeVector (Math|Conversions|ToFloat(Integer) (Math|Random|RandomIntegerinRange _randommin _randommax)) (Math|Conversions|ToFloat(Integer) (Math|Random|RandomIntegerinRange _randommin _randommax)) (Math|Conversions|ToFloat(Integer) (Math|Random|RandomIntegerinRange _randommin _randommax)))) "Undefined" "MultiplyWithRoot" 0 0))
      (Variables|Default|SetTargetFlyObject _returnvalue)
      (bind _returnvalue_2 (Utilities|Time|SetTimerbyEvent (delegate Custom|RotateToPlanet) 0.01 true))
      (Variables|Default|SetRotationTimer _returnvalue_2)
      (Default|MapToggle (Variables|Default|GetSpaceController)))))

(event Custom|RotateToPlanet
  (bind _returnvalue (Utilities|Time|GetWorldDeltaSeconds))
  (bind _rootcomponent (Variables|Transformation|GetRootComponent))
  (bind _targetflyobject (Variables|Default|GetTargetFlyObject))
  (bind _spacecontroller (Variables|Default|GetSpaceController))
  (bind _spacecontroller_2 (Variables|Default|GetSpaceController))
  (bind _returnvalue_2 (Transformation|GetWorldLocation _rootcomponent))
  (bind _returnvalue_3 (Transformation|GetActorLocation _targetflyobject))
  (bind _timespeed (Variables|/Script/DarkEraProject.SpacePlayerController|GettimeSpeed _spacecontroller))
  (bind _blackhole (Variables|/Game/BP_SpacePlayerController.BP_SpacePlayerController_C|GetBlackHole _spacecontroller_2))
  (bind _returnvalue_4 (Math|Rotator|FindLookatRotation _returnvalue_2 _returnvalue_3))
  ;[1 1 1] trigger fly
  (bind _output_get (Variables|Default|SettimerRotationValue (+ (Variables|Default|GettimerRotationValue) _returnvalue)))
  (Transformation|SetWorldRotation _rootcomponent (Math|Interpolation|RInterpTo (Transformation|GetWorldRotation _rootcomponent) _returnvalue_4 _returnvalue (/ _timespeed 1.0)) false false)
  (if (>= _output_get (- 5.0 _timespeed))
    (Utilities|Time|ClearandInvalidateTimerbyHandle (Variables|Default|GetRotationTimer))
    (Variables|Default|SettimerRotationValue 0.0)
    (Transformation|SetWorldRotation _rootcomponent _returnvalue_4 false false)
    (Components|Activation|Activate (Variables|Default|GetP_Flamethrower) false)
    (Variables|/Game/BP_SpacePlayerController.BP_SpacePlayerController_C|SetIstravelling _spacecontroller_2 true)
    (Variables|/Script/DarkEraProject.BlackHole|SetMassLossRate _blackhole (* (Variables|/Script/DarkEraProject.BlackHole|GetMassLossRate _blackhole) 2.0))))

(event Custom|ExtractObject
  (bind _spacecontroller (Variables|Default|GetSpaceController))
  (bind _spacecontroller_2 (Variables|Default|GetSpaceController))
  (bind _blackhole (Variables|/Game/BP_SpacePlayerController.BP_SpacePlayerController_C|GetBlackHole _spacecontroller_2))
  ;[1 1 1] ExtractObject
  (bind _asbp_space_body_base (Utilities|Casting|CastToBP_SpaceBodyBase (Variables|Default|GetTargetFlyObject)))
  (Variables|/Script/DarkEraProject.BlackHole|SetCurrentMass _blackhole (+ (Variables|/Game/Blueprints/ExtructableObjects/BP_SpaceBodyBase.BP_SpaceBodyBase_C|GetMass _asbp_space_body_base) (Variables|/Script/DarkEraProject.BlackHole|GetCurrentMass _blackhole)))
  (Actor|DestroyActor (Variables|Default|GetTargetFlyObject))
  (Variables|Default|SetTargetFlyObject 0)
  ;[1 1 1] Fly To object
  (Utilities|FlowControl|DoOnce false) ; enters at Reset
)

(event EventBeginPlay
  (Components|Activation|Deactivate (Variables|Default|GetP_Flamethrower))
  (bind _asbp_space_player_controller (Utilities|Casting|CastToBP_SpacePlayerController (Game|GetPlayerController 0)))
  (Variables|Default|SetSpaceController _asbp_space_player_controller))

(event EventTick
  (params (DeltaSeconds :type Float%20%28single-precision%29))
  (bind _returnvalue (Transformation|GetActorLocation))
  (bind _returnvalue_2 (Utilities|Time|GetWorldDeltaSeconds))
  (bind _spacecontroller (Variables|Default|GetSpaceController))
  (bind _targetflyobject (Variables|Default|GetTargetFlyObject))
  (bind _spacecontroller_2 (Variables|Default|GetSpaceController))
  (bind _returnvalue_3 (Transformation|GetActorLocation _targetflyobject))
  (bind _returnvalue_4 (/ _returnvalue_2 2e+01))
  (bind _timespeed (Variables|/Script/DarkEraProject.SpacePlayerController|GettimeSpeed _spacecontroller_2))
  (bind _returnvalue_5 (* _returnvalue_4 _timespeed))
  (bind _returnvalue_6 (Math|Vector|Lerp(Vector) _returnvalue_3 _returnvalue _returnvalue_5))
  ;[1 1 1] Fly To object
  (Utilities|IsValid (Variables|Default|GetTargetFlyObject)
    (:Is%20Valid
      (if (Variables|/Game/BP_SpacePlayerController.BP_SpacePlayerController_C|GetIstravelling (Variables|Default|GetSpaceController))
        (if (not (Variables|/Script/DarkEraProject.SpacePlayerController|GetIsTimeFrozen _spacecontroller_2))
          (if (>= (Math|Vector|Distance(Vector) _returnvalue_6 _returnvalue) 1.5e+02)
            (Transformation|SetActorLocation (Variables|Default|GetTargetFlyObject) _returnvalue_6 false false)
            (Rendering|Material|SetVectorParameterValue "/Game/Materials/MPC_Collection.MPC_Collection" "spaceOffset" (Math|Conversions|ToLinearColor(Vector) (- "" _returnvalue_6)) :!class /Script/Engine.KismetMaterialLibrary)
            (else
              (Utilities|FlowControl|DoOnce false
                (:Completed
                  (Components|Activation|Deactivate (Variables|BP_Ship_C|GetP_Flamethrower (Variables|/Game/BP_SpacePlayerController.BP_SpacePlayerController_C|GetSpaceShip _spacecontroller)))
                  (Widget|SetVisibility (Variables|/Game/UI/WBP_GameHUD.WBP_GameHUD_C|GetExtractButton (Variables|/Game/UI/WBP_GeneralUI.WBP_GeneralUI_C|GetWBP_GameHUD (Variables|/Game/BP_SpacePlayerController.BP_SpacePlayerController_C|GetGeneralUI _spacecontroller))) "Visible")
                  (Variables|/Game/BP_SpacePlayerController.BP_SpacePlayerController_C|SetIstravelling _spacecontroller false)
                  (Variables|/Script/DarkEraProject.BlackHole|SetMassLossRate (Variables|/Game/BP_SpacePlayerController.BP_SpacePlayerController_C|GetBlackHole _spacecontroller) 1.0))))))))))

(fn ConstructionScript)