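; Actor that drives the singularity mode's visuals: a growing black hole, rotating Increasers with lights, and the return to base.
; UpdateHoleVisuals maps one progress value onto hole material, camera offset, ship and base transforms, and UI, blending a color palette across lights, surroundings and widgets.
; LeaveSingularity starts a looping timer that lerps the spectator back, then resets the scene and game state.
; BeginPlay creates the hole's dynamic material and starts TimeSpeed-scaled rotation.
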(event Custom|RotateBase
  (bind _increasers (Variables|Default|GetIncreasers))
  (Transformation|SetRelativeRotation _increasers (Math|Rotator|MakeRotator 0.0 0.0 (+ (.yaw (Variables|/Script/Engine.SceneComponent|GetRelativeRotation _increasers)) (* 0.05 (Variables|/Script/DarkEraProject.SpacePlayerController|GettimeSpeed (stale EventBeginPlay _output_get))))) false false))

(event Custom|SetLightsColor
  (params (NewLightColor :type Linear%20Color%20Structure))
  (for _array_element (Utilities|Array|MakeArray (Variables|Default|GetPointLight5) (Variables|Default|GetPointLight7) (Variables|Default|GetPointLight4) (Variables|Default|GetPointLight3) (Variables|Default|GetPointLight2) (Variables|Default|GetPointLight1) (Variables|Default|GetPointLight) (Variables|Default|GetPointLight6))
    (Rendering|Components|Light|SetLightColor _array_element NewLightColor true)))

(event Custom|UpdateHoleVisuals
  (params (A :type Float%20%28double-precision%29))
  (bind _spacecontroller (Variables|Default|GetSpaceController))
  (bind _spacecontroller_2 (Variables|Default|GetSpaceController))
  (bind _colorsarray (Variables|Default|GetColorsArray))
  (bind _spacecontroller_3 (Variables|Default|GetSpaceController))
  (bind _spacecontroller_4 (Variables|Default|GetSpaceController))
  (bind _spacecontroller_5 (Variables|Default|GetSpaceController))
  (bind _abdynamicmaterial (Variables|Default|GetABDynamicMaterial))
  (bind _spaceship (Variables|/Game/BP_SpacePlayerController.BP_SpacePlayerController_C|GetSpaceShip _spacecontroller))
  (bind _generalui (Variables|/Game/BP_SpacePlayerController.BP_SpacePlayerController_C|GetGeneralUI _spacecontroller_4))
  (bind _spaceship_2 (Variables|/Game/BP_SpacePlayerController.BP_SpacePlayerController_C|GetSpaceShip _spacecontroller_3))
  (bind _generalui_2 (Variables|/Game/BP_SpacePlayerController.BP_SpacePlayerController_C|GetGeneralUI _spacecontroller_5))
  (bind _indicator (Variables|/Game/Blueprints/BP_Ship.BP_Ship_C|GetIndicator _spaceship))
  (bind _wbp_singularitywindow (Variables|/Game/UI/HUD/WBP_GeneralUI.WBP_GeneralUI_C|GetWBP_SingularityWindow _generalui_2))
  (bind _wbp_singularitywindow_2 (Variables|/Game/UI/HUD/WBP_GeneralUI.WBP_GeneralUI_C|GetWBP_SingularityWindow _generalui))
  (bind _output_get (Variables|Default|SetLerpTrack A))
  (Variables|/Game/BP_SpacePlayerController.BP_SpacePlayerController_C|SetSingularityProgression (Variables|Default|GetSpaceController) _output_get)
  (if (> (Variables|Default|GetLerpTrack) 0.3)
    (Variables|/Game/BP_SpacePlayerController.BP_SpacePlayerController_C|SetSingularityOffset _spacecontroller_2 (Math|Vector|MakeVector (Math|Float|Lerp 4e+03 1.5e+04 (Variables|Default|GetLerpTrack)) 0.0 0.0))
    (Variables|/Script/Engine.SpringArmComponent|SetSocketOffset (Variables|/Game/BP_SpectatorPawn.BP_SpectatorPawn_C|GetSpringArm (Variables|/Game/BP_SpacePlayerController.BP_SpacePlayerController_C|GetBP_spectator _spacecontroller_2)) (- "" (Variables|/Game/BP_SpacePlayerController.BP_SpacePlayerController_C|GetSingularityOffset _spacecontroller_2))))
  (Rendering|Material|SetScalarParameterValue _abdynamicmaterial "Emission_Intensity" (Math|Float|Lerp 0.001 0.1 (Variables|Default|GetLerpTrack)) :!class /Script/Engine.MaterialInstanceDynamic)
  (Rendering|Material|SetScalarParameterValue _abdynamicmaterial "Blackhole_Size" (* (Variables|Default|GetLerpTrack) 2e+01) :!class /Script/Engine.MaterialInstanceDynamic)
  (if (< (Variables|Default|GetLerpTrack) 0.65)
    (Rendering|Material|SetScalarParameterValue _abdynamicmaterial "Ring_Intensity_falloff" (+ (* (Variables|Default|GetLerpTrack) 2.5) 1.5) :!class /Script/Engine.MaterialInstanceDynamic))
  (Rendering|Material|SetScalarParameterValue _abdynamicmaterial "Ring_speed" (Math|Float|Lerp 0.001 1.2 (Variables|Default|GetLerpTrack)) :!class /Script/Engine.MaterialInstanceDynamic)
  (if (> (Variables|Default|GetLerpTrack) 0.5)
    (Transformation|SetRelativeScale3D (Variables|Default|GetIncreasers) (Math|Vector|MakeVector (* (Variables|Default|GetLerpTrack) 3.0) (* (Variables|Default|GetLerpTrack) 3.0) (* (Variables|Default|GetLerpTrack) 3.0))))
  (Variables|Default|SetCurrentColorIndex (Math|Conversions|ToInteger(Byte) (Class|KismetMathLibrary|ToInt64(Float) (Math|Float|Lerp 0.0 6.9 (Variables|Default|GetLerpTrack)))))
  (Rendering|Material|SetVectorParameterValue _abdynamicmaterial "Disk_Color" (Math|Color|Lerp(LinearColor) (Utilities|Array|Get(acopy) _colorsarray (Variables|Default|GetCurrentColorIndex)) (Utilities|Array|Get(acopy) _colorsarray (Math|Integer|%(Integer) (+ (Variables|Default|GetCurrentColorIndex) 1) (Utilities|Array|Length _colorsarray))) (Math|Float|Lerp 0.0 1.0 (- (Math|Float|Lerp 0.0 6.9 (Variables|Default|GetLerpTrack)) (Variables|Default|GetCurrentColorIndex)))) :!class /Script/Engine.MaterialInstanceDynamic)
  (Progress|SetPercent (Variables|/Game/UI/SingularityWindow/WBP_SingularityWindow.WBP_SingularityWindow_C|GetProgressBar_Temperature _wbp_singularitywindow_2) (Variables|Default|GetLerpTrack))
  (Default|SetGameColor (Variables|/Game/BP_SpacePlayerController.BP_SpacePlayerController_C|GetBaseSurrounding _spacecontroller_4) (Math|Color|Lerp(LinearColor) (Utilities|Array|Get(acopy) _colorsarray (Variables|Default|GetCurrentColorIndex)) (Utilities|Array|Get(acopy) _colorsarray (Math|Integer|%(Integer) (+ (Variables|Default|GetCurrentColorIndex) 1) (Utilities|Array|Length _colorsarray))) (Math|Float|Lerp 0.0 1.0 (- (Math|Float|Lerp 0.0 6.9 (Variables|Default|GetLerpTrack)) (Variables|Default|GetCurrentColorIndex)))))
  (CallFunction|SetLightsColor (Math|Color|Lerp(LinearColor) (Utilities|Array|Get(acopy) _colorsarray (Variables|Default|GetCurrentColorIndex)) (Utilities|Array|Get(acopy) _colorsarray (Math|Integer|%(Integer) (+ (Variables|Default|GetCurrentColorIndex) 1) (Utilities|Array|Length _colorsarray))) (Math|Float|Lerp 0.0 1.0 (- (Math|Float|Lerp 0.0 6.9 (Variables|Default|GetLerpTrack)) (Variables|Default|GetCurrentColorIndex)))))
  (Rendering|Components|TextRender|SetText (Variables|/Game/UI/SingularityWindow/WBP_SingularityWindow.WBP_SingularityWindow_C|GetMassPlankText _wbp_singularitywindow_2) (Utilities|Text|ToText(Float) (Math|Float|Lerp 0.0 21.76 (Variables|Default|GetLerpTrack)) "HalfToEven" false true 1 324 0 2))
  (Transformation|SetRelativeScale3D (Variables|/Script/Engine.Actor|GetRootComponent _spaceship_2) (Math|Vector|MakeVector (Math|Float|Lerp 0.2 0.01 (Variables|Default|GetLerpTrack)) (Math|Float|Lerp 0.2 0.01 (Variables|Default|GetLerpTrack)) (Math|Float|Lerp 0.2 0.01 (Variables|Default|GetLerpTrack))))
  (Rendering|SetVisibility (Variables|/Game/Blueprints/BP_MainBlackHole.BP_MainBlackHole_C|GetDefaultSceneRoot (Variables|/Game/BP_SpacePlayerController.BP_SpacePlayerController_C|GetBlackHole _spacecontroller_3)) false true)
  (Transformation|SetActorLocation (Variables|/Game/BP_SpacePlayerController.BP_SpacePlayerController_C|GetBaseSurrounding _spacecontroller_3) (Math|Vector|MakeVector (Math|Float|Lerp -2e+03 -1e+04 (Variables|Default|GetLerpTrack)) 0.0 0.0) false false)
  (Transformation|SetActorLocation _spaceship_2 (Math|Vector|MakeVector (Math|Float|Lerp -2e+03 -1e+04 (Variables|Default|GetLerpTrack)) 0.0 0.0) false false)
  (Rendering|SetVisibility _indicator (> (Variables|Default|GetLerpTrack) 0.5) false)
  (Class|WidgetComponent|SetDrawSize _indicator (Math|Vector2D|MakeVector2D (Math|Float|Lerp 25.0 75.0 (Variables|Default|GetLerpTrack)) (Math|Float|Lerp 25.0 75.0 (Variables|Default|GetLerpTrack))))
  (if (> (Variables|Default|GetLerpTrack) 0.85)
    (if (> (Variables|Default|GetLerpTrack) 0.975)
      (Transformation|SetRelativeLocation _indicator (Math|Vector|MakeVector 3e+04 0.0 0.0) false false)
      (else
        (Transformation|SetRelativeLocation _indicator (Math|Vector|MakeVector 1e+04 0.0 0.0) false false)))
    (else
      (Transformation|SetRelativeLocation _indicator (Math|Vector|MakeVector (Math|Float|Lerp 1e+03 5e+03 (Variables|Default|GetLerpTrack)) 0.0 0.0) false false)))
  (CallFunction|ScaleIncreasers (Math|Float|Lerp 0.03 0.003 (Variables|Default|GetLerpTrack)))
  (Appearance|SetColorandOpacity (Variables|/Game/UI/SingularityWindow/WBP_SingularityWindow.WBP_SingularityWindow_C|GetLeftPannel _wbp_singularitywindow) (Math|Color|Lerp(LinearColor) (Utilities|Array|Get(acopy) _colorsarray (Variables|Default|GetCurrentColorIndex)) (Utilities|Array|Get(acopy) _colorsarray (Math|Integer|%(Integer) (+ (Variables|Default|GetCurrentColorIndex) 1) (Utilities|Array|Length _colorsarray))) (Math|Float|Lerp 0.0 1.0 (- (Math|Float|Lerp 0.0 6.9 (Variables|Default|GetLerpTrack)) (Variables|Default|GetCurrentColorIndex)))) :!class /Script/UMG.Image)
  (Class|Button|SetBackgroundColor (Variables|/Game/UI/SingularityWindow/WBP_SingularityWindow.WBP_SingularityWindow_C|GetStructuresButton _wbp_singularitywindow) (Math|Color|Lerp(LinearColor) (Utilities|Array|Get(acopy) _colorsarray (Variables|Default|GetCurrentColorIndex)) (Utilities|Array|Get(acopy) _colorsarray (Math|Integer|%(Integer) (+ (Variables|Default|GetCurrentColorIndex) 1) (Utilities|Array|Length _colorsarray))) (Math|Float|Lerp 0.0 1.0 (- (Math|Float|Lerp 0.0 6.9 (Variables|Default|GetLerpTrack)) (Variables|Default|GetCurrentColorIndex))))))

(event Custom|ScaleIncreasers
  (params (New%20Scale%203D%20X :type Float%20%28double-precision%29))
  (for _array_element (Utilities|Array|MakeArray (Variables|Default|GetaBP_Increaser2) (Variables|Default|GetaBP_Increaser3) (Variables|Default|GetaBP_Increaser1) (Variables|Default|GetaBP_Increaser7) (Variables|Default|GetaBP_Increaser6) (Variables|Default|GetaBP_Increaser5) (Variables|Default|GetaBP_Increaser4) (Variables|Default|GetaBP_Increaser))
    (Transformation|SetRelativeScale3D _array_element (Math|Conversions|ToVector(Float) New%20Scale%203D%20X))))

(event Custom|LeaveSingularity
  ;[1 1 1] LeaveSingularity
  (bind _returnvalue (Utilities|Time|SetTimerbyEvent (delegate Custom|BackToBase) 0.001 true))
  (Variables|Default|SetBackToBaseAnimation _returnvalue))

(event Custom|BackToBase
  (bind _spacecontroller (Variables|Default|GetSpaceController))
  (bind _spacecontroller_2 (Variables|Default|GetSpaceController))
  (bind _spacecontroller_3 (Variables|Default|GetSpaceController))
  (bind _spacecontroller_4 (Variables|Default|GetSpaceController))
  (bind _bp_spectator (Variables|/Game/BP_SpacePlayerController.BP_SpacePlayerController_C|GetBP_spectator _spacecontroller))
  (bind _blackhole (Variables|/Game/BP_SpacePlayerController.BP_SpacePlayerController_C|GetBlackHole _spacecontroller_2))
  ;[1 1 1] AnimationToBase
  (bind _output_get (Variables|Default|SetSingularityClose (+ (Variables|Default|GetSingularityClose) 0.001)))
  (Transformation|SetActorLocation _bp_spectator (Math|Vector|MakeVector (Math|Float|Lerp 0.0 (.x (Transformation|GetActorLocation (Variables|/Game/BP_SpacePlayerController.BP_SpacePlayerController_C|GetSpaceShip _spacecontroller))) _output_get) 0.0 0.0) false false)
  (Variables|/Script/Engine.SpringArmComponent|SetSocketOffset (Variables|/Game/BP_SpectatorPawn.BP_SpectatorPawn_C|GetSpringArm _bp_spectator) (Math|Vector|MakeVector (Math|Float|Lerp (.X (Math|Vector|BreakVector (- "" (Variables|/Game/BP_SpacePlayerController.BP_SpacePlayerController_C|GetSingularityOffset _spacecontroller)))) 0.0 (Variables|Default|GetSingularityClose)) 0.0 0.0))
  (if (>= (Variables|Default|GetSingularityClose) 1.0)
    (Utilities|Time|ClearandInvalidateTimerbyHandle (Variables|Default|GetBackToBaseAnimation))
    (Rendering|SetActorHiddenInGame (Variables|Default|GetSingularityHole) true)
    (Rendering|SetActorHiddenInGame (Variables|/Game/BP_SpacePlayerController.BP_SpacePlayerController_C|GetBaseSurrounding _spacecontroller_3) false)
    (Rendering|SetVisibility (Variables|/Game/Blueprints/BP_Ship.BP_Ship_C|GetIndicator (Variables|/Game/BP_SpacePlayerController.BP_SpacePlayerController_C|GetSpaceShip _spacecontroller_3)) false false)
    (Transformation|SetActorLocation (Variables|/Game/BP_SpacePlayerController.BP_SpacePlayerController_C|GetBP_spectator _spacecontroller_4) "0, 0, 0" false false)
    (Transformation|SetActorLocation (Variables|/Game/BP_SpacePlayerController.BP_SpacePlayerController_C|GetBaseSurrounding _spacecontroller_4) "0, 0, 0" false false)
    (Transformation|SetActorLocation (Variables|/Game/BP_SpacePlayerController.BP_SpacePlayerController_C|GetSpaceShip _spacecontroller_4) "0, 0, 0" false false)
    (Transformation|SetActorLocation (Variables|/Game/BP_SpacePlayerController.BP_SpacePlayerController_C|GetBlackHole _spacecontroller_4) "0, 0, 0" false false)
    (Variables|/Script/UMG.WidgetSwitcher|SetActiveWidgetIndex (Variables|/Game/UI/HUD/WBP_GeneralUI.WBP_GeneralUI_C|GetHudmenus (Variables|/Game/BP_SpacePlayerController.BP_SpacePlayerController_C|GetGeneralUI _spacecontroller_4)) 0)
    (Variables|/Game/BP_SpacePlayerController.BP_SpacePlayerController_C|SetIsSingularityMode _spacecontroller_2 false)
    (Default|ChangeGameState _spacecontroller_2)
    (Widget|SetVisibility (Variables|/Game/UI/Map/WBP_Map.WBP_Map_C|GetMassiveBlackHolesOverlay (Variables|/Game/UI/HUD/WBP_GeneralUI.WBP_GeneralUI_C|GetWBP_Map (Variables|/Game/BP_SpacePlayerController.BP_SpacePlayerController_C|GetGeneralUI _spacecontroller_2))) "Hidden")
    (Transformation|SetActorRelativeScale3D (Variables|/Game/BP_SpacePlayerController.BP_SpacePlayerController_C|GetSpaceShip _spacecontroller_2) "0.200000,0.200000,0.200000")
    (Rendering|SetVisibility (Variables|/Game/Blueprints/BP_MainBlackHole.BP_MainBlackHole_C|GetSphere _blackhole) true true)
    (Transformation|SetActorRelativeScale3D _blackhole "1.000000,1.000000,1.000000")
    (Variables|Default|SetSingularityClose 0.0)
    (Actor|DestroyActor (Variables|/Game/Blueprints/BP_Ship.BP_Ship_C|GetTargetFlyObject (Variables|/Game/BP_SpacePlayerController.BP_SpacePlayerController_C|GetSpaceShip (Variables|Default|GetSpaceController))))))

(event EventBeginPlay
  (bind _asbp_space_player_controller (Utilities|Casting|CastToBP_SpacePlayerController (Game|GetPlayerController 0)))
  (bind _output_get (Variables|Default|SetSpaceController _asbp_space_player_controller))
  (Utilities|Time|SetTimerbyEvent (delegate Custom|RotateBase) 0.01 true)
  (bind _returnvalue (Actor|GetActorOfClass "/Game/Materials/BlackHoleAdvanced/BP_BlackHoleAdvanced.BP_BlackHoleAdvanced_C"))
  (bind _output_get_2 (Variables|Default|SetSingularityHole _returnvalue))
  (bind _returnvalue_2 (Rendering|Material|CreateDynamicMaterialInstance (Variables|/Game/Materials/BlackHoleAdvanced/BP_BlackHoleAdvanced.BP_BlackHoleAdvanced_C|GetStaticMesh _output_get_2) 0 "/Game/Materials/BlackHoleAdvanced/M_BlackHoleAdvanced_Inst.M_BlackHoleAdvanced_Inst" "None" :!class /Script/Engine.PrimitiveComponent))
  (Variables|Default|SetABDynamicMaterial _returnvalue_2))

(fn ConstructionScript)