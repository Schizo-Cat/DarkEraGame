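; Voice-over manager that plays VO lines through one audio component and shows their subtitles in a viewport widget.
; Normal lines join MediaQueue and play in order without spatialization or attenuation, each advancing on a delay based on clip duration.
; Important lines clear the queue and stop current audio first.
; Skipping stops audio and clears text, leaving the timed queue untouched; the sound-mix cleanup binding is never executed.
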(event Custom|RemoveSoundMix
  (Audio|PopSoundMixModifier 0)
  (Audio|PopSoundMixModifier 0))

(event Custom|PlayVO
  (params (VOData :type VO%20Structure%20Structure))
  (bind _vofile (Utilities|Struct|BreakVOStructure VOData))
  ;[1 1 1] Playing VOs
  (Utilities|IsValid _vofile
    (:Is%20Valid
      (Variables|Default|SetCurrentAudio _vofile)
      (Utilities|PlayMedia VOData))))

(event Custom|PlayVOImportant
  (params (VOData :type VO%20Structure%20Structure))
  ;[1 1 1] Playing VOs
  (CallFunction|StopPlaying)
  (CallFunction|PlayVO VOData))

(event EventBeginPlay
  (bind _returnvalue (UserInterface|CreateWidget "/Game/VO/WBP_VOSubtitles.WBP_VOSubtitles_C"))
  (bind _output_get (Variables|Default|SetSubtitlesWidget _returnvalue))
  (UserInterface|Viewport|AddtoViewport _output_get 0)
  (CallFunction|SetSubtitlesVisibility true))

(fn ConstructionScript)

(fn SetSubtitlesVisibility
  (params (State :type Boolean))
  (bind _subtitleswidget (Variables|Default|GetSubtitlesWidget))
  (if State
    (Widget|SetVisibility _subtitleswidget "Visible")
    (else
      (Widget|SetVisibility _subtitleswidget "Collapsed"))))

(fn StopPlaying
  (Utilities|Array|Clear (Variables|Default|GetMediaQueue))
  (bind _audio (Variables|Default|GetAudio)
    (:then
      (Audio|Components|Audio|Stop _audio))
    (:else)))

(fn SkipVO
  (Utilities|IsValid (Variables|Default|GetCurrentAudio)
    (:Is%20Valid
      (bind _audio (Variables|Default|GetAudio)
        (:then
          (Audio|Components|Audio|Stop _audio)
          (Default|ClearText (Variables|Default|GetSubtitlesWidget)))
        (:else)))))