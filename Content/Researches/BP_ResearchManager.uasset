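; Research manager that runs the active research over time, scaled by the player controller's time speed.
; Tick accumulates progress and updates the research window and a material parameter collection scalar against the research's duration.
; At a fixed threshold of 100 it adds the journal entry, applies Warp Drive or Hawking Radiation ship unlocks, the latter also advancing tasks, then resets.
; Starting and finishing research both call the controller's game-state change.
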(event Custom|SetResearch
  (params (CurrentResearch :type Research%20Structure%20Structure))
  (Variables|Default|SetCurrentResearch CurrentResearch)
  (Variables|Default|SetIsResearching true)
  (Default|ChangeGameState (Variables|Default|GetBP%20Space%20Player%20Controller)))

(event EventTick
  (params (DeltaSeconds :type Float%20%28single-precision%29))
  (bind _bp_space_player_controller (Variables|Default|GetBP%20Space%20Player%20Controller))
  (bind _generalui (Variables|/Game/BP_SpacePlayerController.BP_SpacePlayerController_C|GetGeneralUI _bp_space_player_controller))
  (bind _spaceship (Variables|/Game/BP_SpacePlayerController.BP_SpacePlayerController_C|GetSpaceShip _bp_space_player_controller))
  (bind _tasksystem (Variables|/Game/BP_SpacePlayerController.BP_SpacePlayerController_C|GetTaskSystem _bp_space_player_controller))
  (Utilities|IsValid (.image (Variables|Default|GetCurrentResearch))
    (:Is%20Valid
      (if (!= (.timeforresearch (Variables|Default|GetCurrentResearch)) 0.0)
        (Variables|Default|SetResearchProgress (+ (* DeltaSeconds (Variables|/Script/DarkEraProject.SpacePlayerController|GettimeSpeed _bp_space_player_controller)) (Variables|Default|GetResearchProgress)))
        (Utilities|SetUIProgress (.timeforresearch (Variables|Default|GetCurrentResearch)))
        (if (>= (Variables|Default|GetResearchProgress) 1e+02)
          (bind _returnvalue (Utilities|GetDataTableRow (.DataTable (Utilities|Struct|BreakDataTableRowHandle (.entry (Variables|Default|GetCurrentResearch)))) (.RowName (Utilities|Struct|BreakDataTableRowHandle (.entry (Variables|Default|GetCurrentResearch)))))
            (:then
              (Default|AddEntry (Variables|/Game/UI/HUD/WBP_GeneralUI.WBP_GeneralUI_C|GetWBP_JournalWidget _generalui) _returnvalue))
            (:RowNotFound
              _))
          (Utilities|FlowControl|Sequence
            (:then_0
              (switch name (.RowName (Utilities|Struct|BreakDataTableRowHandle (.entry (Variables|Default|GetCurrentResearch))))
                (:warpDrive
                  (Default|TurnWarpDriver _spaceship)
                  (Math|Integer|IncrementInt (Variables|/Game/BP_SpacePlayerController.BP_SpacePlayerController_C|GetCurrentRangeAbility _bp_space_player_controller)))
                (:hawkingRadiation
                  (Default|TurnExtractor _spaceship)
                  (bind _returnvalue_2 (Utilities|GetDataTableRow "/Game/Tasks/TaskList.TaskList" "extractionResearch")
                    (:then
                      (Default|CompleteTask _tasksystem _returnvalue_2)
                      (bind _returnvalue_3 (Utilities|GetDataTableRow "/Game/Tasks/TaskList.TaskList" "extractBlackHoles")
                        (:then
                          (Default|AddTask _tasksystem _returnvalue_3))))))))
            (:then_1
              (Variables|Default|SetCurrentResearch "")
              (Variables|Default|SetResearchProgress 0.0)
              (Utilities|SetUIProgress 0.0)
              (Rendering|Components|TextRender|SetText (Variables|/Game/UI/ResearchWindow/ResearchWindow.ResearchWindow_C|GetPercentText (Variables|/Game/UI/HUD/WBP_GeneralUI.WBP_GeneralUI_C|GetResearchWindow _generalui)) "")
              (Variables|Default|SetIsResearching false)
              (Default|ChangeGameState (Variables|Default|GetBP%20Space%20Player%20Controller)))))))))

(event EventBeginPlay
  (bind _asbp_space_player_controller (Utilities|Casting|CastToBP_SpacePlayerController (Game|GetPlayerController 0)))
  (Variables|Default|SetBP%20Space%20Player%20Controller _asbp_space_player_controller))

(fn ConstructionScript)