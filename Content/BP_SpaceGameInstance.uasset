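; Game instance for the space game that persists player progress and audio settings.
; On level load it signals whether a save exists, and SaveGame writes black hole name, mass, research, tasks and journal from the player controller to the save slot.
; Settings load lazily into their own save object, with Music, SFX and Voice volumes applied as SMIX_Main class overrides and mirrored on the controller's AudioMix.
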(event Custom|FinishLevelLoaded
  (bind _returnvalue (SaveGame|LoadGamefromSlot "Save"))
  (bind _asbp_save_object (Utilities|Casting|CastToBP_SaveObject _returnvalue)
    (:then
      (Utilities|IsValid _asbp_save_object
        (:Is%20Valid
          (Default|CallOnSaveLoaded))
        (:Is%20Not%20Valid
          (Default|CallOnLoadWithoutSave :!label _label))))
    (:CastFailed
      (goto _label))))

(fn SaveSettings
  (bind _returnvalue (SaveGame|DoesSaveGameExist (Variables|Default|GetSettingsSave)))
  (if _returnvalue
    _
    (else
      (Utilities|IsValid (Variables|Default|GetSettingsSaveObject)
        (:Is%20Valid
          _)
        (:Is%20Not%20Valid
          (bind _returnvalue_2 (SaveGame|CreateSaveGameObject "/Game/SaveGame/BP_Setting_SaveGame.BP_Setting_SaveGame_C"))
          (Variables|Default|SetSettingsSaveObject _returnvalue_2)))))
  (bind _returnvalue_3 (Actor|GetActorOfClass "/Game/BP_SpacePlayerController.BP_SpacePlayerController_C"))
  (Variables|/Game/SaveGame/BP_Setting_SaveGame.BP_Setting_SaveGame_C|SetAudioMix (CallFunction|GetSettings) (Variables|/Game/BP_SpacePlayerController.BP_SpacePlayerController_C|GetAudioMix _returnvalue_3))
  (SaveGame|SaveGametoSlot (Variables|Default|GetSettingsSaveObject) (Variables|Default|GetSettingsSave))
  (return))

(fn InitAudioMixSettings
  (bind _settingssaveobject (Variables|Default|GetSettingsSaveObject))
  (bind _audiomix (Variables|/Game/SaveGame/BP_Setting_SaveGame.BP_Setting_SaveGame_C|GetAudioMix _settingssaveobject))
  (Utilities|FlowControl|Sequence
    (:then_0
      (Audio|SetSoundMixClassOverride "/Engine/EngineSounds/SMIX_Main.SMIX_Main" "/Engine/EngineSounds/Music.Music" (.music _audiomix) 1.0 0.0 true))
    (:then_1
      (Audio|SetSoundMixClassOverride "/Engine/EngineSounds/SMIX_Main.SMIX_Main" "/Engine/EngineSounds/SFX.SFX" (.effects _audiomix) 1.0 0.0 true))
    (:then_2
      (Audio|SetSoundMixClassOverride "/Engine/EngineSounds/SMIX_Main.SMIX_Main" "/Engine/EngineSounds/Voice.Voice" (.voice _audiomix) 1.0 0.0 true))))

(fn InitSettings
  (CallFunction|InitAudioMixSettings)
  (bind _returnvalue (Actor|GetActorOfClass "/Game/BP_SpacePlayerController.BP_SpacePlayerController_C"))
  (Variables|/Game/BP_SpacePlayerController.BP_SpacePlayerController_C|SetAudioMix _returnvalue (Variables|/Game/SaveGame/BP_Setting_SaveGame.BP_Setting_SaveGame_C|GetAudioMix (Variables|Default|GetSettingsSaveObject))))

(fn LoadSettings
  (bind _returnvalue (SaveGame|DoesSaveGameExist (Variables|Default|GetSettingsSave)))
  (if _returnvalue
    (bind _returnvalue_2 (SaveGame|LoadGamefromSlot (Variables|Default|GetSettingsSave)))
    (bind _asbp_setting_save_game (Utilities|Casting|CastToBP_Setting_SaveGame _returnvalue_2))
    (Variables|Default|SetSettingsSaveObject _asbp_setting_save_game)
    (else
      (bind _returnvalue_3 (SaveGame|CreateSaveGameObject "/Game/SaveGame/BP_Setting_SaveGame.BP_Setting_SaveGame_C"))
      (Variables|Default|SetSettingsSaveObject _returnvalue_3)))
  (CallFunction|InitSettings)
  (return))

(fn GetSettings
  (bind _settingssaveobject (Variables|Default|GetSettingsSaveObject))
  (Utilities|IsValid _settingssaveobject
    (:Is%20Valid
      (return _settingssaveobject))
    (:Is%20Not%20Valid
      (CallFunction|LoadSettings)
      (return (Variables|Default|GetSettingsSaveObject)))))

(fn UpdateSoundMix
  (params (InSoundClass :type E_SoundClasses%20Enum :default "NewEnumerator0") (Volume :type Float%20%28single-precision%29))
  (switch Utilities|FlowControl|Switch|SwitchonE_SoundClasses InSoundClass
    (:NewEnumerator0
      (Audio|SetSoundMixClassOverride "/Engine/EngineSounds/SMIX_Main.SMIX_Main" "/Engine/EngineSounds/Music.Music" Volume 1.0 0.0 true)
      (bind _returnvalue (Actor|GetActorOfClass "/Game/BP_SpacePlayerController.BP_SpacePlayerController_C"))
      (Utilities|Struct|SetmembersinF_AudioMix (Variables|/Game/BP_SpacePlayerController.BP_SpacePlayerController_C|GetAudioMix _returnvalue) Volume)
      (Audio|PushSoundMixModifier "/Engine/EngineSounds/SMIX_Main.SMIX_Main"))
    (:NewEnumerator1
      (Audio|SetSoundMixClassOverride "/Engine/EngineSounds/SMIX_Main.SMIX_Main" "/Engine/EngineSounds/SFX.SFX" Volume 1.0 0.0 true)
      (bind _returnvalue_2 (Actor|GetActorOfClass "/Game/BP_SpacePlayerController.BP_SpacePlayerController_C"))
      (Utilities|Struct|SetmembersinF_AudioMix (Variables|/Game/BP_SpacePlayerController.BP_SpacePlayerController_C|GetAudioMix _returnvalue_2) Volume)
      (Audio|PushSoundMixModifier "/Engine/EngineSounds/SMIX_Main.SMIX_Main"))
    (:NewEnumerator2
      (Audio|SetSoundMixClassOverride "/Engine/EngineSounds/SMIX_Main.SMIX_Main" "/Engine/EngineSounds/Voice.Voice" Volume 1.0 0.0 true)
      (bind _returnvalue_3 (Actor|GetActorOfClass "/Game/BP_SpacePlayerController.BP_SpacePlayerController_C"))
      (Utilities|Struct|SetmembersinF_AudioMix (Variables|/Game/BP_SpacePlayerController.BP_SpacePlayerController_C|GetAudioMix _returnvalue_3) Volume)
      (Audio|PushSoundMixModifier "/Engine/EngineSounds/SMIX_Main.SMIX_Main"))))

(fn SaveGame
  (bind _returnvalue (SaveGame|DoesSaveGameExist "Save"))
  (if _returnvalue
    (bind _returnvalue_2 (SaveGame|LoadGamefromSlot "Save"))
    (bind _asbp_save_object (Utilities|Casting|CastToBP_SaveObject _returnvalue_2))
    (Variables|Default|SetSave%20Object _asbp_save_object)
    (else
      (bind _returnvalue_3 (SaveGame|CreateSaveGameObject "/Game/SaveGame/BP_SaveObject.BP_SaveObject_C"))
      (Variables|Default|SetSave%20Object _returnvalue_3)))
  (bind _returnvalue_4 (Actor|GetActorOfClass "/Game/BP_SpacePlayerController.BP_SpacePlayerController_C"))
  (Variables|/Game/SaveGame/BP_SaveObject.BP_SaveObject_C|SetName (Variables|Default|GetSave%20Object) (Utilities|String|ToString(Text) (Variables|/Script/UMG.TextBlock|GetText (Variables|/Game/UI/HUD/WBP_GameHUD.WBP_GameHUD_C|GetNameText (Variables|/Game/UI/HUD/WBP_GeneralUI.WBP_GeneralUI_C|GetWBP_GameHUD (Variables|/Game/BP_SpacePlayerController.BP_SpacePlayerController_C|GetGeneralUI _returnvalue_4))))))
  (Variables|/Game/SaveGame/BP_SaveObject.BP_SaveObject_C|SetMass (Variables|Default|GetSave%20Object) (Variables|/Game/Blueprints/BP_MainBlackHole.BP_MainBlackHole_C|GetCurrentMass (Variables|/Game/BP_SpacePlayerController.BP_SpacePlayerController_C|GetBlackHole _returnvalue_4)))
  (Variables|/Game/SaveGame/BP_SaveObject.BP_SaveObject_C|SetResearches (Variables|Default|GetSave%20Object) (Variables|/Game/Researches/BP_ResearchManager.BP_ResearchManager_C|GetResearchedTechnologies (Variables|/Game/BP_SpacePlayerController.BP_SpacePlayerController_C|GetResearchManager _returnvalue_4)))
  (Variables|/Game/SaveGame/BP_SaveObject.BP_SaveObject_C|SetCurrentTasks (Variables|Default|GetSave%20Object) (Variables|/Game/Tasks/BP_TasksSystem.BP_TasksSystem_C|GetCurrentTasks (Variables|/Game/BP_SpacePlayerController.BP_SpacePlayerController_C|GetTaskSystem _returnvalue_4)))
  (Variables|/Game/SaveGame/BP_SaveObject.BP_SaveObject_C|SetJournalEnries (Variables|Default|GetSave%20Object) (Variables|/Game/Journal/WBP_JournalWidget.WBP_JournalWidget_C|GetJournalData (Variables|/Game/BP_SpacePlayerController.BP_SpacePlayerController_C|GetJournal _returnvalue_4)))
  (SaveGame|SaveGametoSlot (Variables|Default|GetSave%20Object) "Save"))