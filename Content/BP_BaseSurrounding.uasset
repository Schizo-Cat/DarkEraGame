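; BP_BaseSurrounding is a surrounding actor whose lighting and materials react to the player's black hole.
; Every tick it pushes Color to MPC_Collection and three lights.
; While the controller's BlackHole is valid, its current-to-initial mass ratio sets point light intensity and drives the "deathofuniverse" material parameter, offset and clamped at zero.
; Under that same condition, eight widget components rotate to face the player pawn.
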(event EventBeginPlay
  (bind _asbp_space_player_controller (Utilities|Casting|CastToBP_SpacePlayerController (Game|GetPlayerController 0)))
  (Variables|Default|SetBP%20Space%20Player%20Controller _asbp_space_player_controller))

(event EventTick
  (params (DeltaSeconds :type Float%20%28single-precision%29))
  (bind _bp_space_player_controller (Variables|Default|GetBP%20Space%20Player%20Controller))
  (bind _color (Variables|Default|GetColor))
  (bind _pointlight (Variables|Default|GetPointLight))
  (bind _blackhole (Variables|/Game/BP_SpacePlayerController.BP_SpacePlayerController_C|GetBlackHole _bp_space_player_controller))
  (bind _currentmass (Variables|/Script/DarkEraProject.BlackHole|GetCurrentMass _blackhole))
  (bind _initialmass (Variables|/Script/DarkEraProject.BlackHole|GetInitialMass _blackhole))
  (bind _returnvalue (/ _currentmass _initialmass))
  (bind _returnvalue_2 (- _returnvalue 0.2))
  (Rendering|Material|SetVectorParameterValue "/Game/Materials/MPC_Collection.MPC_Collection" "color" _color :!class /Script/Engine.KismetMaterialLibrary)
  (Rendering|Components|Light|SetLightColor _pointlight _color true)
  (Utilities|IsValid _blackhole
    (:Is%20Valid
      (Rendering|Components|Light|SetIntensity _pointlight _returnvalue)
      (if (<= _returnvalue_2 0.0)
        (Rendering|Material|SetScalarParameterValue "/Game/Materials/MPC_Collection.MPC_Collection" "deathofuniverse" 0.0 :!class /Script/Engine.KismetMaterialLibrary)
        (else
          (Rendering|Material|SetScalarParameterValue "/Game/Materials/MPC_Collection.MPC_Collection" "deathofuniverse" _returnvalue_2 :!class /Script/Engine.KismetMaterialLibrary)))
      (for _array_element (Utilities|Array|MakeArray (Variables|Default|GetWidget6) (Variables|Default|GetWidget5) (Variables|Default|GetWidget4) (Variables|Default|GetWidget3) (Variables|Default|GetWidget2) (Variables|Default|GetWidget1) (Variables|Default|GetWidget7) (Variables|Default|GetWidget))
        (Transformation|SetWorldRotation _array_element (Math|Rotator|FindLookatRotation (Transformation|GetWorldLocation _array_element) (Transformation|GetActorLocation (Game|Player|GetPlayerPawn 0))) false false)))))

(fn ConstructionScript)