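; BP_Colony is a colony building Blueprint that continuously rolls its scene component while a black hole exists.
; A looping 0.01-second timer, started after the parent BeginPlay, increments the relative roll in proportion to the black hole's current mass and the SpaceController's time speed.
; Rotation stops while time is frozen or no valid black hole exists.
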(event Custom|Move%20around
  (bind _scene (Variables|Default|GetScene))
  (bind _space_controller (Variables|Default|GetSpace%20Controller))
  (bind _blackhole (Variables|/Game/BP_SpacePlayerController.BP_SpacePlayerController_C|GetBlackHole _space_controller))
  (bind _relativerotation (Variables|/Script/Engine.SceneComponent|GetRelativeRotation _scene))
  (if (not (Variables|/Script/DarkEraProject.SpacePlayerController|GetIsTimeFrozen _space_controller))
    (Utilities|IsValid _blackhole
      (:Is%20Valid
        (Transformation|SetRelativeRotation _scene (Math|Rotator|MakeRotator (+ (.roll _relativerotation) (* 0.01 (/ (Variables|/Game/Blueprints/BP_MainBlackHole.BP_MainBlackHole_C|GetCurrentMass _blackhole) 1e+01) (Variables|/Script/DarkEraProject.SpacePlayerController|GettimeSpeed _space_controller))) (.pitch _relativerotation) (.yaw _relativerotation)) false false)))))

(event EventBeginPlay
  (|CallParentFunction)
  (Utilities|Time|SetTimerbyEvent (delegate Custom|Move%20around) 0.01 true))

(fn ConstructionScript)