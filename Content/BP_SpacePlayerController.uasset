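; Player controller for the space black hole game, running the main UI, menu toggles and time controls.
; Input actions and HUD buttons share paths that set pause or speed and switch panels, some freezing time.
; Tick shows black hole mass, switching music, surroundings color and glitch overlay when critical.
; Losing the black hole triggers an explosion, color flash and final screen, then loads the main menu.
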(event Custom|SetTimeSpeed
  (params (Time%20Speed :type Float%20%28single-precision%29))
  (bind _spaceship (Variables|References|GetSpaceShip))
  (bind _spaceship_2 (Variables|References|GetSpaceShip))
  (bind _generalui (Variables|References|GetGeneralUI))
  (bind _wbp_gamehud (Variables|/Game/UI/HUD/WBP_GeneralUI.WBP_GeneralUI_C|GetWBP_GameHUD _generalui))
  (bind _p_flamethrower (Variables|/Game/Blueprints/BP_Ship.BP_Ship_C|GetP_Flamethrower _spaceship_2))
  (if (Variables|Default|GetCanChangeTime)
    (bind _output_get (Variables|Default|SettimeSpeed Time%20Speed))
    (if (> _output_get 0.0)
      (Variables|Default|SetSavedSpeed _output_get))
    (Utilities|IsValid _spaceship
      (:Is%20Valid
        (Variables|/Script/Engine.ParticleSystemComponent|SetCustomTimeDilation (Variables|/Game/Blueprints/BP_Ship.BP_Ship_C|GetP_Flamethrower _spaceship) _output_get)
        (if (Variables|Default|GetIsTimeFrozen)
          (Variables|/Script/Engine.ParticleSystemComponent|SetCustomTimeDilation _p_flamethrower 0.0)
          (Default|SetButtonSelected _wbp_gamehud (Variables|/Game/UI/HUD/WBP_GameHUD.WBP_GameHUD_C|GetPauseButton _wbp_gamehud))
          (else
            (bind _output_get_2 (Variables|Default|SettimeSpeed (Variables|Default|GetSavedSpeed)))
            (Variables|/Script/Engine.ParticleSystemComponent|SetCustomTimeDilation _p_flamethrower _output_get_2)
            (if (== _output_get_2 (Variables|Default|GetSpeedOne))
              (Default|SetButtonSelected _wbp_gamehud (Variables|/Game/UI/HUD/WBP_GameHUD.WBP_GameHUD_C|GetSpeedOneButton _wbp_gamehud))
              (elif (== _output_get_2 (Variables|Default|GetSpeedTwo))
                (Default|SetButtonSelected _wbp_gamehud (Variables|/Game/UI/HUD/WBP_GameHUD.WBP_GameHUD_C|GetSpeedTwoButton _wbp_gamehud))
                (elif (== _output_get_2 (Variables|Default|GetSpeedThree))
                  (Default|SetButtonSelected _wbp_gamehud (Variables|/Game/UI/HUD/WBP_GameHUD.WBP_GameHUD_C|GetSpeedThreeButton _wbp_gamehud)))))))))))

(event Custom|LerpColor
  (bind _returnvalue (Rendering|Material|GetVectorParameterValue "/Game/Materials/MPC_Collection.MPC_Collection" "color" :!class /Script/Engine.KismetMaterialLibrary))
  (Rendering|Material|SetVectorParameterValue "/Game/Materials/MPC_Collection.MPC_Collection" "color" (* _returnvalue 2.0) :!class /Script/Engine.KismetMaterialLibrary))

(event Custom|SetBlackHoleName
  (params (BlackHoleName :type Text))
  (bind _output_get (Variables|Default|SetBlackHoleName BlackHoleName))
  (Rendering|Components|TextRender|SetText (Variables|/Game/UI/HUD/WBP_GameHUD.WBP_GameHUD_C|GetNameText (Variables|/Game/UI/HUD/WBP_GeneralUI.WBP_GeneralUI_C|GetWBP_GameHUD (Variables|References|GetGeneralUI))) _output_get))

(event Custom|ChangeGameState
  (bind _basesurrounding (Variables|References|GetBaseSurrounding))
  (bind _researchmanager (Variables|References|GetResearchManager))
  (bind _istravelling (Variables|Default|GetIstravelling))
  (bind _basesurrounding_2 (Variables|References|GetBaseSurrounding))
  (bind _isresearching (Variables|/Game/Researches/BP_ResearchManager.BP_ResearchManager_C|GetIsResearching _researchmanager))
  ;[1 1 1] GameState
  (Variables|Default|SetAppendColor "(R=1.000000,G=1.000000,B=1.000000,A=1.000000)")
  (if (Variables|Default|GetIsMassCritical)
    (if (Variables|/Game/Blueprints/BP_BaseSurrounding.BP_BaseSurrounding_C|GetSlotsAvailable _basesurrounding)
      (Utilities|CompareMusic (Variables|Default|GetEndMusic))
      (Default|TurnVisibility _basesurrounding false)
      (Default|SetDangerNotificationActive (Variables|/Game/UI/HUD/WBP_GeneralUI.WBP_GeneralUI_C|GetWBP_GameHUD (Variables|References|GetGeneralUI)) true)
      (Variables|/Game/Blueprints/BP_BaseSurrounding.BP_BaseSurrounding_C|SetSlotsAvailable _basesurrounding false)
      (Default|SetGameColor _basesurrounding "(R=1.000000,G=0.000000,B=0.000000,A=1.000000)")
      (bind _returnvalue (UserInterface|CreateWidget "/Game/UI/CriticalUI/WBP_GlitchingEffects.WBP_GlitchingEffects_C"))
      (bind _output_get (Variables|Default|SetGlitchScreen _returnvalue))
      (UserInterface|Viewport|AddtoViewport _output_get -15))
    (else
      (Utilities|FlowControl|Sequence
        (:then_0
          (if _isresearching
            (Utilities|CompareMusic (Variables|Default|GetResearchMusic))
            (Variables|Default|SetAppendColor (* (Variables|Default|GetAppendColor) "(R=0.000000,G=0.796079,B=1.000000,A=1.000000)"))))
        (:then_1
          (if _istravelling
            (Variables|Default|SetAppendColor (* (Variables|Default|GetAppendColor) "(R=1.000000,G=0.850980,B=0.000000,A=1.000000)"))))
        (:then_2
          (if (not (or _isresearching _istravelling))
            (Utilities|CompareMusic (Variables|Default|GetCommon%20Music))))
        (:then_3
          (Default|SetGameColor _basesurrounding_2 (Variables|Default|GetAppendColor))
          (Default|TurnVisibility _basesurrounding_2 true)
          (Default|SetDangerNotificationActive (Variables|/Game/UI/HUD/WBP_GeneralUI.WBP_GeneralUI_C|GetWBP_GameHUD (Variables|References|GetGeneralUI)) false)
          (Variables|/Game/Blueprints/BP_BaseSurrounding.BP_BaseSurrounding_C|SetSlotsAvailable _basesurrounding_2 true)
          (Utilities|IsValid (Variables|Default|GetGlitchScreen)
            (:Is%20Valid
              (Widget|RemovefromParent (Variables|Default|GetGlitchScreen)))))))))

(event EventTick
  (params (DeltaSeconds :type Float%20%28single-precision%29))
  (bind _blackhole (Variables|References|GetBlackHole))
  (bind _returnvalue (Class|BlackHole|GetMass _blackhole))
  (bind _returnvalue_2 (Math|Float|Round _returnvalue))
  ;[1 1 1] Black Hole Mass UI
  (Utilities|IsValid _blackhole
    (:Is%20Valid
      (Rendering|Components|TextRender|SetText (Variables|/Game/UI/HUD/WBP_GameHUD.WBP_GameHUD_C|GetMassText (Variables|/Game/UI/HUD/WBP_GeneralUI.WBP_GeneralUI_C|GetWBP_GameHUD (Variables|References|GetGeneralUI))) (Utilities|Text|ToText(Integer) _returnvalue_2))
      (bind _output_get (Variables|Default|SetIsMassCritical (<= _returnvalue_2 100)))
      (if _output_get
        (Utilities|FlowControl|DoOnce false :!label _label
          (:Completed
            (CallFunction|ChangeGameState)
            (goto _label_2 Reset)))
        (else
          (Utilities|FlowControl|DoOnce true :!label _label_2
            (:Completed
              (CallFunction|ChangeGameState)
              (goto _label Reset))))))
    (:Is%20Not%20Valid
      (Utilities|FlowControl|DoOnce false
        (:Completed
          (bind _returnvalue_3 (Utilities|Time|SetTimerbyEvent (delegate Custom|LerpColor) 0.03 true))
          (Variables|Default|SetlerpTimer _returnvalue_3)
          (Utilities|Time|ClearandInvalidateTimerbyHandle (Variables|/Game/Blueprints/TimeManager.TimeManager_C|GetTimerSetTime (Variables|References|GetTimeManager)))
          (Widget|RemovefromParent (Variables|References|GetGeneralUI))
          (Audio|Components|Audio|SetSound (Variables|Default|GetAudioPlayer) "/Game/Sounds/blackholeexplosion.blackholeexplosion")
          (Utilities|FlowControl|Delay 0.6)
          (Utilities|Time|ClearandInvalidateTimerbyHandle (Variables|Default|GetlerpTimer))
          (bind _returnvalue_4 (UserInterface|CreateWidget "/Game/UI/CriticalUI/FinalScreen.FinalScreen_C"))
          (UserInterface|Viewport|AddtoViewport _returnvalue_4 0)
          (Utilities|FlowControl|Delay 31.0)
          (Game|OpenLevel(byObjectReference) "/Game/Maps/MainMenu.MainMenu"))))))

(event Custom|PauseTime
  (bind _generalui (Variables|References|GetGeneralUI))
  (bind _wbp_gamehud (Variables|/Game/UI/HUD/WBP_GeneralUI.WBP_GeneralUI_C|GetWBP_GameHUD _generalui))
  ;[1 1 1] Time
  (if (Variables|Default|GetCanChangeTime)
    (Variables|Default|SetIsTimeFrozen (not (Variables|Default|GetIsTimeFrozen)))
    (Default|SetButtonSelected _wbp_gamehud (Variables|/Game/UI/HUD/WBP_GameHUD.WBP_GameHUD_C|GetPauseButton _wbp_gamehud))
    (CallFunction|SetTimeSpeed 0.0)))

(event Custom|ToggleResearchMenu
  ;[1 1 1] ResearchToggle
  (Utilities|ToggleWidget (Variables|/Game/UI/HUD/WBP_GeneralUI.WBP_GeneralUI_C|GetResearchWindow (Variables|References|GetGeneralUI)) false))

(event Custom|ToggleSettings
  (bind _generalui (Variables|References|GetGeneralUI))
  (bind _wbp_settings (Variables|/Game/UI/HUD/WBP_GeneralUI.WBP_GeneralUI_C|GetWBP_Settings _generalui))
  ;[1 1 1] sETTINGStOGGLE
  (Default|SetMenuColor _wbp_settings)
  (Utilities|ToggleWidget _wbp_settings true))

(event Custom|ToggleContact
  ;[1 1 1] CommunicateWindowToggle
  (Utilities|ToggleWidget (Variables|/Game/UI/HUD/WBP_GeneralUI.WBP_GeneralUI_C|GetWBP_dialogueWindow (Variables|References|GetGeneralUI)) false))

(event Custom|ToggleJournal
  (bind _generalui (Variables|References|GetGeneralUI))
  (bind _wbp_journalwidget (Variables|/Game/UI/HUD/WBP_GeneralUI.WBP_GeneralUI_C|GetWBP_JournalWidget _generalui))
  ;[1 1 1] JournalToggle
  (Utilities|ToggleWidget _wbp_journalwidget true)
  (Default|CheckJournalOpen _wbp_journalwidget)
  (UserInterface|Animation|PlayAnimation _wbp_journalwidget (Variables|/Game/Journal/WBP_JournalWidget.WBP_JournalWidget_C|GetOpenJournal _wbp_journalwidget) 0.0 1 "Forward" 1.0 false))

(event Custom|Speed1
  ;[1 1 1] Time
  (CallFunction|SetTimeSpeed (Variables|Default|GetSpeedOne))
  (Variables|Default|SetIsTimeFrozen false))

(event Custom|Speed2
  ;[1 1 1] Time
  (CallFunction|SetTimeSpeed (Variables|Default|GetSpeedTwo))
  (Variables|Default|SetIsTimeFrozen false))

(event Custom|Speed3
  ;[1 1 1] Time
  (CallFunction|SetTimeSpeed (Variables|Default|GetSpeedThree))
  (Variables|Default|SetIsTimeFrozen false))

(event Custom|MapToggle
  ;[1 1 1] MapToggle
  (Utilities|ToggleWidget (Variables|/Game/UI/HUD/WBP_GeneralUI.WBP_GeneralUI_C|GetWBP_Map (Variables|References|GetGeneralUI)) false))

(event Custom|ToggleEscMenu
  (bind _generalui (Variables|References|GetGeneralUI))
  (bind _wbp_menuhud (Variables|/Game/UI/HUD/WBP_GeneralUI.WBP_GeneralUI_C|GetWBP_MenuHUD _generalui))
  ;[1 1 1] Open Menu Hud
  (Default|SetColorMenu _wbp_menuhud)
  (Utilities|ToggleWidget _wbp_menuhud true))

(event Input|EnhancedActionEvents|EnhancedInputActionIA_Journal
  (params (ActionValue :type Boolean) (ElapsedSeconds :type Float%20%28double-precision%29) (TriggeredSeconds :type Float%20%28double-precision%29) (InputAction :type Input%20Action%20Object%20Reference :default "/Game/Input/MenuControls/IA_Journal.IA_Journal"))
  (bind _generalui (Variables|References|GetGeneralUI))
  (bind _wbp_journalwidget (Variables|/Game/UI/HUD/WBP_GeneralUI.WBP_GeneralUI_C|GetWBP_JournalWidget _generalui))
  ;[1 1 1] JournalToggle
  (:Started
    (Utilities|ToggleWidget _wbp_journalwidget true)
    (Default|CheckJournalOpen _wbp_journalwidget)
    (UserInterface|Animation|PlayAnimation _wbp_journalwidget (Variables|/Game/Journal/WBP_JournalWidget.WBP_JournalWidget_C|GetOpenJournal _wbp_journalwidget) 0.0 1 "Forward" 1.0 false)))

(event Input|EnhancedActionEvents|EnhancedInputActionIA_Research
  (params (ActionValue :type Boolean) (ElapsedSeconds :type Float%20%28double-precision%29) (TriggeredSeconds :type Float%20%28double-precision%29) (InputAction :type Input%20Action%20Object%20Reference :default "/Game/Input/MenuControls/IA_Research.IA_Research"))
  ;[1 1 1] ResearchToggle
  (:Started
    (Utilities|ToggleWidget (Variables|/Game/UI/HUD/WBP_GeneralUI.WBP_GeneralUI_C|GetResearchWindow (Variables|References|GetGeneralUI)) false)))

(event Input|EnhancedActionEvents|EnhancedInputActionIA_Contact
  (params (ActionValue :type Boolean) (ElapsedSeconds :type Float%20%28double-precision%29) (TriggeredSeconds :type Float%20%28double-precision%29) (InputAction :type Input%20Action%20Object%20Reference :default "/Game/Input/MenuControls/IA_Contact.IA_Contact"))
  ;[1 1 1] CommunicateWindowToggle
  (:Started
    (Utilities|ToggleWidget (Variables|/Game/UI/HUD/WBP_GeneralUI.WBP_GeneralUI_C|GetWBP_dialogueWindow (Variables|References|GetGeneralUI)) false)))

(event Input|EnhancedActionEvents|EnhancedInputActionIA_Pause
  (params (ActionValue :type Boolean) (ElapsedSeconds :type Float%20%28double-precision%29) (TriggeredSeconds :type Float%20%28double-precision%29) (InputAction :type Input%20Action%20Object%20Reference :default "/Game/Input/MenuControls/IA_Pause.IA_Pause"))
  (bind _generalui (Variables|References|GetGeneralUI))
  (bind _wbp_gamehud (Variables|/Game/UI/HUD/WBP_GeneralUI.WBP_GeneralUI_C|GetWBP_GameHUD _generalui))
  ;[1 1 1] Time
  (:Started
    (if (Variables|Default|GetCanChangeTime)
      (Variables|Default|SetIsTimeFrozen (not (Variables|Default|GetIsTimeFrozen)))
      (Default|SetButtonSelected _wbp_gamehud (Variables|/Game/UI/HUD/WBP_GameHUD.WBP_GameHUD_C|GetPauseButton _wbp_gamehud))
      (CallFunction|SetTimeSpeed 0.0))))

(event Input|EnhancedActionEvents|EnhancedInputActionIA_Speed1
  (params (ActionValue :type Boolean) (ElapsedSeconds :type Float%20%28double-precision%29) (TriggeredSeconds :type Float%20%28double-precision%29) (InputAction :type Input%20Action%20Object%20Reference :default "/Game/Input/MenuControls/IA_Speed1.IA_Speed1"))
  ;[1 1 1] Time
  (:Started
    (CallFunction|SetTimeSpeed (Variables|Default|GetSpeedOne))
    (Variables|Default|SetIsTimeFrozen false)))

(event Input|EnhancedActionEvents|EnhancedInputActionIA_Speed2
  (params (ActionValue :type Boolean) (ElapsedSeconds :type Float%20%28double-precision%29) (TriggeredSeconds :type Float%20%28double-precision%29) (InputAction :type Input%20Action%20Object%20Reference :default "/Game/Input/MenuControls/IA_Speed2.IA_Speed2"))
  ;[1 1 1] Time
  (:Started
    (CallFunction|SetTimeSpeed (Variables|Default|GetSpeedTwo))
    (Variables|Default|SetIsTimeFrozen false)))

(event Input|EnhancedActionEvents|EnhancedInputActionIA_Speed3
  (params (ActionValue :type Boolean) (ElapsedSeconds :type Float%20%28double-precision%29) (TriggeredSeconds :type Float%20%28double-precision%29) (InputAction :type Input%20Action%20Object%20Reference :default "/Game/Input/MenuControls/IA_Speed3.IA_Speed3"))
  ;[1 1 1] Time
  (:Started
    (CallFunction|SetTimeSpeed (Variables|Default|GetSpeedThree))
    (Variables|Default|SetIsTimeFrozen false)))

(event Input|EnhancedActionEvents|EnhancedInputActionIA_Map
  (params (ActionValue :type Boolean) (ElapsedSeconds :type Float%20%28double-precision%29) (TriggeredSeconds :type Float%20%28double-precision%29) (InputAction :type Input%20Action%20Object%20Reference :default "/Game/Input/MenuControls/IA_Map.IA_Map"))
  ;[1 1 1] MapToggle
  (:Started
    (Utilities|ToggleWidget (Variables|/Game/UI/HUD/WBP_GeneralUI.WBP_GeneralUI_C|GetWBP_Map (Variables|References|GetGeneralUI)) false)))

(event Input|EnhancedActionEvents|EnhancedInputActionIA_Exit
  (params (ActionValue :type Boolean) (ElapsedSeconds :type Float%20%28double-precision%29) (TriggeredSeconds :type Float%20%28double-precision%29) (InputAction :type Input%20Action%20Object%20Reference :default "/Game/Input/MenuControls/IA_Exit.IA_Exit"))
  (bind _generalui (Variables|References|GetGeneralUI))
  (bind _wbp_menuhud (Variables|/Game/UI/HUD/WBP_GeneralUI.WBP_GeneralUI_C|GetWBP_MenuHUD _generalui))
  ;[1 1 1] Open Menu Hud
  (:Started
    (Default|SetColorMenu _wbp_menuhud)
    (Utilities|ToggleWidget _wbp_menuhud true)))

(event EventBeginPlay
  (bind _returnvalue (Game|GetPlayerController 0))
  (bind _returnvalue_2 (Actor|GetActorOfClass "/Game/Tasks/BP_TasksSystem.BP_TasksSystem_C"))
  (Variables|Default|SetTaskSystem _returnvalue_2)
  (bind _returnvalue_3 (Actor|GetActorOfClass "/Game/Blueprints/TimeManager.TimeManager_C"))
  (Variables|References|SetTimeManager _returnvalue_3)
  (bind _returnvalue_4 (Actor|GetActorOfClass "/Game/Blueprints/BP_BaseSurrounding.BP_BaseSurrounding_C"))
  (Variables|References|SetBaseSurrounding _returnvalue_4)
  (bind _returnvalue_5 (Actor|GetActorOfClass "/Game/Blueprints/BP_Ship.BP_Ship_C"))
  (Variables|References|SetSpaceShip _returnvalue_5)
  (Input|AddMappingContext (PlayerController|LocalPlayerSubsystems|GetEnhancedInputLocalPlayerSubsystem (Game|GetPlayerController 0)) "/Game/Input/MenuControls/IMC_MenuControl.IMC_MenuControl" 0 "(bIgnoreAllPressedKeysUntilRelease=True,bForceImmediately=False,bNotifyUserSettings=False)")
  (Input|AddMappingContext (PlayerController|LocalPlayerSubsystems|GetEnhancedInputLocalPlayerSubsystem _returnvalue) "/Game/Input/Movement/IMC_Spectating.IMC_Spectating" 0 "(bIgnoreAllPressedKeysUntilRelease=True,bForceImmediately=False,bNotifyUserSettings=False)")
  (Input|SetInputModeGameandUI _returnvalue 0 "DoNotLock" true false)
  (bind _returnvalue_6 (Actor|GetActorOfClass "/Game/Researches/BP_ResearchManager.BP_ResearchManager_C"))
  (Variables|References|SetResearchManager _returnvalue_6)
  (bind _returnvalue_7 (Actor|GetActorOfClass "/Game/Blueprints/MainBlackHole.MainBlackHole_C"))
  (Variables|References|SetBlackHole _returnvalue_7)
  (bind _returnvalue_8 (UserInterface|CreateWidget "/Game/UI/HUD/WBP_GeneralUI.WBP_GeneralUI_C"))
  (bind _output_get (Variables|References|SetGeneralUI _returnvalue_8))
  (UserInterface|Viewport|AddtoViewport _output_get 0)
  (Variables|Default|SetbShowMouseCursor true)
  (Utilities|FlowControl|Sequence
    (:then_0
      (EventDispatchers|BindEventtoOnClicked (Variables|/Game/UI/HUD/WBP_GameHUD.WBP_GameHUD_C|GetJournalButton (Variables|/Game/UI/HUD/WBP_GeneralUI.WBP_GeneralUI_C|GetWBP_GameHUD (Variables|References|GetGeneralUI))) (delegate Custom|ToggleJournal))
      (EventDispatchers|BindEventtoOnClicked (Variables|/Game/UI/HUD/WBP_GameHUD.WBP_GameHUD_C|GetResearchButton (Variables|/Game/UI/HUD/WBP_GeneralUI.WBP_GeneralUI_C|GetWBP_GameHUD (Variables|References|GetGeneralUI))) (delegate Custom|ToggleResearchMenu))
      (EventDispatchers|BindEventtoOnClicked (Variables|/Game/UI/HUD/WBP_GameHUD.WBP_GameHUD_C|GetContactButton (Variables|/Game/UI/HUD/WBP_GeneralUI.WBP_GeneralUI_C|GetWBP_GameHUD (Variables|References|GetGeneralUI))) (delegate Custom|ToggleContact))
      (EventDispatchers|BindEventtoOnClicked (Variables|/Game/UI/HUD/WBP_GameHUD.WBP_GameHUD_C|GetMapButton (Variables|/Game/UI/HUD/WBP_GeneralUI.WBP_GeneralUI_C|GetWBP_GameHUD (Variables|References|GetGeneralUI))) (delegate Custom|MapToggle)))
    (:then_1
      ;[1 1 1] Time
      (EventDispatchers|BindEventtoOnClicked (Variables|/Game/UI/HUD/WBP_GameHUD.WBP_GameHUD_C|GetPauseButton (Variables|/Game/UI/HUD/WBP_GeneralUI.WBP_GeneralUI_C|GetWBP_GameHUD (Variables|References|GetGeneralUI))) (delegate Custom|PauseTime))
      (EventDispatchers|BindEventtoOnClicked (Variables|/Game/UI/HUD/WBP_GameHUD.WBP_GameHUD_C|GetSpeedOneButton (Variables|/Game/UI/HUD/WBP_GeneralUI.WBP_GeneralUI_C|GetWBP_GameHUD (Variables|References|GetGeneralUI))) (delegate Custom|Speed1))
      (EventDispatchers|BindEventtoOnClicked (Variables|/Game/UI/HUD/WBP_GameHUD.WBP_GameHUD_C|GetSpeedTwoButton (Variables|/Game/UI/HUD/WBP_GeneralUI.WBP_GeneralUI_C|GetWBP_GameHUD (Variables|References|GetGeneralUI))) (delegate Custom|Speed2))
      (EventDispatchers|BindEventtoOnClicked (Variables|/Game/UI/HUD/WBP_GameHUD.WBP_GameHUD_C|GetSpeedThreeButton (Variables|/Game/UI/HUD/WBP_GeneralUI.WBP_GeneralUI_C|GetWBP_GameHUD (Variables|References|GetGeneralUI))) (delegate Custom|Speed3)))))

(fn ConstructionScript)