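; Quest manager for the space game that adds, tracks and completes tasks shown in the HUD task list.
; AddTask creates task widgets and can bind ship object-collection events for subtask progress.
; ExplorationProgress maps neutron stars, black holes and quest ruins to subtasks, completing the task when none remain.
; CompleteTask shows notifications, chains data-table follow-up tasks and hardcodes per-task rewards like research unlocks, dialogues and map destinations.
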(event EventBeginPlay
  (bind _asbp_space_player_controller (Utilities|Casting|CastToBP_SpacePlayerController (Game|GetPlayerController 0)))
  (Variables|Default|SetSpaceController _asbp_space_player_controller))

(fn ConstructionScript)

(fn AddTask
  (params (Task :type Task%20Structure%20Structure))
  (bind _taskid (Utilities|Struct|BreakTaskStructure Task))
  (bind _spacecontroller (Variables|Default|GetSpaceController))
  (Utilities|Array|Add (Variables|Default|GetCurrentTasks) Task)
  (bind _returnvalue (UserInterface|CreateWidget "/Game/Tasks/WBP_Task.WBP_Task_C" 0 Task))
  (Utilities|IsValid _returnvalue
    (:Is%20Valid
      (Utilities|Array|Add (Variables|Default|GetTasksWBP) _returnvalue)
      (Widget|Panel|AddChild (Variables|/Game/UI/HUD/WBP_GameHUD.WBP_GameHUD_C|GetTasksScrollBox (Variables|/Game/UI/HUD/WBP_GeneralUI.WBP_GeneralUI_C|GetWBP_GameHUD (Variables|/Game/Core/Player/BP_SpacePlayerController.BP_SpacePlayerController_C|GetGeneralUI _spacecontroller))) _returnvalue)
      (switch string _taskid
        (:explorationExtraction
          (Variables|Default|SetTask%20Id _taskid)
          (EventDispatchers|BindEventtoOnObjectCollected (Variables|/Game/Core/Player/BP_SpacePlayerController.BP_SpacePlayerController_C|GetSpaceShip _spacecontroller) (EventDispatchers|CreateEvent :!event ExplorationProgress)))))))

(fn CompleteTask
  (params (TaskToEnd :type Task%20Structure%20Structure))
  (bind (_task _subtasks _completionmessage _taskid _nexttask) (Utilities|Struct|BreakTaskStructure TaskToEnd))
  (bind _spacecontroller (Variables|Default|GetSpaceController))
  (bind _spacecontroller_2 (Variables|Default|GetSpaceController))
  (bind _spacecontroller_3 (Variables|Default|GetSpaceController))
  (bind _spacecontroller_4 (Variables|Default|GetSpaceController))
  (bind _generalui (Variables|/Game/Core/Player/BP_SpacePlayerController.BP_SpacePlayerController_C|GetGeneralUI _spacecontroller_4))
  (bind _generalui_2 (Variables|/Game/Core/Player/BP_SpacePlayerController.BP_SpacePlayerController_C|GetGeneralUI _spacecontroller))
  (bind _tasksystem (Variables|/Game/Core/Player/BP_SpacePlayerController.BP_SpacePlayerController_C|GetTaskSystem _spacecontroller_2))
  (bind _researchwindow (Variables|/Game/UI/HUD/WBP_GeneralUI.WBP_GeneralUI_C|GetResearchWindow _generalui_2))
  (bind _researchwindow_2 (Variables|/Game/UI/HUD/WBP_GeneralUI.WBP_GeneralUI_C|GetResearchWindow _generalui))
  (bind _colonyresearch_button_1 (Variables|/Game/UI/ResearchWindow/ResearchWindow.ResearchWindow_C|GetColonyResearch_Button_1 _researchwindow))
  (bind _singularityresearch_button_1 (Variables|/Game/UI/ResearchWindow/ResearchWindow.ResearchWindow_C|GetSingularityResearch_Button_1 _researchwindow_2))
  (if (Utilities|Array|ContainsItem (Variables|Default|GetCurrentTasks) TaskToEnd)
    (bind _array_element (Utilities|Array|ForEachLoopwithBreak (Variables|Default|GetTasksWBP))
      (:LoopBody
        (if (and true (Utilities|Enum|Equal(Enum) (.task (Variables|/Game/Tasks/WBP_Task.WBP_Task_C|GetTask _array_element)) _task))
          (if (Utilities|Text|TextIsEmpty (Utilities|Text|ToText(String) (.completionmessage (Variables|/Game/Tasks/WBP_Task.WBP_Task_C|GetTask _array_element))))
            _
            (else
              (bind _returnvalue (UserInterface|CreateWidget "/Game/Tasks/WBP_Notification.WBP_Notification_C" 0 (Utilities|Text|ToText(String) (.completionmessage (Variables|/Game/Tasks/WBP_Task.WBP_Task_C|GetTask _array_element)))))
              (UserInterface|Viewport|AddtoViewport _returnvalue 0)))
          (Widget|RemovefromParent _array_element)
          (Utilities|Array|RemoveItem (Variables|Default|GetTasksWBP) _array_element)
          (Utilities|Array|RemoveItem (Variables|Default|GetCurrentTasks) TaskToEnd)))
      (:Completed
        (Audio|PlaySound2D "/Game/Core/Audio/SFX/Notifications/error_sci-fi_sound.error_sci-fi_sound" 1.0 1.0 0.0 0 0)
        (Utilities|IsValid (.datatable _nexttask)
          (:Is%20Valid
            (bind _returnvalue_2 (Utilities|GetDataTableRow (.datatable _nexttask) (.rowname _nexttask))
              (:then
                (CallFunction|AddTask _returnvalue_2))
              (:RowNotFound
                _)))
          (:Is%20Not%20Valid
            _))
        ;[1 1 1] TaksImpact
        (switch string _taskid
          (:buildResearch
            (Default|CallResearchStatusChange (Variables|Default|GetSpaceController) true)
            (bind _returnvalue_3 (Utilities|GetDataTableRow "/Game/Core/DataTables/TaskList.TaskList" "FLY_Somewhere")
              (:then
                (CallFunction|AddTask _tasksystem _returnvalue_3)
                (bind _returnvalue_4 (Utilities|GetDataTableRow "/Game/Core/DataTables/TaskList.TaskList" "R_Extraction")
                  (:then
                    (CallFunction|AddTask _tasksystem _returnvalue_4))))))
          (:extractor
            (Widget|SetIsEnabled (Variables|/Game/UI/HUD/WBP_GameHUD.WBP_GameHUD_C|GetExtractButton (Variables|/Game/UI/HUD/WBP_GeneralUI.WBP_GeneralUI_C|GetWBP_GameHUD (Variables|/Game/Core/Player/BP_SpacePlayerController.BP_SpacePlayerController_C|GetGeneralUI (Variables|Default|GetSpaceController)))) true))
          (:exploreEnemySector
            (bind _returnvalue_5 (Utilities|GetDataTableRow "/Game/Core/DataTables/DT_Dialogues.DT_Dialogues" "SF_2ED_Result")
              (:then
                (bind _returnvalue_6 (Utilities|GetDataTableRow "/Game/Core/DataTables/DT_FractionsList.DT_FractionsList" "ResearchFraction")
                  (:then
                    (Default|InitiateDialogue (Variables|/Game/Core/Player/BP_SpacePlayerController.BP_SpacePlayerController_C|GetDialogueSystem _spacecontroller_4) _returnvalue_5 _returnvalue_6)
                    (Widget|SetVisibility _singularityresearch_button_1 "Visible")
                    (Variables|/Game/UI/ResearchWindow/Research_Button.Research_Button_C|SetIsquestDisabled _singularityresearch_button_1 false))))))
          (:explorationExtraction
            (Widget|SetVisibility _colonyresearch_button_1 "Visible")
            (Variables|/Game/UI/ResearchWindow/Research_Button.Research_Button_C|SetIsquestDisabled (Variables|/Game/UI/ResearchWindow/ResearchWindow.ResearchWindow_C|GetWarpDrivelResearch_Button _researchwindow) false)
            (Variables|/Game/UI/ResearchWindow/Research_Button.Research_Button_C|SetIsquestDisabled _colonyresearch_button_1 false)
            (bind _returnvalue_7 (Utilities|GetDataTableRow "/Game/Core/DataTables/TaskList.TaskList" "B_Colony")
              (:then
                (CallFunction|AddTask _returnvalue_7))))
          (:researchSingularity
            (bind _returnvalue_8 (Utilities|GetDataTableRow "/Game/Core/DataTables/DT_Dialogues.DT_Dialogues" "SF_2ED_ResultResearch")
              (:then
                (bind _returnvalue_9 (Utilities|GetDataTableRow "/Game/Core/DataTables/DT_FractionsList.DT_FractionsList" "ResearchFraction")
                  (:then
                    (Default|InitiateDialogue (Variables|/Game/Core/Player/BP_SpacePlayerController.BP_SpacePlayerController_C|GetDialogueSystem _spacecontroller_3) _returnvalue_8 _returnvalue_9))))))
          (:flyBase
            (Default|AddNewDestination (Variables|/Game/UI/HUD/WBP_GeneralUI.WBP_GeneralUI_C|GetWBP_Map (Variables|/Game/Core/Player/BP_SpacePlayerController.BP_SpacePlayerController_C|GetGeneralUI _spacecontroller_3)) (Variables|Default|GetRelicDataTable))))))))

(fn ExplorationProgress
  (params (ObjectType :type BP%20Space%20Body%20Base%20Object%20Reference))
  (Utilities|Casting|CastToBP_NeutronStar ObjectType
    (:then
      (Variables|Default|SetSubTaskToUpdate "neutronStarExtraction"))
    (:CastFailed
      (Utilities|Casting|CastToBP_BlackHole ObjectType
        (:then
          (Variables|Default|SetSubTaskToUpdate "blackHoleExtraction"))
        (:CastFailed
          (Utilities|Casting|CastToBP_QuestRuins ObjectType)
          (Variables|Default|SetSubTaskToUpdate "questRelicExtraction")))))
  (CallFunction|UpdateProgress))

(fn UpdateProgress
  (bind _array_element (Utilities|Array|ForEachLoopwithBreak (Variables|Default|GetTasksWBP) :!label _label)
    (:LoopBody
      (if (Utilities|Enum|Equal(Enum) (.taskid (Variables|/Game/Tasks/WBP_Task.WBP_Task_C|GetTask _array_element)) (Variables|Default|GetTask%20Id))
        (Variables|Default|SetArray%20Element _array_element)
        (goto _label Break)))
    (:Completed
      (Utilities|IsValid (Variables|Default|GetArray%20Element)
        (:Is%20Valid
          (bind _array_element_2 (Utilities|Array|ForEachLoopwithBreak (.subtasks (Variables|/Game/Tasks/WBP_Task.WBP_Task_C|GetTask _array_element)) :!label _label_2)
            (:LoopBody
              (if (Utilities|Enum|Equal(Enum) (Variables|Default|GetSubTaskToUpdate) (.SubTaskId (Utilities|Struct|BreakSubtaskStructure _array_element_2)))
                (Variables|Default|SetSubtaskToProgress _array_element_2)
                (goto _label_2 Break)))
            (:Completed
              (bind _array_element_3 (Utilities|Array|ForEachLoopwithBreak (Variables|/Game/Tasks/WBP_Task.WBP_Task_C|GetSubtasksWBP (Variables|Default|GetArray%20Element)) :!label _label_3)
                (:LoopBody
                  (if (Utilities|Enum|Equal(Enum) (.SubTaskId (Utilities|Struct|BreakSubtaskStructure _array_element_2)) (.subtaskid (Variables|/Game/Tasks/WBP_Subtask.WBP_Subtask_C|GetSubtask _array_element_3)))
                    (Variables|Default|SetSubtaskWidget _array_element_3)
                    (bind _result (Math|Integer|IncrementInt (Variables|/Game/Tasks/WBP_Subtask.WBP_Subtask_C|GetProgress (Variables|Default|GetSubtaskWidget)))
                      (:%20%20
                        (if (< _result (.completionnumber (Variables|/Game/Tasks/WBP_Subtask.WBP_Subtask_C|GetSubtask _array_element_3)))
                          (Default|UpdateProgress _array_element_3)
                          (goto _label_3 Break)
                          (else
                            (Utilities|Array|RemoveItem (Variables|/Game/Tasks/WBP_Task.WBP_Task_C|GetSubtasksWBP (Variables|Default|GetArray%20Element)) (Variables|Default|GetSubtaskWidget))
                            (Widget|RemovefromParent (Variables|Default|GetSubtaskWidget))
                            (Development|PrintString (Utilities|String|ToString(Integer) (Utilities|Array|Length (Variables|/Game/Tasks/WBP_Task.WBP_Task_C|GetSubtasksWBP (Variables|Default|GetArray%20Element)))))
                            (if (Utilities|Array|IsEmpty (Variables|/Game/Tasks/WBP_Task.WBP_Task_C|GetSubtasksWBP (Variables|Default|GetArray%20Element)))
                              (CallFunction|CompleteTask (Variables|/Game/Tasks/WBP_Task.WBP_Task_C|GetTask (Variables|Default|GetArray%20Element)))
                              (goto _label_3 Break))))))))))))))))

(fn ClearTasks
  (bind _taskswbp (Variables|Default|GetTasksWBP))
  (for _array_element _taskswbp
    (Widget|RemovefromParent _array_element)
    (Utilities|Array|RemoveItem _taskswbp _array_element)))